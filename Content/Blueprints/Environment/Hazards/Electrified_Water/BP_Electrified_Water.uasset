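; BP_Electrified_Water is an environmental hazard that continuously damages actors standing inside it.
; Begin and end overlap events add and remove actors from ActorsToDamage, maintain a SomeoneInWater flag and print debug messages.
; Tick applies BP_DamageTypeBasic damage to every tracked actor, scaling DPS by delta time for a frame-rate-independent rate.
; Overlapping actors are not filtered, and the flag is set but never read here.
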(event `self.ReceiveTick`
  (params (DeltaSeconds :type "Float (single-precision)"))
  (for _array_element (`self.ActorsToDamage`)
    (`GameplayStatics.ApplyDamage` _array_element (* DeltaSeconds (`self.DPS`)) null null "/Game/Blueprints/Character/BP_DamageTypeBasic.BP_DamageTypeBasic_C")))

(event `self.ReceiveActorBeginOverlap`
  (params (OtherActor :type "Actor Object Reference"))
  (`KismetArrayLibrary.Array_Add` (`self.ActorsToDamage`) OtherActor)
  (set `self.SomeoneInWater` true)
  (`KismetSystemLibrary.PrintString` "start to hurt the person"))

(event `self.ReceiveActorEndOverlap`
  (params (OtherActor :type "Actor Object Reference"))
  (bind _actorstodamage (`self.ActorsToDamage`))
  (`KismetArrayLibrary.Array_RemoveItem` _actorstodamage OtherActor)
  (if (<= (`KismetArrayLibrary.Array_Length` _actorstodamage) 0)
    (set `self.SomeoneInWater` false))
  (`KismetSystemLibrary.PrintString` "im done hurting you"))

(fn `UserConstructionScript`)