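; BP_LaserManager is a laser hazard controller that toggles an array of lasers one after another in a staggered sequence.
; Tick accumulates time and starts a new Toggle pass whenever the array length times DelayRate has elapsed.
; Toggle loops through the array with a latent Delay, calling ToggleLasers on each element and waiting DelayRate between steps, then resets its index after the last.
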(event `self.ReceiveTick`
  (params (DeltaSeconds :type "Float (single-precision)"))
  (bind _output_get (set `self.Counter` (+ DeltaSeconds (`self.Counter`))))
  (if (>= _output_get (* (`KismetArrayLibrary.Array_Length` (`self.Laser Array`)) (`self.DelayRate`)))
    (set `self.Counter` 0.0)
    (`self.Toggle` (`KismetArrayLibrary.Array_Length` (`self.Laser Array`)))))

(fn `UserConstructionScript`)