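; BP_WardenBomb is a thrown bomb for the Warden boss fight that damages the player and notifies any Warden caught in the blast.
; It launches with an initial impulse, freezes on first surface hit, and explodes on player overlap or player bullet.
; A Gate delays automatic detonation until the second Tick, leaving time to push the player away.
; The one-shot explosion sphere-traces pawns, requiring line of sight for player damage and calling BombHit on Wardens.
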(event `self.ReceiveBeginPlay`
  (bind _returnvalue (`self.GetInstigator`))
  ;[1 1 1] ignore collisions with whatever spawned this bomb
  (`PrimitiveComponent.IgnoreActorWhenMoving` (`self.Hit Box`) _returnvalue true)
  (`PrimitiveComponent.IgnoreActorWhenMoving` (`self.StaticMesh`) _returnvalue true)
  (`PrimitiveComponent.AddImpulse` (`self.StaticMesh`) (`self.Initial Velocity`) "None" true))

(event `self.Hit Box.OnComponentBeginOverlap`
  (params (OtherActor :type "Actor Object Reference") (OtherComp :type "PrimitiveComponent Object Reference") (OtherBodyIndex :type Integer) (bFromSweep :type Boolean) (SweepResult :type "HitResult Structure (by ref)"))
  (if (`self.IsActorTickEnabled`)
    (cast `/Game/Blueprints/Character/BP_MainCharacter` OtherActor
      (:`then`
        (`self.Explode`))
      (:`CastFailed`
        (bind _asbullet (cast `/Game/Blueprints/Bullet` OtherActor))
        (cast `/Game/Blueprints/Character/BP_MainCharacter` (`self.GetOwner` _asbullet))
        (`self.Explode`)))))

(event `self.StaticMesh.OnComponentHit`
  (params (OtherActor :type "Actor Object Reference") (OtherComp :type "PrimitiveComponent Object Reference") (NormalImpulse :type "Vector Structure") (Hit :type "HitResult Structure (by ref)"))
  ;[1 1 1] freeze the actor when it touches a surface.
  (`/Engine/EditorBlueprintResources/StandardMacros.DoOnce` false
    (:`Completed`
      (`PrimitiveComponent.SetSimulatePhysics` (`self.StaticMesh`) false))))

(event `self.ReceiveTick`
  (params (DeltaSeconds :type "Float (single-precision)"))
  ;[1 1 1] First tick, gate is closed, so it opens gate. Second tick, gate is open, bomb explodes, future ticks are turned off in Explode. This work around is used to allow the player enough time to use the bomb's location to push the player away from the explosion
  (`|ExecutionSequence`
    (:`then_0`
      (`/Engine/EditorBlueprintResources/StandardMacros.Gate` true :!label _label
        (:`Exit`
          (`self.Explode`))))
    (:`then_1`
      (goto _label :!via `Open`))))

(event `Explode`
  (bind _returnvalue (`self.K2_GetActorLocation`))
  (`/Engine/EditorBlueprintResources/StandardMacros.DoOnce` false
    (:`Completed`
      (`self.SetActorTickEnabled` false)
      (`SceneComponent.SetVisibility` (`self.StaticMesh`) false false)
      (bind _returnvalue_2 (`GameplayStatics.SpawnEmitterAtLocation` "/Game/Particles/Emitters/P_Explosion_A.P_Explosion_A" (+ _returnvalue (0.0 0.0 50.0))))
      (`SceneComponent.SetWorldScale3D` _returnvalue_2 (4.0 4.0 4.0)) ; I'd prefer a larger particle effect as opposed to scaling this one.
      (bind _outhits (`KismetSystemLibrary.SphereTraceMultiForObjects` _returnvalue (+ _returnvalue (0.0 0.0 10.0)) 380.0 (`|MakeArray` "ObjectTypeQuery3" :!type "EObjectTypeQuery Enum"))) ; sphere trace for pawns
      ;[1 1 1] loop over sweep results until we find a player. (breaks when first player is found)
      (for _array_element _outhits
        (bind (_bblockinghit _binitialoverlap _time _location _impactpoint _normal _impactnormal _physmat _hitactor) (`GameplayStatics.BreakHitResult` _array_element))
        (bind _asbp_main_character (cast `/Game/Blueprints/Character/BP_MainCharacter` _hitactor)
          (:`then`
            ;[1 1 1] confirm the player is within a direct line of the bomb before dealing damage.
            (bind _outhit (`KismetSystemLibrary.LineTraceSingle` (+ _returnvalue (0.0 0.0 25.0)) (`self.K2_GetActorLocation` _asbp_main_character) "TraceTypeQuery1"))
            (if (== (`.HitActor` (`GameplayStatics.BreakHitResult` _outhit)) _asbp_main_character)
              (`GameplayStatics.ApplyDamage` _asbp_main_character 30.0 null self "/Game/Blueprints/Character/BP_ContactDamage.BP_ContactDamage_C")
              (break)
              (else
                (break))))
          (:`CastFailed`
            (bind _asbp_warden (cast `/Game/Blueprints/Bosses/Warden/BP_Warden` _hitactor))
            (`/Game/Blueprints/Bosses/Warden/BP_Warden.BombHit` _asbp_warden)))))))

(fn `UserConstructionScript`)