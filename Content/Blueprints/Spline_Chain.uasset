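; Spline-driven chain actor that builds a run of prison chain-link meshes along a spline in the level.
; The construction script divides spline length by Spacing and adds one static mesh component at each interval, using world-space location and rotation with manual attachment.
; Each link gets a random roll between 0 and 180 degrees from a random stream, combined with the spline's rotation.
; The event graph has no active logic.
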(event `self.ReceiveBeginPlay`)

(event `self.ReceiveActorBeginOverlap`
  (params (OtherActor :type "Actor Object Reference")))

(event `self.ReceiveTick`
  (params (DeltaSeconds :type "Float (single-precision)")))

(fn `UserConstructionScript`
  (bind _splinecomonentexample (`self.Splinecomonentexample`))
  (bind _spacing (`self.Spacing`))
  (for _index (range (+ (`.ReturnValue` (`KismetMathLibrary.FMod` (`SplineComponent.GetSplineLength` _splinecomonentexample) _spacing)) 1))
    (bind _returnvalue (* _index _spacing))
    (bind _returnvalue_2 (`AddComponent|Static Mesh Component_13` :`bManualAttachment` true :`RelativeTransform` (`KismetMathLibrary.MakeTransform` (`SplineComponent.GetLocationAtDistanceAlongSpline` _splinecomonentexample _returnvalue "World") (`KismetMathLibrary.ComposeRotators` (`KismetMathLibrary.MakeRotator` (`KismetMathLibrary.RandomFloatInRangeFromStream` 0.0 180.0 (`self.RandomStream`))) (`SplineComponent.GetRotationAtDistanceAlongSpline` _splinecomonentexample _returnvalue "World")))))
    (`StaticMeshComponent.SetStaticMesh` _returnvalue_2 "/Game/3D_Assets/Prison/ChainLink/SM_Prison_ChainLink.SM_Prison_ChainLink")
    (`PrimitiveComponent.SetMaterial` _returnvalue_2 0 null)))