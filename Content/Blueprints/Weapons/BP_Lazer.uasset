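; BP_Lazer is a laser projectile that bounces only off reflective surfaces.
; On each bounce event from its ProjectileMovement component, it checks the hit component for the T_Reflectable tag; without it, the projectile stops and destroys itself.
; Tick resets the actor's rotation to zero every frame after calling the parent.
; The impact particle effect is only a placeholder comment.
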(event `self.ReceiveBeginPlay`
  (`parent.ReceiveBeginPlay`))

(event `self.ReceiveActorBeginOverlap`
  (params (OtherActor :type "Actor Object Reference")))

(event `self.ReceiveTick`
  (params (DeltaSeconds :type "Float (single-precision)"))
  (`parent.ReceiveTick` 0.0)
  (`self.SetActorRotation` (struct)))

(event `self.ProjectileMovement.OnProjectileBounce`
  (params (ImpactResult :type "HitResult Structure (by ref)") (ImpactVelocity :type "Vector Structure (by ref)"))
  ;[1 1 1] A lazer should only 'bounce' against a reflective object. If the hit object is not reflective, stop bouncing, play particle effect, destroy all lazer projectiles.
  (if (not (`KismetArrayLibrary.Array_Contains` (`ActorComponent.ComponentTags` (`.HitComponent` (`GameplayStatics.BreakHitResult` ImpactResult))) (`KismetStringLibrary.Conv_StringToName` "T_Reflectable")))
    (`ProjectileMovementComponent.SetVelocityInLocalSpace` (`self.ProjectileMovement`) (0.0 0.0 0.0))
    (`self.K2_DestroyActor`) ; Put a particle effect before this!
  ))

(fn `UserConstructionScript`
  (`parent.UserConstructionScript`))