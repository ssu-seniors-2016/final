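; Blueprint function library of trace helpers that cast from an actor's location along a given direction for a given length.
; ChannelTraceActorVector runs a line trace by channel and returns the hit, the result flag and the distance from the actor to the hit location.
; ObjectSphereTraceVector sweeps a sphere of given radius against object types and returns only the hit and result flag.
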(fn `Channel Trace Actor Vector`
  (params (Target :type "Actor Object Reference") (Length :type "Float (double-precision)") (TraceChannel :type "ETraceTypeQuery Enum") (ActorsToIgnore :type "Array of Actor Object Reference (by ref)") (DrawDebugType :type "EDrawDebugTrace Enum") (bIgnoreSelf :type Boolean) (bTraceComplex :type Boolean) (Direction :type "Vector Structure"))
  (returns (`Out Length` :type "Float (double-precision)") (OutHit :type "HitResult Structure") (ReturnValue :type Boolean))
  (bind _returnvalue (`Actor.K2_GetActorLocation` Target))
  (bind (_outhit _returnvalue_2) (`KismetSystemLibrary.LineTraceSingle` null _returnvalue (+ (* Direction Length) _returnvalue) TraceChannel bTraceComplex ActorsToIgnore DrawDebugType bIgnoreSelf))
  (return (`KismetMathLibrary.VSize` (- (`.Location` (`GameplayStatics.BreakHitResult` _outhit)) _returnvalue)) _outhit _returnvalue_2))

(fn `Object Sphere Trace Vector`
  (params (Actor :type "Actor Object Reference") (Direction :type "Vector Structure") (Length :type "Float (double-precision)") (ObjectTypes :type "Array of EObjectTypeQuery Enum (by ref)") (bTraceComplex :type Boolean) (ActorsToIgnore :type "Array of Actor Object Reference (by ref)") (DrawDebugType :type "EDrawDebugTrace Enum") (bIgnoreSelf :type Boolean) (Radius :type "Float (double-precision)"))
  (returns (`Return Value` :type Boolean) (OutHit :type "HitResult Structure"))
  (bind _returnvalue (`Actor.K2_GetActorLocation` Actor))
  (bind (_outhit _returnvalue_2) (`KismetSystemLibrary.SphereTraceSingleForObjects` null _returnvalue (+ _returnvalue (* Direction Length)) Radius ObjectTypes bTraceComplex ActorsToIgnore DrawDebugType bIgnoreSelf))
  (return _returnvalue_2 _outhit))