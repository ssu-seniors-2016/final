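; Shield component for BP_MainCharacter that manages a timed, rechargeable energy shield.
; It spawns a Shield actor on the capsule at BeginPlay, and activation and deactivation toggle its visibility and collision.
; Tick drains charge while active, refills it while inactive, and runs a cooldown after depletion.
; Each tick also creates a new dynamic material, scaling green with charge and switching opacity for a brief post-activation reflect window with the upgrade.
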(event `self.ReceiveBeginPlay`
  (`self.Create_Shield`))

(event `self.ReceiveTick`
  (params (DeltaSeconds :type "Float (single-precision)"))
  (bind _maxshieldtime (`self.maxShieldTime`))
  (`self.Update_Shield_Color`)
  (if (`self.isDestroyed`)
    ;[0.02671 0.9235 1] Shield was destroyed, cooldown timer
    (set `self.destroyTimer` (- (`self.destroyTimer`) DeltaSeconds))
    (if (<= (`self.destroyTimer`) 0.0)
      (set `self.isDestroyed` false)
      (set `self.destroyTimer` 5.0)
      (set `self.Shield Timer` (`self.maxShieldTime`)))
    (elif (`self.isShieldActive`)
      ;[0 1 0.07377] Subtracting from shield timer, shield is active
      (set `self.Shield Timer` (- (`self.Shield Timer`) DeltaSeconds))
      (if (<= (`self.Shield Timer`) 0.0)
        (set `self.isDestroyed` true)
        (`self.Deactivate_Shield`)
        (set `self.Shield Timer` 0.0))
      (else
        ;[1 0 0.01801] adding to shield timer, shield if not active
        (set `self.Shield Timer` (+ (`self.Shield Timer`) DeltaSeconds))
        (if (> (`self.Shield Timer`) _maxshieldtime)
          (set `self.Shield Timer` _maxshieldtime))))))

(fn `Activate_Shield`
  (bind _mshield (`self.mShield`))
  (if (`self.Nostartit`)
    (set `self.Nostartit` false)
    (`KismetSystemLibrary.PrintString` "set no start it to false in Activate")
    (else
      (set `self.isShieldActive` true)
      (if (not (`self.isDestroyed`))
        (`SceneComponent.SetVisibility` (`/Game/Blueprints/Shield.DefaultSceneRoot` _mshield) true true)
        (`PrimitiveComponent.SetCollisionEnabled` (`/Game/Blueprints/Shield.Sphere` _mshield) "QueryAndPhysics")
        (set `self.Shield Start Time` (`self.Shield Timer`))))))

(fn `Create_Shield`
  (bind _owner (`self.owner`))
  (bind _capsulecomponent (`Character.CapsuleComponent` (`self.owner`)))
  (bind _asbp_main_character (cast `/Game/Blueprints/Character/BP_MainCharacter` (`self.GetOwner`)))
  (set `self.owner` _asbp_main_character)
  (if (`self.Has Shield`)
    (bind _returnvalue (`|SpawnActorFromClass` "/Game/Blueprints/Shield.Shield_C" (`KismetMathLibrary.Conv_VectorToTransform` (`Actor.K2_GetActorLocation` _owner)) "AlwaysSpawn" "OverrideRootScale" null _owner))
    (set `self.mShield` _returnvalue)
    (`PrimitiveComponent.IgnoreActorWhenMoving` _capsulecomponent _returnvalue true)
    (`SceneComponent.K2_AttachTo` (`/Game/Blueprints/Shield.DefaultSceneRoot` _returnvalue) _capsulecomponent "None" "KeepWorldPosition" false)
    (`self.Deactivate_Shield`)))

(fn `Deactivate_Shield`
  (bind _mshield (`self.mShield`))
  (if (`self.isShieldActive`)
    (set `self.isShieldActive` false)
    (`SceneComponent.SetVisibility` (`/Game/Blueprints/Shield.DefaultSceneRoot` _mshield) false true)
    (`PrimitiveComponent.SetCollisionEnabled` (`/Game/Blueprints/Shield.Sphere` _mshield) "NoCollision")
    (elif (`self.isDestroyed`)
      _
      (elif (not (`self.Nostartit`))
        (set `self.Nostartit` true)
        (`KismetSystemLibrary.PrintString` "Set no start it to true in deactivate")))))

(fn `Update_Shield_Color`
  (bind (_r _g _b _a) (`KismetMathLibrary.BreakColor` (`self.Shield Color`)))
  (bind _returnvalue (`KismetMaterialLibrary.CreateDynamicMaterialInstance` "/Game/Particles/Materials/M_Shield.M_Shield"))
  (set `self.Shield Color` (`KismetMathLibrary.MakeColor` _r (* (`self.Max Green`) (/ (`self.Shield Timer`) (`self.maxShieldTime`))) _b _a))
  (`MaterialInstanceDynamic.SetVectorParameterValue` _returnvalue "Base_Color" (`self.Shield Color`))
  (if (`/Game/Blueprints/Character/BP_MainCharacter.Has Shield Upgrade` (`self.owner`))
    (bind _output_get (set `self.Is Not Reflecting` (< (`self.Shield Timer`) (- (`self.Shield Start Time`) 0.2))))
    (if _output_get
      (`MaterialInstanceDynamic.SetScalarParameterValue` _returnvalue "Opacity" (`self.Regular Opacity`) :!label _label)
      (else
        (`MaterialInstanceDynamic.SetScalarParameterValue` _returnvalue "Opacity" (`self.Upgrade Opacity`))))
    (else
      (goto _label)))
  (`/Game/Blueprints/Shield.Set Material` (`self.mShield`) _returnvalue))