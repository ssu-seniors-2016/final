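; Gun component that lets its owning actor fire bullets from a list of types, starting with BP_Lazer.
; FireBullet spawns the selected bullet slightly ahead of the owner along the given direction, rotated by an offset against owner velocity that an author note marks as not working.
; A successful spawn blocks firing for a delay that ChangeBulletType reads from the bullet class's default Firerate.
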(event `self.ReceiveBeginPlay`
  (set `self.Owner` (`self.GetOwner`))
  (`self.Change Bullet Type` "/Game/Blueprints/Weapons/BP_Lazer.BP_Lazer_C"))

(event `self.ReceiveTick`
  (params (DeltaSeconds :type "Float (single-precision)")))

(event `Firerate Delay`
  (`KismetSystemLibrary.Delay` (`self.Firerate`))
  (set `self.Can Fire?` true))

(fn `Change Bullet Type`
  (params (`New Bullet Class` :type "/Game/Blueprints/Bullet Class Reference"))
  ;[1 1 1] Eventually, this needs to handle switching our current bullet type on GUI input. - Don
  (bind _output_get (set `self.Bullet Selection Index` (`KismetArrayLibrary.Array_Find` (`self.BulletTypes`) `New Bullet Class`)))
  (set `self.Firerate` (`.Firerate` (defaults `/Game/Blueprints/Character/AC_GunComponent` (`KismetArrayLibrary.Array_Get` (`self.BulletTypes`) _output_get)))))

(fn `Fire Bullet`
  (params (Direction :type "Vector Structure"))
  (bind _owner (`self.Owner`))
  (if (`self.Can Fire?`)
    (set `self.Can Fire?` false)
    (bind _returnvalue (`|SpawnActorFromClass` (`KismetArrayLibrary.Array_Get` (`self.BulletTypes`) (`self.Bullet Selection Index`)) (`KismetMathLibrary.MakeTransform` (+ (* Direction 50.0) (`Actor.K2_GetActorLocation` _owner)) (`KismetMathLibrary.MakeRotationFromAxes` (`KismetMathLibrary.Normal` (+ Direction (* (`Actor.GetVelocity` _owner) -1.0))) (`Actor.GetActorRightVector` _owner) (`Actor.GetActorUpVector` _owner))) "AlwaysSpawn" "OverrideRootScale" (`self.Owner`) Direction))
    (`/Engine/EditorBlueprintResources/StandardMacros.IsValid` _returnvalue
      (:`Is Valid`
        (`self.Firerate Delay`))
      (:`Is Not Valid`
        (set `self.Can Fire?` true)))))