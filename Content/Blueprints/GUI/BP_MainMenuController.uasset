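; BP_MainMenuController is the main menu's player controller, spawning the title screen widget and managing input for it.
; On BeginPlay it checks the save game count, disabling Continue and Load and focusing New Game when none exist, otherwise focusing Continue.
; Menu up/down key types and mouse movement toggle a controller-usage flag and cursor visibility, while cancel is forwarded to the title screen.
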(event `self.ReceiveTick`
  (params (DeltaSeconds :type "Float (single-precision)")))

(event `self.ReceiveBeginPlay`
  (bind _titlescreen (`self.TitleScreen`))
  (bind _continue_button (`/Game/Blueprints/GUI/Widgets/BPW_TitleScreen.Continue Button` _titlescreen))
  (bind _returnvalue (`|CreateWidget` "/Game/Blueprints/GUI/Widgets/BPW_TitleScreen.BPW_TitleScreen_C" self))
  (`UserWidget.AddToViewport` _returnvalue 0)
  (set `self.TitleScreen` _returnvalue)
  (bind _newparam (`/Game/Blueprints/GUI/BPL_SaveGameFunctions.CheckSaveGameCount`))
  (set `self.Save Game Count` _newparam)
  (if (== _newparam 0)
    (`Widget.SetIsEnabled` _continue_button false)
    (`Widget.SetIsEnabled` (`/Game/Blueprints/GUI/Widgets/BPW_TitleScreen.Load Button` _titlescreen) false)
    (`Widget.SetKeyboardFocus` (`/Game/Blueprints/GUI/Widgets/BPW_TitleScreen.New Game Button` _titlescreen))
    (else
      (`Widget.SetKeyboardFocus` _continue_button))))

(event `InputAction|MenuUp`
  (params (Key :type "Key Structure" :default "AnyKey"))
  (:`Pressed`
    (`self.Switch Control Type` Key)))

(event `InputAction|MenuCancel`
  (params (Key :type "Key Structure" :default "AnyKey"))
  (:`Pressed`
    (`/Game/Blueprints/GUI/Widgets/BPW_TitleScreen.Cancel Button Pressed` (`self.TitleScreen`))))

(event `InputAction|MenuDown`
  (params (Key :type "Key Structure" :default "AnyKey"))
  (:`Pressed`
    (`self.Switch Control Type` Key)))

(event `InputAxisKey|MouseX`
  (params (AxisValue :type "Float (single-precision)"))
  (if (!= AxisValue 0.0)
    (if (`self.Using Controller`) :!label _label
      (set `self.bShowMouseCursor` true)
      (set `self.Using Controller` false))))

(event `InputAxisKey|MouseY`
  (params (AxisValue :type "Float (single-precision)"))
  (if (!= AxisValue 0.0)
    (goto _label)))

(fn `UserConstructionScript`)