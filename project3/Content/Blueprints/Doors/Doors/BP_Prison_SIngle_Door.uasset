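; Prison single door Blueprint with sliding left, right and bottom panels set in a wall and frame.
; The construction script applies configurable meshes and a wall material, then caches each panel's relative location as its closed position.
; Every Tick polls OpenSesame to play or reverse the DoorOpener timeline, which offsets the panels from those closed positions.
; The file only reads OpenSesame and never sets it.
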(event `self.ReceiveBeginPlay`
  (`parent.ReceiveBeginPlay`))

(event `self.ReceiveTick`
  (params (DeltaSeconds :type "Float (single-precision)"))
  (`parent.ReceiveTick` 0.0)
  (if (`self.OpenSesame`)
    (bind (_direction _door_right_location _door_left_location _door_bottom_location) (`Timeline|DoorOpener` :!label _label)
      (:`Update`
        (`SceneComponent.K2_SetRelativeLocation` (`self.DoorRight`) (+ _door_right_location (`self.DoorRightClosed`)) false false)
        (`SceneComponent.K2_SetRelativeLocation` (`self.DoorLeft`) (+ _door_left_location (`self.DoorLeftClosed`)) false false)
        (`SceneComponent.K2_SetRelativeLocation` (`self.DoorBottom`) (+ _door_bottom_location (`self.DoorBottomClosed`)) false false)))
    (else
      (goto _label :!via `Reverse`))))

(fn `UserConstructionScript`
  (bind _wall (`self.Wall`))
  (`parent.UserConstructionScript`)
  (`StaticMeshComponent.SetStaticMesh` (`self.DoorLeft`) (`self.DoorLeftMesh`))
  (`StaticMeshComponent.SetStaticMesh` (`self.DoorRight`) (`self.DoorRightMesh`))
  (`StaticMeshComponent.SetStaticMesh` (`self.DoorBottom`) (`self.DoorBottomMesh`))
  (`StaticMeshComponent.SetStaticMesh` _wall (`self.WallMesh`))
  (`PrimitiveComponent.SetMaterial` _wall 0 (`self.WallMaterial`))
  (`StaticMeshComponent.SetStaticMesh` (`self.DoorFrame`) (`self.DoorFrameMesh`))
  (set `self.DoorRightClosed` (`SceneComponent.RelativeLocation` (`self.DoorRight`)))
  (set `self.DoorLeftClosed` (`SceneComponent.RelativeLocation` (`self.DoorLeft`)))
  (set `self.DoorBottomClosed` (`SceneComponent.RelativeLocation` (`self.DoorBottom`))))