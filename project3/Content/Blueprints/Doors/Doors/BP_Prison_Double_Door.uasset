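; Prison double door actor that slides open and rotates its lock while a flag is set, and reverses when it is cleared.
; Construction script applies configurable meshes and doorway material, then caches the closed position and lock rotation.
; Tick polls OpenSesame to drive the DoorOpener timeline, which offsets both from those cached values.
; Optional flags hide the sliding door or the whole frame hierarchy at BeginPlay.
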(event `self.ReceiveBeginPlay`
  (`parent.ReceiveBeginPlay`)
  (if (`self.Hide?`)
    (if (`self.EverythingHidden?`)
      (`SceneComponent.SetHiddenInGame` (`self.Door_Frame`) true true)
      (else
        (`SceneComponent.SetHiddenInGame` (`self.Sliding_Door`) true false)))))

(event `self.ReceiveTick`
  (params (DeltaSeconds :type "Float (single-precision)"))
  (`parent.ReceiveTick` DeltaSeconds)
  (if (`self.OpenSesame`)
    (bind (_direction _lockrotation _doorlocation) (`Timeline|DoorOpener` :!label _label)
      (:`Update`
        (`SceneComponent.K2_SetRelativeLocation` (`self.Sliding_Door`) (+ _doorlocation (`self.DoorClosed`)) false false)
        (`SceneComponent.K2_SetRelativeRotation` (`self.Door_Lock`) (`KismetMathLibrary.MakeRotator` (.roll (`self.DoorLockRotator`)) (+ _lockrotation (`self.LockStart`)) (.yaw (`self.DoorLockRotator`))) false false)))
    (else
      (goto _label :!via `Reverse`))))

(fn `UserConstructionScript`
  (bind _relativerotation (`SceneComponent.RelativeRotation` (`self.Door_Lock`)))
  (`parent.UserConstructionScript`)
  (`StaticMeshComponent.SetStaticMesh` (`self.Door_Frame`) (`self.Door Frame Mesh`))
  (`StaticMeshComponent.SetStaticMesh` (`self.Sliding_Door`) (`self.Sliding Door Mesh`))
  (`StaticMeshComponent.SetStaticMesh` (`self.Doorway1`) (`self.Doorway1 Mesh`))
  (`StaticMeshComponent.SetStaticMesh` (`self.Doorway2`) (`self.Doorway2 Mesh`))
  (`StaticMeshComponent.SetStaticMesh` (`self.Door_Lock`) (`self.Door Lock Mesh`))
  (`StaticMeshComponent.SetStaticMesh` (`self.Wall_Half1`) (`self.Wall Half1 Mesh`))
  (`StaticMeshComponent.SetStaticMesh` (`self.Wall_Half2`) (`self.Wall Half2 Mesh`))
  (`PrimitiveComponent.SetMaterial` (`self.Doorway1`) 0 (`self.Doorway1 Material`))
  (`PrimitiveComponent.SetMaterial` (`self.Doorway2`) 0 (`self.Doorway1 Material`))
  (set `self.DoorClosed` (`SceneComponent.RelativeLocation` (`self.Sliding_Door`)))
  (set `self.DoorLockRotator` _relativerotation)
  (set `self.LockStart` (.pitch _relativerotation)))