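; BP_Door is a proximity door that tracks whether it should be open through an OpenSesame flag.
; A BP_MainCharacter entering the Box trigger sets the flag, and it clears once no main character still overlaps the box.
; While Locked is true, Tick forces the flag back to false.
; The construction script sizes the trigger's Y extent from Distance; this graph contains no door movement itself.
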(event `self.ReceiveTick`
  (params (DeltaSeconds :type "Float (single-precision)"))
  (if (`self.Locked`)
    (set `self.OpenSesame` false)))

(event `self.Box.OnComponentBeginOverlap`
  (params (OtherActor :type "Actor Object Reference") (OtherComp :type "PrimitiveComponent Object Reference") (OtherBodyIndex :type Integer) (bFromSweep :type Boolean) (SweepResult :type "HitResult Structure (by ref)"))
  (cast `/Game/Blueprints/Character/BP_MainCharacter` OtherActor)
  (set `self.OpenSesame` true))

(event `self.ReceiveActorEndOverlap`
  (params (OtherActor :type "Actor Object Reference"))
  (if (== (`KismetArrayLibrary.Array_Length` (`PrimitiveComponent.GetOverlappingActors` (`self.Box`) "/Game/Blueprints/Character/BP_MainCharacter.BP_MainCharacter_C")) 0)
    (set `self.OpenSesame` false)))

(fn `UserConstructionScript`
  (bind _box (`self.Box`))
  (`BoxComponent.SetBoxExtent` _box (`KismetMathLibrary.MakeVector` (.x (`BoxComponent.BoxExtent` _box)) (`self.Distance`) (.z (`BoxComponent.BoxExtent` _box))) true))