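; Editor-style helper actor that lines up other level actors on a shared world X or Y coordinate.
; Its Construction Script teleports every actor of the classes in ClassesToAlign, plus those in OtherActorsToAlign, to AlignmentPosition on one axis, keeping the other two coordinates.
; AlignOnYAxis true sets X, forming a line along Y; false sets Y.
; The event graph has no active logic.
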(event `self.ReceiveBeginPlay`)

(event `self.ReceiveActorBeginOverlap`
  (params (OtherActor :type "Actor Object Reference")))

(event `self.ReceiveTick`
  (params (DeltaSeconds :type "Float (single-precision)")))

(fn `UserConstructionScript`
  (bind _alignment_position (`self.Alignment Position`))
  (bind _alignment_position_2 (`self.Alignment Position`))
  (for _array_element (`self.Classes to Align`)
    (bind _outactors (`GameplayStatics.GetAllActorsOfClass` _array_element))
    (for _array_element_2 _outactors
      (bind _z (.z (`self.K2_GetActorLocation` _array_element_2)))
      (`self.K2_SetActorLocation` _array_element_2 (`KismetMathLibrary.SelectVector` (`KismetMathLibrary.MakeVector` _alignment_position_2 (.y (`self.K2_GetActorLocation` _array_element_2)) _z) (`KismetMathLibrary.MakeVector` (.x (`self.K2_GetActorLocation` _array_element_2)) _alignment_position_2 _z) (`self.Align on Y axis?`)) false true)))
  (for _array_element_3 (`self.Other Actors to Align`)
    (bind _z_2 (.z (`self.K2_GetActorLocation` _array_element_3)))
    (`self.K2_SetActorLocation` _array_element_3 (`KismetMathLibrary.SelectVector` (`KismetMathLibrary.MakeVector` _alignment_position (.y (`self.K2_GetActorLocation` _array_element_3)) _z_2) (`KismetMathLibrary.MakeVector` (.x (`self.K2_GetActorLocation` _array_element_3)) _alignment_position _z_2) (`self.Align on Y axis?`)) false true)))