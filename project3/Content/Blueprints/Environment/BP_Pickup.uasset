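; BP_Pickup is an environment pickup that reacts when the main character overlaps its collision box.
; On overlap it casts the other actor to BP_MainCharacter and calls the PickedUp dispatcher with that character, leaving the pickup's effect to whatever is bound.
; The construction script creates dynamic materials for the light cone and item capsule meshes, tinting both from one Color variable.
; BeginPlay only runs a delay with nothing after it.
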(event `self.ReceiveBeginPlay`
  (`KismetSystemLibrary.Delay` 1.0))

(event `self.Pickup_Collbox.OnComponentBeginOverlap`
  (params (OtherActor :type "Actor Object Reference") (OtherComp :type "PrimitiveComponent Object Reference") (OtherBodyIndex :type Integer) (bFromSweep :type Boolean) (SweepResult :type "HitResult Structure (by ref)"))
  (bind _asbp_main_character (cast `/Game/Blueprints/Character/BP_MainCharacter` OtherActor))
  (`self.Picked Up` _asbp_main_character))

(fn `UserConstructionScript`
  (bind _color (`self.Color`))
  (bind _returnvalue (`PrimitiveComponent.CreateDynamicMaterialInstance` (`self.AnotherMesh`) 0 "/Game/3D_Assets/Prison/LightCone/MI_LightCone_White.MI_LightCone_White"))
  (`MaterialInstanceDynamic.SetVectorParameterValue` _returnvalue "Color" _color)
  (bind _returnvalue_2 (`PrimitiveComponent.CreateDynamicMaterialInstance` (`self.Item_Type_Mesh`) 0 "/Game/3D_Assets/Weapons/ItemCapsule/MI_Item_Capsule.MI_Item_Capsule"))
  (`MaterialInstanceDynamic.SetVectorParameterValue` _returnvalue_2 "Glow Color" _color))