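; BP_Weapon_Pickup is a timed pickup that unlocks its BulletClass on the collecting player's ACGunComponent, then destroys itself.
; BeginPlay binds the PickedUp event, which is guarded to fire once, and sets a timer for 80% of InitialLifeSpan.
; That timer starts a self-rescheduling function that blinks the Icon increasingly fast as expiry nears.
; An icon-bobbing Timeline exists but is never triggered.
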(event `Picked Up_Event_0` :!signature `self.Picked Up`
  (params (Player :type "/Game/Blueprints/Character/BP_MainCharacter Object Reference"))
  (bind _bullet_class (`self.Bullet Class`))
  (`/Engine/EditorBlueprintResources/StandardMacros.DoOnce` false
    (:`Completed`
      (`KismetSystemLibrary.PrintString` (`KismetSystemLibrary.GetClassDisplayName` _bullet_class))
      (`/Game/Blueprints/Character/AC_GunComponent.Unlock Bullet` (`/Game/Blueprints/Character/BP_MainCharacter.AC_GunComponent` Player) _bullet_class)
      (`self.K2_DestroyActor`))))

(event `self.ReceiveBeginPlay`
  (bind _returnvalue (* (`self.InitialLifeSpan`) 0.8))
  (add `self.Picked Up` (delegate `Picked Up_Event_0`))
  (set `self.Life Time` _returnvalue)
  (`KismetSystemLibrary.K2_SetTimer` null "Running Out of Time" _returnvalue))

(event `self.ReceiveBeginPlay`)

(event `self.ReceiveActorBeginOverlap`
  (params (OtherActor :type "Actor Object Reference")))

(event `self.ReceiveTick`
  (params (DeltaSeconds :type "Float (single-precision)")))

(fn `Running Out of Time`
  (bind _icon (`self.Icon`))
  (bind _returnvalue (`SceneComponent.IsVisible` _icon))
  (bind _returnvalue_2 (/ (`self.Life Time`) (`self.InitialLifeSpan`)))
  (bind _returnvalue_3 (`KismetMathLibrary.SelectFloat` 0.1 (`KismetMathLibrary.SelectFloat` 0.3 0.5 (> _returnvalue_2 0.85)) (> _returnvalue_2 0.9)))
  (set `self.Life Time` (+ (`self.Life Time`) _returnvalue_3))
  (`SceneComponent.SetVisibility` _icon (not _returnvalue) true)
  (`KismetSystemLibrary.K2_SetTimer` null "Running Out of Time" (`KismetMathLibrary.SelectFloat` _returnvalue_3 0.1 _returnvalue)))

(fn `UserConstructionScript`
  (`parent.UserConstructionScript`))