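; BP_RootDoors is a root door that opens the way when stunned.
; It always reports that it can be stunned, and the first GetStunned event destroys its Cube component, guarded by a DoOnce.
; For visuals only, the construction script adds an unattached static mesh just under 200 units below the root's world location when Hidden is set.
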(event `/Game/Blueprints/Character/BPI_StunInterface.GetStunned`
  (params (Stunner :type "Actor Object Reference"))
  (`/Engine/EditorBlueprintResources/StandardMacros.DoOnce` false
    (:`Completed`
      (`ActorComponent.K2_DestroyComponent` (`self.Cube`)))))

(fn `CanBeStunned`
  (returns (`Yes?` :type Boolean))
  (return true))

(fn `UserConstructionScript`
  ;[1 1 1] This is just for visuals
  (if (`self.Hidden`)
    (`AddComponent|Static Mesh Component_162` :`bManualAttachment` true :`RelativeTransform` (`KismetMathLibrary.MakeTransform` (`KismetMathLibrary.MakeVector` (.x (`SceneComponent.K2_GetComponentLocation` (`self.DefaultSceneRoot`))) (.y (`SceneComponent.K2_GetComponentLocation` (`self.DefaultSceneRoot`))) (- (.z (`SceneComponent.K2_GetComponentLocation` (`self.DefaultSceneRoot`))) 199.5))))))