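; BP_LaserGate is a hazard gate that groups several BP_WallLaser child actors into one switchable barrier.
; The construction script collects the wall lasers from child actor components under Lasers into LaserArray.
; On BeginPlay, each laser adds the gate to its ignore list, disables collision on its Node and receives a base damage value.
; Toggle flips every laser and the gate's Box collision together, tracked by TurnedOn.
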(event `self.ReceiveBeginPlay`
  (for _array_element (`self.Laser Array`)
    (`KismetArrayLibrary.Array_Add` (`/Game/Blueprints/Environment/Hazards/Lazer/BP_WallLaser.IgnorePlayer` _array_element) self)
    (`PrimitiveComponent.SetCollisionEnabled` (`/Game/Blueprints/Environment/Hazards/Lazer/BP_WallLaser.Node` _array_element) "NoCollision")
    (set `/Game/Blueprints/Environment/Hazards/Lazer/BP_WallLaser.BaseDamage` 15.0 _array_element)))

(fn `Toggle`
  (`PrimitiveComponent.SetCollisionEnabled` (`self.Box`) (select `bool` (`self.Turned On?`) :`false` "QueryAndPhysics" :`true` "NoCollision" :!type "ECollisionEnabled Enum"))
  (for _array_element (`self.Laser Array`)
    (`/Game/Blueprints/Environment/Hazards/Lazer/BP_WallLaser.ToggleLasers` _array_element))
  (set `self.Turned On?` (not (`self.Turned On?`))))

(fn `UserConstructionScript`
  (for _array_element (`SceneComponent.GetChildrenComponents` (`self.Lasers`) false)
    (bind _aschild_actor_component (cast `ChildActorComponent` _array_element))
    (bind _asbp_wall_laser (cast `/Game/Blueprints/Environment/Hazards/Lazer/BP_WallLaser` (`ChildActorComponent.ChildActor` _aschild_actor_component)))
    (`KismetArrayLibrary.Array_AddUnique` (`self.Laser Array`) _asbp_wall_laser)))