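; BP_Electrified_Water is an environmental hazard that damages characters while they stand in it.
; Begin and end overlap events add or remove overlapping Characters from an ActorsToDamage list.
; Tick applies BP_ContactDamage to every listed actor, scaling a DPS value by delta time for continuous damage.
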(event `self.ReceiveTick`
  (params (DeltaSeconds :type "Float (single-precision)"))
  (for _array_element (`self.ActorsToDamage`)
    (`GameplayStatics.ApplyDamage` _array_element (* DeltaSeconds (`self.DPS`)) null self "/Game/Blueprints/Character/BP_ContactDamage.BP_ContactDamage_C")))

(event `self.ReceiveActorBeginOverlap`
  (params (OtherActor :type "Actor Object Reference"))
  (bind _ascharacter (cast `Character` OtherActor))
  (`KismetArrayLibrary.Array_Add` (`self.ActorsToDamage`) _ascharacter))

(event `self.ReceiveActorEndOverlap`
  (params (OtherActor :type "Actor Object Reference"))
  (bind _ascharacter (cast `Character` OtherActor))
  (`KismetArrayLibrary.Array_RemoveItem` (`self.ActorsToDamage`) _ascharacter))

(fn `UserConstructionScript`)