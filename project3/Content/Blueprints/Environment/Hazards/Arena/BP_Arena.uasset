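; BP_Arena is a one-shot combat arena that locks its BP_Doors when its trigger box is first overlapped and unlocks them once all enemies are dead.
; It cycles through SpawnArray, spawning an enemy from each unfinished spawner with a delay between spawns, until all report done.
; A delayed polling loop then checks each spawner's enemy count, removing cleared spawners from the array until it empties.
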(event `self.TriggerBox.OnComponentBeginOverlap`
  (params (OtherActor :type "Actor Object Reference") (OtherComp :type "PrimitiveComponent Object Reference") (OtherBodyIndex :type Integer) (bFromSweep :type Boolean) (SweepResult :type "HitResult Structure (by ref)"))
  (bind _item (`KismetArrayLibrary.Array_Get` (`self.SpawnArray`) (`self.index`)))
  (bind _item_2 (`KismetArrayLibrary.Array_Get` (`self.SpawnArray`) (`self.index`)))
  (`/Engine/EditorBlueprintResources/StandardMacros.DoOnce` false
    (:`Completed`
      ;[1 1 1] Locking Doors
      (for _array_element (`self.DoorArray`)
        (bind _asbp_door (cast `/Game/Blueprints/Doors/Doors/BP_Door` _array_element))
        (set `/Game/Blueprints/Doors/Doors/BP_Door.Locked` true _asbp_door))
      ;[1 1 1] Checking if Spawns are Complete
      (set `self.StillSpawning` false :!label _label)
      (for _array_element_2 (`self.SpawnArray`)
        (if (not (`/Game/Blueprints/Environment/Hazards/Arena/BP_SpawnPoint.doneSpawning` _array_element_2))
          (set `self.StillSpawning` true)))
      ;[1 1 1] Spawning Enemies
      (if (`self.StillSpawning`)
        (if (< (`self.index`) (`KismetArrayLibrary.Array_Length` (`self.SpawnArray`))) :!label _label_2
          (if (`/Game/Blueprints/Environment/Hazards/Arena/BP_SpawnPoint.doneSpawning` _item)
            (`/Engine/EditorBlueprintResources/StandardMacros.IncrementInt` (`self.index`)
              (:`  `
                (goto _label_2)))
            (else
              (`/Game/Blueprints/Environment/Hazards/Arena/BP_SpawnPoint.Spawn Enemy` _item)
              (`/Engine/EditorBlueprintResources/StandardMacros.IncrementInt` (`self.index`)
                (:`  `
                  (`KismetSystemLibrary.Delay` (`self.SpawnTime`))
                  (goto _label_2)))))
          (else
            (set `self.index` 0)
            (goto _label)))
        (else
          ;[1 1 1] Ugly Stuff. Shield your eyes
          (if (<= (`KismetArrayLibrary.Array_Length` (`self.SpawnArray`)) 0) :!label _label_3
            (for _array_element_3 (`self.DoorArray`)
              (bind _asbp_door_2 (cast `/Game/Blueprints/Doors/Doors/BP_Door` _array_element_3))
              (set `/Game/Blueprints/Doors/Doors/BP_Door.Locked` false _asbp_door_2)
              (`KismetSystemLibrary.PrintString` "unlocked"))
            (else
              (if (< (`self.index`) (`KismetArrayLibrary.Array_Length` (`self.SpawnArray`))) :!label _label_4
                (`KismetSystemLibrary.Delay` 0.1)
                (`/Game/Blueprints/Environment/Hazards/Arena/BP_SpawnPoint.CheckEnemyCount` _item_2)
                (if (`/Game/Blueprints/Environment/Hazards/Arena/BP_SpawnPoint.AllEnemiesDead` _item_2)
                  (`KismetArrayLibrary.Array_RemoveItem` (`self.SpawnArray`) _item_2)
                  (set `self.index` 0)
                  (goto _label_4)
                  (else
                    (`/Engine/EditorBlueprintResources/StandardMacros.IncrementInt` (`self.index`)
                      (:`  `
                        (goto _label_4)))))
                (else
                  (set `self.index` 0)
                  (goto _label_3))))))))))

(fn `UserConstructionScript`)