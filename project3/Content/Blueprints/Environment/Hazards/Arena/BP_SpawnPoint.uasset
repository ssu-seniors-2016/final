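; Arena spawn point that spawns queued enemies at its root location and reports when they are all dead.
; Each SpawnEnemy call spawns the first class in EnemyList, gives it a default controller, and flags DoneSpawning once the list empties.
; Spiders spawn yawed 90 degrees, and floating mobs receive a patrol location indexed by spawn count.
; CheckEnemyCount adds invalid EnemyArray references to DeadEnemies without resetting it, setting AllEnemiesDead when that equals EnemyCount.
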(fn ConstructionScript)

(fn SpawnEnemy
  (bind _enemylist (Variables|Default|GetEnemyList))
  (bind _item (Utilities|Array|Get(acopy) _enemylist))
  (if (not (< (Utilities|Array|Length _enemylist) 1))
    (bind _returnvalue (Game|SpawnActorfromClass _item (Math|Transform|MakeTransform (Transformation|GetWorldLocation (Variables|Default|GetDefaultSceneRoot)) (select (== _item "/Game/Blueprints/Mobs/BP_Spider.BP_Spider_C") (Math|Rotator|MakeRotator 0.0 0.0 9e+01) (Math|Rotator|MakeRotator 0.0 0.0 0.0)) "1.000000,1.000000,1.000000") "AlwaysSpawn" 0 0))
    (Utilities|Array|Add (Variables|Default|GetEnemyArray) _returnvalue)
    (if (not (== _item "/Game/Blueprints/Mobs/BP_FloatingMob.BP_FloatingMob_C"))
      _
      (else
        (bind _asbp_floating_mob (Utilities|Casting|CastToBP_FloatingMob _returnvalue))
        (Default|ChangePatrolLocation _asbp_floating_mob (Utilities|Array|Get(acopy) (Variables|Default|GetPatrol%20Location) (Variables|Default|GetEnemyCount)))))
    (Pawn|SpawnDefaultController _returnvalue)
    (Variables|Default|SetEnemyCount (+ (Variables|Default|GetEnemyCount) 1))
    (Utilities|Array|RemoveIndex (Variables|Default|GetEnemyList))
    (if (< (Utilities|Array|Length (Variables|Default|GetEnemyList)) 1)
      (Variables|Default|SetdoneSpawning true))))

(fn CheckEnemyCount
  (for _array_element (Variables|Default|GetEnemyArray)
    (Utilities|IsValid _array_element
      (:Is%20Not%20Valid
        (LocalVariables|SetDeadEnemies (+ (LocalVariables|GetDeadEnemies) 1)))))
  ;[1 1 1] If all enemies are dead, set the all enemies are dead bool
  (if (== (Variables|Default|GetEnemyCount) (LocalVariables|GetDeadEnemies))
    (Variables|Default|SetAllEnemiesDead true)))