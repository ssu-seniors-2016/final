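; BP_FallingLava is an environment hazard that pours lava on and off in a repeating cycle.
; On BeginPlay, a timeline sized by LavafallTime acts as a looping timer, toggling the PPouringLava component each time it finishes and then restarting.
; The construction script scales PPouringLava by a multiplier.
; Separate functions toggle the pour or destroy the Lava component, though neither is called within this Blueprint.
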(event `self.ReceiveBeginPlay`
  (`TimelineComponent.SetTimelineLength` (`self.LavaTimer`) (`self.LavafallTime`))
  (`Timeline|LavaTimer` :!label _label
    (:`Finished`
      (`ActorComponent.ToggleActive` (`self.P_Pouring_Lava`))
      (goto _label :!via `PlayFromStart`))))

(fn `Create Lava`
  (`ActorComponent.ToggleActive` (`self.P_Pouring_Lava`)))

(fn `LavaNONO`
  (`ActorComponent.K2_DestroyComponent` (`self.Lava`)))

(fn `UserConstructionScript`
  (bind _p_pouring_lava (`self.P_Pouring_Lava`))
  (`SceneComponent.SetRelativeScale3D` _p_pouring_lava (* (`SceneComponent.RelativeScale3D` _p_pouring_lava) (`self.ScaleMultplier`))))