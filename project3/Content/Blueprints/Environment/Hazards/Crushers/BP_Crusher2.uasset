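; BP_Crusher2 is a crusher hazard that moves along a Timeline-driven lerp between StartPos and EndPos and deals lethal-scale damage to the main character.
; It runs either once per player overlap of TriggerBox, or repeatedly from Tick when RunContinuosly is set.
; HasActivated guards against restarting mid-cycle and clears when the Timeline finishes.
; A separate Box overlap applies the damage to BP_MainCharacter.
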(event `self.ReceiveActorBeginOverlap`
  (params (OtherActor :type "Actor Object Reference")))

(event `self.TriggerBox.OnComponentBeginOverlap`
  (params (OtherActor :type "Actor Object Reference") (OtherComp :type "PrimitiveComponent Object Reference") (OtherBodyIndex :type Integer) (bFromSweep :type Boolean) (SweepResult :type "HitResult Structure (by ref)"))
  ;[0 0.01084 1] Move Crusher
  (if (`self.Run_Continuosly`)
    _
    (elif (`self.Has_Activated`)
      _
      (elif (== "/Game/Blueprints/Character/BP_MainCharacter.BP_MainCharacter_C" (`GameplayStatics.GetObjectClass` OtherActor))
        (bind (_direction _alpha) (`Timeline|Timeline` :!via `PlayFromStart` :!label _label)
          (:`Update`
            (set `self.Has_Activated` true)
            (`SceneComponent.K2_SetWorldLocation` (`self.Crusher`) (`KismetMathLibrary.VLerp` (`SceneComponent.K2_GetComponentLocation` (`self.Start_Pos`)) (`SceneComponent.K2_GetComponentLocation` (`self.End_Pos`)) _alpha) false false))
          (:`Finished`
            (set `self.Has_Activated` false)))))))

(event `self.ReceiveTick`
  (params (DeltaSeconds :type "Float (single-precision)"))
  ;[0 0.01084 1] Move Crusher
  (if (`self.Run_Continuosly`)
    (if (`self.Has_Activated`)
      (goto _label)
      (else
        (goto _label :!via `PlayFromStart`)))))

(event `self.Box.OnComponentBeginOverlap`
  (params (OtherActor :type "Actor Object Reference") (OtherComp :type "PrimitiveComponent Object Reference") (OtherBodyIndex :type Integer) (bFromSweep :type Boolean) (SweepResult :type "HitResult Structure (by ref)"))
  ;[0.7783 1 0] Crusher Hit Detection
  (bind _asbp_main_character (cast `/Game/Blueprints/Character/BP_MainCharacter` OtherActor))
  (`GameplayStatics.ApplyDamage` _asbp_main_character 1000.0 null null "/Game/Blueprints/Character/BP_DamageTypeBasic.BP_DamageTypeBasic_C"))

(fn `UserConstructionScript`)