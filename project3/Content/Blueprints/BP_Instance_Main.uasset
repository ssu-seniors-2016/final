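; BP_Instance_Main, apparently the game instance, handles level transitions for new games, Versus matches and returning to the main menu.
; A new game writes a fresh save to the chosen slot, then opens PRISON.
; Versus stores players, match style and rules from the menu before opening the selected map.
; Called during Versus, it removes extra local players and cycles to the next map; returning to menu also removes them.
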(fn `Return to Main Menu`
  (for _index (range 1 4)
    (bind _returnvalue (`GameplayStatics.GetPlayerController` _index))
    (`/Engine/EditorBlueprintResources/StandardMacros.IsValid` _returnvalue
      (:`Is Valid`
        (`GameplayStatics.RemovePlayer` _returnvalue))))
  (`GameplayStatics.OpenLevel` "MainMenu"))

(fn `Start New Versus`
  (bind _returnvalue (`GameplayStatics.GetGameMode`))
  (bind _map_name (`self.Map Name`))
  (bind _map_selection_index (`self.Map Selection Index`))
  (bind _asbp_main_menu_mode (cast `/Game/Blueprints/GameModes/MainMenu/BP_MainMenuMode` _returnvalue)
    (:`then`
      (bind _asbp_main_menu_controller (cast `/Game/Blueprints/GameModes/MainMenu/BP_MainMenuController` (`GameplayStatics.GetPlayerController` 0)))
      (bind _output_get (set `self.Players In Versus Match` (`/Game/Blueprints/GameModes/MainMenu/BP_MainMenuMode.PlayersInGame` _asbp_main_menu_mode)))
      (for (_array_element _array_index) _output_get
        (if _array_element
          (`KismetSystemLibrary.PrintString` (`KismetStringLibrary.Concat_StrStr` "Player " (`KismetStringLibrary.Conv_IntToString` _array_index) " is ready") false false (struct :`R` 0.062356 :`G` 1.0 :`A` 1.0) 20.0)))
      (set `self.Match Style` (`/Game/Blueprints/GameModes/MainMenu/BP_MainMenuController.Versus Menu Choice` _asbp_main_menu_controller))
      (set `self.Deathmatch Rules` (`/Game/Blueprints/GameModes/MainMenu/BP_MainMenuController.Deathmatch Rules` _asbp_main_menu_controller)))
    (:`CastFailed`
      (bind _asversus_game_mode (cast `/Game/Blueprints/GameModes/Versus/VersusGameMode` _returnvalue))
      (for _index (range 1 4)
        (bind _item (`KismetArrayLibrary.Array_Get` (`/Game/Blueprints/GameModes/Versus/VersusGameMode.Player Controllers` _asversus_game_mode) _index))
        (`/Engine/EditorBlueprintResources/StandardMacros.IsValid` _item
          (:`Is Valid`
            (`GameplayStatics.RemovePlayer` _item))))
      (bind _result (`/Engine/EditorBlueprintResources/StandardMacros.IncrementInt` _map_selection_index)
        (:`  `
          (if (> _result (- (`KismetArrayLibrary.Array_Length` _map_name) 1))
            (set `self.Map Selection Index` 0))))))
  (`GameplayStatics.OpenLevel` (`KismetArrayLibrary.Array_Get` _map_name _map_selection_index)))

(fn `StartNewGame`
  (params (Slot :type Integer))
  (bind _returnvalue (`GameplayStatics.CreateSaveGameObject` "/Game/Blueprints/Save/BP_SaveGame.BP_SaveGame_C"))
  (`GameplayStatics.SaveGameToSlot` _returnvalue (`KismetStringLibrary.Concat_StrStr` "SaveGame" (`KismetStringLibrary.Conv_IntToString` Slot)))
  (`GameplayStatics.OpenLevel` "PRISON"))