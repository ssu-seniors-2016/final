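; Main menu game mode that runs the local player join screen for starting a versus match.
; ToggleJoinMenu lazily creates the BPW_JoinMenu widget, binds its events and toggles its visibility, while player join and leave requests are forwarded by controller ID when it is visible.
; Closing it returns keyboard focus to the controller's versus menu.
; Ready-to-start queries the ready player indices, then calls StartNewVersus on the game instance.
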(event `Ready to Start_Event_0`
  (`/Game/Blueprints/GUI/Widgets/BPW_JoinMenu.Get Ready Player Indices` (`self.JoinMenu`) (`self.PlayersInGame`))
  (bind _asbp_instance_main (cast `/Game/Blueprints/BP_Instance_Main` (`GameplayStatics.GetGameInstance`)))
  (`/Game/Blueprints/BP_Instance_Main.Start New Versus` _asbp_instance_main))

(event `ToggleJoinMenu`
  (bind _joinmenu (`self.JoinMenu`))
  (bind _returnvalue (`|EnumEquality` (`Widget.GetVisibility` _joinmenu) "Visible"))
  (`/Engine/EditorBlueprintResources/StandardMacros.IsValid` _joinmenu
    (:`Is Valid`
      (`Widget.SetVisibility` _joinmenu (select `bool` _returnvalue :`false` "Visible" :`true` "Hidden" :!type "ESlateVisibility Enum"))
      (if _returnvalue
        (`WidgetBlueprintLibrary.SetFocusToGameViewport`)))
    (:`Is Not Valid`
      (bind _returnvalue_2 (`|CreateWidget` "/Game/Blueprints/GUI/Widgets/BPW_JoinMenu.BPW_JoinMenu_C"))
      (bind _output_get (set `self.JoinMenu` _returnvalue_2))
      (`UserWidget.AddToViewport` _output_get 0)
      (`Widget.SetVisibility` _output_get "Visible")
      (`WidgetBlueprintLibrary.SetFocusToGameViewport`)
      (add `/Game/Blueprints/GUI/Widgets/BPW_JoinMenu.CloseMe` _output_get (delegate `CloseMe_Event_0`))
      (add `/Game/Blueprints/GUI/Widgets/BPW_JoinMenu.Ready to Start` _output_get (delegate `Ready to Start_Event_0`)))))

(event `CloseMe_Event_0`
  (`Widget.SetVisibility` (`self.JoinMenu`) "Hidden")
  (bind _asbp_main_menu_controller (cast `/Game/Blueprints/GameModes/MainMenu/BP_MainMenuController` (`GameplayStatics.GetPlayerController` 0)))
  (bind _versusmenu (`/Game/Blueprints/GameModes/MainMenu/BP_MainMenuController.VersusMenu` _asbp_main_menu_controller))
  (`/Game/Blueprints/GUI/Widgets/BPW_MenuButton.Set KB Focus` (`/Game/Blueprints/GUI/Widgets/VersusMenu/BPW_VersusMenu.Start` _versusmenu))
  (`Widget.SetVisibility` _versusmenu "Visible"))

(event `self.TryAddNewPlayer`
  (params (ControllerId :type Integer))
  (bind _joinmenu (`self.JoinMenu`))
  (`KismetSystemLibrary.PrintString` (`KismetStringLibrary.Concat_StrStr` "Player " (`KismetStringLibrary.Conv_IntToString` ControllerId) " pressed start.") false false)
  (`/Engine/EditorBlueprintResources/StandardMacros.IsValid` _joinmenu
    (:`Is Valid`
      (if (`|EnumEquality` (`Widget.GetVisibility` _joinmenu) "Visible")
        (`/Game/Blueprints/GUI/Widgets/BPW_JoinMenu.Player Joined` (`self.JoinMenu`) ControllerId)))))

(event `self.TryRemovePlayer`
  (params (ControllerId :type Integer))
  (bind _joinmenu (`self.JoinMenu`))
  (`/Engine/EditorBlueprintResources/StandardMacros.IsValid` _joinmenu
    (:`Is Valid`
      (if (`Widget.IsVisible` _joinmenu)
        (`/Game/Blueprints/GUI/Widgets/BPW_JoinMenu.Player Left` (`self.JoinMenu`) ControllerId)))))

(fn `UserConstructionScript`)