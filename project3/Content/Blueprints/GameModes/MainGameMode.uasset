(event `self.ReceiveBeginPlay`
  (`GameplayStatics.CreatePlayer` 1)
  (`GameplayStatics.CreatePlayer` 2)
  (`GameplayStatics.CreatePlayer` 3)
  (bind _returnvalue (`|SpawnActorFromClass` "/Game/Blueprints/Character/UtilComponents/BP_ChaseCamera.BP_ChaseCamera_C" (`KismetMathLibrary.MakeTransform` (0.0 0.0 0.0)) "Undefined" "OverrideRootScale"))
  (set `self.Chase Cam` _returnvalue))

(fn `Add Player to World`
  (params (Controller :type "/Game/Blueprints/GameModes/MainPlayerController Object Reference"))
  (bind _chase_cam (`self.Chase Cam`))
  (bind _players (`/Game/Blueprints/Character/UtilComponents/BP_ChaseCamera.Players` _chase_cam))
  (bind _outactors (`GameplayStatics.GetAllActorsOfClass` "/Game/Blueprints/Character/BP_MainCharacter.BP_MainCharacter_C"))
  (bind _outactors_2 (`GameplayStatics.GetAllActorsOfClass` "/Script/Engine.PlayerStart"))
  (bind _returnvalue (`|SpawnActorFromClass` "/Game/Blueprints/Character/BP_MainCharacter.BP_MainCharacter_C" (`self.GetTransform` (`KismetArrayLibrary.Array_Get` _outactors_2)) "Undefined" "OverrideRootScale" null true true true 0.0 0.0 (`KismetArrayLibrary.Array_Length` _outactors) true))
  (`Controller.UnPossess` Controller)
  (`Controller.Possess` Controller _returnvalue)
  (`KismetArrayLibrary.Array_Add` _players _returnvalue)
  (if (> (`KismetArrayLibrary.Array_Length` _players) 1)
    (`/Engine/EditorBlueprintResources/StandardMacros.DoOnce` false
      (:`Completed`
        (`/Game/Blueprints/Character/UtilComponents/BP_ChaseCamera.Initialize` _chase_cam)
        (`PlayerController.SetViewTargetWithBlend` (`GameplayStatics.GetPlayerController` 0) _chase_cam 1.0 "VTBlend_Linear" 1.0 false)))
    (else
      (`PlayerController.SetViewTargetWithBlend` (`GameplayStatics.GetPlayerController` 0) (`KismetArrayLibrary.Array_Get` _players) 0.0 "VTBlend_Linear" 0.0 false))))

(fn `Remove Player From World`
  (params (Controller :type "/Game/Blueprints/GameModes/MainPlayerController Object Reference") (Pawn :type "/Game/Blueprints/Character/BP_MainCharacter Object Reference"))
  (bind _players (`/Game/Blueprints/Character/UtilComponents/BP_ChaseCamera.Players` (`self.Chase Cam`)))
  (`Controller.UnPossess` Controller)
  (bind _returnvalue (`|SpawnActorFromClass` "/Game/Blueprints/GameModes/BP_StandbyPlayer.BP_StandbyPlayer_C" (`SceneComponent.K2_GetComponentToWorld` (`Character.CapsuleComponent` Pawn)) "Undefined" "OverrideRootScale"))
  (`Controller.Possess` Controller _returnvalue)
  (`KismetArrayLibrary.Array_RemoveItem` _players Pawn)
  (`self.K2_DestroyActor` Pawn)
  (if (== (`KismetArrayLibrary.Array_Length` _players) 1)
    (`PlayerController.SetViewTargetWithBlend` (`GameplayStatics.GetPlayerController` 0) (`KismetArrayLibrary.Array_Get` _players) 0.0 "VTBlend_Linear" 0.0 false)))

(fn `UserConstructionScript`)