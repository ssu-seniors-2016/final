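; Player controller for local versus matches, handling drop-in/out, stock lives, kills and respawn readiness.
; On possession it initializes the versus HUD and relays gun bullet updates through dispatchers, which also broadcast health, stock, kill and death events.
; Death unpossesses the pawn and costs a stock, with a doubled respawn wait for suicides.
; Holding ResetMe while stationary requests an unstuck reset; debug-style keys restart the match or return to menu.
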(event `ResetRequestDelay`
  ;[1 1 1] reset pawn when stuck
  (if (and (`self.IsInputKeyDown` (stale `InputAction|ResetMe` Key)) (== (`self.K2_GetActorLocation` (`self.K2_GetPawn`)) (stale `InputAction|ResetMe` _output_get)))
    (bind _asbp_main_character (cast `/Game/Blueprints/Character/BP_MainCharacter` (`self.K2_GetPawn`)))
    (`self.Reset Request` _asbp_main_character)
    (else
      (`KismetSystemLibrary.PrintString` "Reset request denied. You moved." true false (select `int` (`self.Index`) :`0` (struct :`G` 1.0 :`B` 0.972981 :`A` 1.0) :`1` (struct :`R` 1.0 :`G` 0.055 :`B` 0.055 :`A` 1.0) :`2` (struct :`R` 1.0 :`G` 0.788235 :`A` 1.0) :`3` (struct :`G` 1.0 :`A` 1.0) :!type "LinearColor Structure") 4.0))))

(event `InputAction|ResetMe`
  (params (Key :type "Key Structure" :default "AnyKey"))
  ;[1 1 1] reset pawn when stuck
  (:`Pressed`
    (`KismetSystemLibrary.K2_SetTimerDelegate` (delegate `ResetRequestDelay`) 3.0)
    (bind _output_get (set `self.Location at Reset Request` (`self.K2_GetActorLocation` (`self.K2_GetPawn`))))))

(event `Key|Equals`
  (params (Key :type "Key Structure" :default "AnyKey")))

(event `Key|Gamepad_LeftThumbstick`
  (params (Key :type "Key Structure" :default "AnyKey")))

(event `self.ReceiveBeginPlay`
  (add `self.New Pawn Possessed` (delegate `New Pawn Possessed_Event_0`)))

(event `Bullet Updated_Event_0`
  (params (Index :type Integer))
  (`self.Update Weapon` Index))

(event `Key|Home`
  (params (Key :type "Key Structure" :default "AnyKey"))
  (:`Pressed`
    (bind _asbp_instance_main (cast `/Game/Blueprints/BP_Instance_Main` (`GameplayStatics.GetGameInstance`)))
    (`/Game/Blueprints/BP_Instance_Main.Return to Main Menu` _asbp_instance_main)))

(event `New Pawn Possessed_Event_0`
  (`self.Init Versus Frame`)
  (bind _asbp_main_character (cast `/Game/Blueprints/Character/BP_MainCharacter` (`self.K2_GetPawn`)))
  (bind _ac_guncomponent (`/Game/Blueprints/Character/BP_MainCharacter.AC_GunComponent` _asbp_main_character))
  (add `/Game/Blueprints/Character/AC_GunComponent.Bullet Updated` _ac_guncomponent (delegate `Bullet Updated_Event_0`))
  (`KismetSystemLibrary.Delay` 0.1)
  (`/Game/Blueprints/Character/AC_GunComponent.Init GUI Element` _ac_guncomponent)
  (set `self.Suicide` false))

(event `InputAction|DropInDropOut`
  (params (Key :type "Key Structure" :default "AnyKey"))
  (:`Released`
    (`/Engine/EditorBlueprintResources/StandardMacros.FlipFlop`
      (:`A`
        (bind _asmain_game_mode (cast `/Game/Blueprints/GameModes/MainGameMode` (`GameplayStatics.GetGameMode`)))
        (`/Game/Blueprints/GameModes/MainGameMode.Add Player to World` _asmain_game_mode self))
      (:`B`
        (bind _asmain_game_mode_2 (cast `/Game/Blueprints/GameModes/MainGameMode` (`GameplayStatics.GetGameMode`)))
        (bind _asbp_main_character (cast `/Game/Blueprints/Character/BP_MainCharacter` (`self.K2_GetPawn`)))
        (`/Game/Blueprints/GameModes/MainGameMode.Remove Player From World` _asmain_game_mode_2 self _asbp_main_character)))))

(event `Pawn Died`
  (params (Murderer :type "/Game/Blueprints/GameModes/MainPlayerController Object Reference"))
  (bind _stock_count (`self.Stock Count`))
  (`self.UnPossess`)
  (set `self.Ready to Spawn` false)
  (`self.HealthUpdated` 0.0)
  (`/Engine/EditorBlueprintResources/StandardMacros.DecrementInt` _stock_count
    (:`  `
      (`self.Update Stock Count` _stock_count)
      (`self.Dead Pawn` self)
      (if (> (`self.Stock Count`) 0)
        (`self.WaitToRespawn` 2.6)
        (`/Engine/EditorBlueprintResources/StandardMacros.IsValid` Murderer
          (:`Is Valid`
            (`self.Confirm Player Kill` Murderer self)))))))

(event `WaitToRespawn`
  (params (`Wait Time` :type "Float (double-precision)"))
  (`KismetSystemLibrary.Delay` (`KismetMathLibrary.SelectFloat` (* `Wait Time` 2.0) `Wait Time` (`self.Suicide`)))
  (set `self.Ready to Spawn` true))

(event `Key|Backslash`
  (params (Key :type "Key Structure" :default "AnyKey"))
  (:`Pressed`
    (bind _asbp_instance_main (cast `/Game/Blueprints/BP_Instance_Main` (`GameplayStatics.GetGameInstance`)))
    (for _index (range 4)
      (bind _returnvalue (`GameplayStatics.GetPlayerController` _index))
      (`/Engine/EditorBlueprintResources/StandardMacros.IsValid` _returnvalue
        (:`Is Valid`
          (`GameplayStatics.RemovePlayer` _returnvalue))))
    (`/Game/Blueprints/BP_Instance_Main.Start New Versus` _asbp_instance_main)))

(fn `Confirm Player Kill`
  (params (Victim :type "/Game/Blueprints/GameModes/MainPlayerController Object Reference"))
  (`/Engine/EditorBlueprintResources/StandardMacros.IncrementInt` (`KismetArrayLibrary.Array_Get` (`self.Player Kills`) (`/Game/Blueprints/GameModes/MainPlayerController.Index` Victim))
    (:`  `
      (if (== Victim self)
        (set `self.Suicide` true)
        (else
          (`self.Kill Event` Victim self)))
      (return))))

(fn `Init Versus Frame`
  (`self.Update Stock Count` (`self.Stock Count`))
  (`self.HealthUpdated` 1.0))

(fn `Request Respawn`
  (`KismetSystemLibrary.PrintString` "Hello")
  (`/Engine/EditorBlueprintResources/StandardMacros.IsValid` (`self.K2_GetPawn`)
    (:`Is Valid`
      (`KismetSystemLibrary.K2_SetTimer` null "Request Respawn"))
    (:`Is Not Valid`
      (`self.Respawn Request` self)
      (`KismetSystemLibrary.K2_SetTimer` null "Request Respawn" 0.1 true))))

(fn `UserConstructionScript`)