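; Checkpoint manager that saves the player's position to a save slot when the player passes a checkpoint.
; On BeginPlay it binds to the PlayerPassed event of every BP_Checkpoint in the level.
; The handler loads or creates a CheckpointSave, stores the player character's current location rather than the checkpoint's, and writes it back.
; An overlap event shares that save path, and two init functions store checkpoint and killbox references.
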(event `Player Passed_Event_0`
  (params (Checkpoint :type "/Game/Blueprints/StreamingTest_BP/BP_Checkpoint Object Reference"))
  (bind _checkpoint_slot_name (`self.Checkpoint Slot name`))
  (bind _returnvalue (`self.K2_GetActorLocation` (`GameplayStatics.GetPlayerCharacter` 0)))
  (bind _returnvalue_2 (`GameplayStatics.LoadGameFromSlot` (`self.Checkpoint Slot name`) :!label _label))
  (`/Engine/EditorBlueprintResources/StandardMacros.IsValid` _returnvalue_2
    (:`Is Valid`
      (bind _ascheckpoint_save (cast `/Game/Blueprints/Save/CheckpointSave` _returnvalue_2))
      (bind _output_get (set `self.Checkpoint Save` _ascheckpoint_save))
      (set `/Game/Blueprints/Save/CheckpointSave.Checkpoint Position` _returnvalue _output_get)
      (`GameplayStatics.SaveGameToSlot` _output_get _checkpoint_slot_name))
    (:`Is Not Valid`
      (bind _returnvalue_3 (`GameplayStatics.CreateSaveGameObject` "/Game/Blueprints/Save/CheckpointSave.CheckpointSave_C"))
      (bind _ascheckpoint_save_2 (cast `/Game/Blueprints/Save/CheckpointSave` _returnvalue_3))
      (bind _output_get_2 (set `self.Checkpoint Save` _ascheckpoint_save_2))
      (set `/Game/Blueprints/Save/CheckpointSave.Checkpoint Position` _returnvalue _output_get_2)
      (`GameplayStatics.SaveGameToSlot` _output_get_2 _checkpoint_slot_name))))

(event `self.ReceiveBeginPlay`
  (bind _outactors (`GameplayStatics.GetAllActorsOfClass` "/Game/Blueprints/StreamingTest_BP/BP_Checkpoint.BP_Checkpoint_C"))
  (for _array_element _outactors
    (bind _asbp_checkpoint (cast `/Game/Blueprints/StreamingTest_BP/BP_Checkpoint` _array_element))
    (add `/Game/Blueprints/StreamingTest_BP/BP_Checkpoint.Player Passed` _asbp_checkpoint (delegate `Player Passed_Event_0`))))

(event `OnActorBeginOverlap_Event_0`
  (params (OtherActor :type "Actor Object Reference"))
  (goto _label))

(fn `init checkpoint`
  (params (checkpoint :type "Array of Actor Object Reference"))
  (set `self.check` checkpoint))

(fn `init killbox`
  (params (killbox :type "Array of Actor Object Reference"))
  (set `self.kill` killbox))

(fn `UserConstructionScript`)