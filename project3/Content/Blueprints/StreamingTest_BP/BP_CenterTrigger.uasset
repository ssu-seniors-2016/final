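; Trigger actor for level streaming that loads every level named in NextArray once the main character overlaps its Center component.
; The overlap opens a Gate on Tick, and a DoOnce serializes the loads, resetting after each blocking, make-visible LoadStreamLevel finishes.
; Each load prints the level name and advances Count, and the Gate closes when the array is exhausted.
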(event `self.ReceiveTick`
  (params (DeltaSeconds :type "Float (single-precision)"))
  (bind _nextarray (`self.NextArray`))
  (bind _count (`self.count`))
  (bind _item (`KismetArrayLibrary.Array_Get` _nextarray _count))
  (bind _returnvalue (+ _count 1))
  (`/Engine/EditorBlueprintResources/StandardMacros.Gate` true :!label _label
    (:`Exit`
      (`/Engine/EditorBlueprintResources/StandardMacros.DoOnce` false :!label _label_2
        (:`Completed`
          (`GameplayStatics.LoadStreamLevel` _item true true)
          (`KismetSystemLibrary.PrintString` (`KismetStringLibrary.Concat_StrStr` "loaded level: " (`KismetStringLibrary.Conv_NameToString` _item)))
          (set `self.count` _returnvalue)
          (if (> _returnvalue (`KismetArrayLibrary.Array_Length` _nextarray))
            (goto _label :!via `Close`)
            (else
              (goto _label_2 :!via `Reset`))))))))

(event `self.Center.OnComponentBeginOverlap`
  (params (OtherActor :type "Actor Object Reference") (OtherComp :type "PrimitiveComponent Object Reference") (OtherBodyIndex :type Integer) (bFromSweep :type Boolean) (SweepResult :type "HitResult Structure (by ref)"))
  (cast `/Game/Blueprints/Character/BP_MainCharacter` OtherActor)
  (goto _label :!via `Open`))

(fn `UserConstructionScript`)