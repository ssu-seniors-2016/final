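; Level-streaming trigger actor with Begin, Center and End boxes that load and unload sublevels as BP_MainCharacter passes through.
; Center loads the combined Begin and End level lists, while End unloads the Begin list and Begin unloads the End list.
; Looping timers process one level per tick, with blocking loads, and clear themselves when a list finishes.
; The construction script sizes and places boxes, merges the lists and optionally shows boxes for debugging.
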(event `self.Center.OnComponentBeginOverlap`
  (params (OtherActor :type "Actor Object Reference") (OtherComp :type "PrimitiveComponent Object Reference") (OtherBodyIndex :type Integer) (bFromSweep :type Boolean) (SweepResult :type "HitResult Structure (by ref)"))
  (cast `/Game/Blueprints/Character/BP_MainCharacter` OtherActor)
  (`KismetSystemLibrary.K2_SetTimerDelegate` (delegate `LoadEvent`) (`self.TickTock`) true))

(event `LoadEvent`
  (bind _centercounter (`self.centerCounter`))
  (bind _centerarray (`self.CenterArray`))
  (bind _returnvalue (+ _centercounter 1))
  (`/Engine/EditorBlueprintResources/StandardMacros.Gate` false
    (:`Exit`
      (`/Engine/EditorBlueprintResources/StandardMacros.DoOnce` false :!label _label
        (:`Completed`
          (`GameplayStatics.LoadStreamLevel` (`KismetArrayLibrary.Array_Get` _centerarray _centercounter) true true)
          (set `self.centerCounter` _returnvalue)
          (if (> _returnvalue (`KismetArrayLibrary.Array_Length` _centerarray))
            (`KismetSystemLibrary.K2_SetTimerDelegate` (delegate `LoadEvent`))
            (set `self.centerCounter` 0)
            (goto _label :!via `Reset`)
            (else
              (goto _label :!via `Reset`))))))))

(event `self.ReceiveBeginPlay`
  (if (`self.Debug`)
    (for _array_element (`self.CenterArray`)
      (`KismetSystemLibrary.PrintString` (`KismetStringLibrary.Conv_NameToString` _array_element)))))

(event `self.End.OnComponentBeginOverlap`
  (params (OtherActor :type "Actor Object Reference") (OtherComp :type "PrimitiveComponent Object Reference") (OtherBodyIndex :type Integer) (bFromSweep :type Boolean) (SweepResult :type "HitResult Structure (by ref)"))
  (cast `/Game/Blueprints/Character/BP_MainCharacter` OtherActor)
  (`KismetSystemLibrary.K2_SetTimerDelegate` (delegate `UnloadEndEvent`) (`self.TickTock`) true))

(event `UnloadEndEvent`
  (bind _endcounter (`self.endCounter`))
  (bind _beginarray (`self.BeginArray`))
  (bind _returnvalue (+ _endcounter 1))
  (`/Engine/EditorBlueprintResources/StandardMacros.Gate` false
    (:`Exit`
      (`/Engine/EditorBlueprintResources/StandardMacros.DoOnce` false :!label _label_2
        (:`Completed`
          (`GameplayStatics.UnloadStreamLevel` (`KismetArrayLibrary.Array_Get` _beginarray _endcounter))
          (set `self.endCounter` _returnvalue)
          (if (> _returnvalue (`KismetArrayLibrary.Array_Length` _beginarray))
            (`KismetSystemLibrary.K2_SetTimerDelegate` (delegate `UnloadEndEvent`))
            (set `self.endCounter` 0)
            (goto _label_2 :!via `Reset`)
            (else
              (goto _label_2 :!via `Reset`))))))))

(event `self.Begin.OnComponentBeginOverlap`
  (params (OtherActor :type "Actor Object Reference") (OtherComp :type "PrimitiveComponent Object Reference") (OtherBodyIndex :type Integer) (bFromSweep :type Boolean) (SweepResult :type "HitResult Structure (by ref)"))
  (cast `/Game/Blueprints/Character/BP_MainCharacter` OtherActor)
  (`KismetSystemLibrary.K2_SetTimerDelegate` (delegate `UnloadBeginEvent`) (`self.TickTock`) true))

(event `UnloadBeginEvent`
  (bind _begincounter (`self.beginCounter`))
  (bind _endarray (`self.EndArray`))
  (bind _returnvalue (+ _begincounter 1))
  (`/Engine/EditorBlueprintResources/StandardMacros.Gate` false
    (:`Exit`
      (`/Engine/EditorBlueprintResources/StandardMacros.DoOnce` false :!label _label_3
        (:`Completed`
          (`GameplayStatics.UnloadStreamLevel` (`KismetArrayLibrary.Array_Get` _endarray _begincounter))
          (set `self.beginCounter` _returnvalue)
          (if (> _returnvalue (`KismetArrayLibrary.Array_Length` _endarray))
            (`KismetSystemLibrary.K2_SetTimerDelegate` (delegate `UnloadBeginEvent`))
            (set `self.beginCounter` 0)
            (goto _label_3 :!via `Reset`)
            (else
              (goto _label_3 :!via `Reset`))))))))

(fn `UserConstructionScript`
  (bind _box_extent (`self.Box Extent`))
  (bind _end (`self.End`))
  (bind _center (`self.Center`))
  (`BoxComponent.SetBoxExtent` (`self.Begin`) _box_extent true)
  (`BoxComponent.SetBoxExtent` _center _box_extent true)
  (`SceneComponent.K2_SetRelativeLocation` _center (`self.Center Location`) false false)
  (`BoxComponent.SetBoxExtent` _end _box_extent true)
  (`SceneComponent.K2_SetRelativeLocation` _end (`self.End Loctation`) false false)
  (`KismetArrayLibrary.Array_Append` (`self.CenterArray`) (`self.BeginArray`))
  (`KismetArrayLibrary.Array_Append` (`self.CenterArray`) (`self.EndArray`))
  (if (`self.Debug`)
    (`SceneComponent.SetHiddenInGame` (`self.Begin`) false false)
    (`SceneComponent.SetHiddenInGame` (`self.End`) false false)
    (`SceneComponent.SetHiddenInGame` (`self.Center`) false false)))