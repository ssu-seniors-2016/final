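; BP_LeverDown is a grapple-activated lever that moves down or up toward world Z zero when the player attaches.
; On BeginPlay it stores its start location and binds to the attach event of its GrappleNode child actor.
; Timeline updates drive constant-speed VInterpTo moves.
; A slower return to the start location exists, but its detach binding is unconnected, so it never runs.
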(event `CustomEvent_0`
  (bind _returnvalue (`self.K2_GetActorLocation`))
  (`Timeline|Timeline_0`
    (:`Update`
      (`self.K2_SetActorLocation` (`KismetMathLibrary.VInterpTo_Constant` _returnvalue (`KismetMathLibrary.MakeVector` (.x _returnvalue) (.y _returnvalue)) (`self.Delta Time`) 200.0)))))

(event `self.ReceiveBeginPlay`
  (set `self.OriginalPos` (`self.K2_GetActorLocation`))
  (bind _asgrapple_node (cast `/Game/Blueprints/Character/GrappleHook/GrappleNode` (`ChildActorComponent.ChildActor` (`self.GrapplePoint`))))
  (add `/Game/Blueprints/Character/GrappleHook/GrappleNode.PlayerIsAttached` _asgrapple_node (delegate `CustomEvent_0`)))

(event `CustomEvent_1`
  (`Timeline|Timeline_1`
    (:`Update`
      (`self.K2_SetActorLocation` (`KismetMathLibrary.VInterpTo_Constant` (`self.K2_GetActorLocation`) (`self.OriginalPos`) (`self.Delta Time`) 50.0)))))

(fn `UserConstructionScript`)