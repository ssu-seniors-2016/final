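; Player shield actor with a sphere component, which caches its instigating BP_MainCharacter on BeginPlay.
; Incoming damage is divided by ShieldHealth and broadcast through DamageReceived; this actor does not reduce the health itself.
; Helper functions swap the sphere material, report health percent against a hardcoded maximum, and spawn BP_ShieldBreak for the break effect.
; Sphere hit and overlap events are empty, leaving bullet reflection and ShieldTimer drain logic disconnected.
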(event `self.ReceiveBeginPlay`
  (bind _asbp_main_character (cast `/Game/Blueprints/Character/BP_MainCharacter` (`self.GetInstigator`)))
  (set `self.Player` _asbp_main_character))

(event `self.ReceiveAnyDamage`
  (params (Damage :type "Float (single-precision)") (DamageType :type "DamageType Object Reference") (InstigatedBy :type "Controller Object Reference") (DamageCauser :type "Actor Object Reference"))
  (`self.Damage Received` (/ Damage (`self.Shield Health`))))

(event `self.Sphere.OnComponentHit`
  (params (OtherActor :type "Actor Object Reference") (OtherComp :type "PrimitiveComponent Object Reference") (NormalImpulse :type "Vector Structure") (Hit :type "HitResult Structure (by ref)")))

(event `self.Sphere.OnComponentBeginOverlap`
  (params (OtherActor :type "Actor Object Reference") (OtherComp :type "PrimitiveComponent Object Reference") (OtherBodyIndex :type Integer) (bFromSweep :type Boolean) (SweepResult :type "HitResult Structure (by ref)")))

(fn `Break`
  (bind _returnvalue (`|SpawnActorFromClass` "/Game/Blueprints/BP_ShieldBreak.BP_ShieldBreak_C" (`KismetMathLibrary.MakeTransform` (.location (`SceneComponent.K2_GetComponentToWorld` (`self.Sphere`)))) "AlwaysSpawn" "OverrideRootScale"))
  (`/Game/Blueprints/BP_ShieldBreak.Break` _returnvalue))

(fn `Get Health Percent`
  (returns (`Health Percent` :type "Float (double-precision)"))
  (return (/ (`self.Shield Health`) 500.0)))

(fn `Set Material`
  (params (Material :type "MaterialInstanceDynamic Object Reference"))
  (`PrimitiveComponent.SetMaterial` (`self.Sphere`) 0 Material))

(fn `UserConstructionScript`)