(fn FocusFailsafe
  (params (Buttons :type Array%20of%20BPW%20Menu%20Button%20Object%20References) (Last%20Focus%20Button :type BPW%20Menu%20Button%20Object%20Reference%20%28by%20ref%29))
  (bind _array_element (Utilities|Array|ForEachLoopwithBreak Buttons :!label _label)
    (:LoopBody
      (if (Class|Widget|HasKeyboardFocus (Variables|/Game/Blueprints/GUI/Widgets/BPW_MenuButton.BPW_MenuButton_C|GetButton_0 _array_element))
        (LocalVariables|SetFailure false)
        (|SetBy-RefVar Last%20Focus%20Button _array_element)
        (goto _label Break)))
    (:Completed
      (return (LocalVariables|GetFailure)))))

(fn MakeButtonArray
  (params (Canvas :type Canvas%20Panel%20Object%20Reference) (Menu%20Buttons :type Array%20of%20BPW%20Menu%20Button%20Object%20References))
  (for _index (range 0 (- (Class|PanelWidget|GetChildrenCount Canvas) 1))
    (bind _aspanel_widget (Utilities|Casting|CastToPanelWidget (Class|PanelWidget|GetChildat Canvas _index))
      (:then
        (for _index_2 (range 0 (- (Class|PanelWidget|GetChildrenCount _aspanel_widget) 1))
          (bind _asbpw_menu_button (Utilities|Casting|CastToBPW_MenuButton (Class|PanelWidget|GetChildat _aspanel_widget _index_2)))
          (Utilities|Array|AddUnique Menu%20Buttons _asbpw_menu_button)))
      (:CastFailed
        (bind _asbpw_menu_button_2 (Utilities|Casting|CastToBPW_MenuButton (Class|PanelWidget|GetChildat Canvas _index)))
        (Utilities|Array|AddUnique Menu%20Buttons _asbpw_menu_button_2)))))