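; BP_FloatingText is a placeable text label actor that displays configurable text in the world through a Widget component hosting BPW_TextWidget.
; The construction script pushes the Text, Color and FontSize variables into the widget's TextBlock, keeping the rest of its font settings.
; BeginPlay reapplies text and color at runtime, but not font size.
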(event `self.ReceiveBeginPlay`
  (bind _asbpw_text_widget (cast `/Game/Blueprints/GUI/BPW_TextWidget` (`WidgetComponent.GetUserWidgetObject` (`self.Widget`))))
  (bind _textblock (`/Game/Blueprints/GUI/BPW_TextWidget.TextBlock` _asbpw_text_widget))
  (`TextBlock.SetText` _textblock (`self.Text`))
  (`TextBlock.SetColorAndOpacity` _textblock (`self.Color`)))

(event `self.ReceiveActorBeginOverlap`
  (params (OtherActor :type "Actor Object Reference")))

(event `self.ReceiveTick`
  (params (DeltaSeconds :type "Float (single-precision)")))

(fn `UserConstructionScript`
  (bind _asbpw_text_widget (cast `/Game/Blueprints/GUI/BPW_TextWidget` (`WidgetComponent.GetUserWidgetObject` (`self.Widget`))))
  (bind _textblock (`/Game/Blueprints/GUI/BPW_TextWidget.TextBlock` _asbpw_text_widget))
  (`TextBlock.SetText` _textblock (`self.Text`))
  (`TextBlock.SetColorAndOpacity` _textblock (`self.Color`))
  (bind (_fontobject _fontmaterial _typefacefontname) (break `SlateFontInfo` (`TextBlock.Font` _textblock)))
  (`TextBlock.SetFont` _textblock (make `SlateFontInfo` _fontobject _fontmaterial _typefacefontname (`self.Font Size`))))