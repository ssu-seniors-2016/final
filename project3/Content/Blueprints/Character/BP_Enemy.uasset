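; Base enemy actor that hurts the player on contact, takes damage from player-owned bullets and can be grappled or stunned.
; Hit box overlaps apply damage, while the sight sphere uses a line trace to switch Waiting or Roaming mobs to Attacking, storing the attack direction.
; Damage lowers health and briefly swaps in a flash material, restoring defaults cached at construction.
; At zero health it spawns an explosion and signals its death.
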(event OnComponentBeginOverlap(HitBox)
  (params (OtherActor :type Actor%20Object%20Reference) (OtherComp :type Primitive%20Component%20Object%20Reference) (OtherBodyIndex :type Integer) (bFromSweep :type Boolean) (SweepResult :type Hit%20Result%20Structure%20%28by%20ref%29))
  (bind _contact_damage (Variables|Default|GetContact%20Damage))
  ;[1 1 1] Hurt player when he's inside of our hit box.
  (bind _asbp_main_character (Utilities|Casting|CastToBP_MainCharacter OtherActor)
    (:then
      (if (> _contact_damage 0.0)
        (Game|Damage|ApplyDamage _asbp_main_character _contact_damage 0 self "/Game/Blueprints/Character/BP_ContactDamage.BP_ContactDamage_C")))
    (:CastFailed
      (bind _asbp_bullet_parent (Utilities|Casting|CastToBP_BulletParent OtherActor))
      (bind _asbp_main_character_2 (Utilities|Casting|CastToBP_MainCharacter (Components|GetOwner _asbp_bullet_parent)))
      (Game|Damage|ApplyDamage self (Variables|/Game/Blueprints/Weapons/BP_BulletParent.BP_BulletParent_C|GetDamage%20Value _asbp_bullet_parent) 0 _asbp_main_character_2)
      (Default|CallConfirmHit _asbp_bullet_parent))))

(event OnComponentBeginOverlap(SightSphere)
  (params (OtherActor :type Actor%20Object%20Reference) (OtherComp :type Primitive%20Component%20Object%20Reference) (OtherBodyIndex :type Integer) (bFromSweep :type Boolean) (SweepResult :type Hit%20Result%20Structure%20%28by%20ref%29))
  (bind _returnvalue (Transformation|GetActorLocation))
  ;[1 1 1] switch to state to attacking when a player is in sight sphere and we can trace a line to him
  (switch Utilities|FlowControl|Switch|SwitchonE_MobState (Variables|Default|GetMob%20State)
    (:NewEnumerator0
      _)
    (:NewEnumerator1
      _))
  (bind _asbp_main_character (Utilities|Casting|CastToBP_MainCharacter OtherActor))
  (bind _outhit (Collision|LineTraceByChannel _returnvalue (Transformation|GetActorLocation _asbp_main_character) "TraceTypeQuery3" false 0 "None"))
  (if (== (.HitActor (Collision|BreakHitResult _outhit)) _asbp_main_character)
    (Variables|Default|SetAttack%20Direction (Math|Vector|Normalize (- (Transformation|GetActorLocation _asbp_main_character) _returnvalue)))
    (Variables|Default|SetMob%20State "NewEnumerator2")))

(event Custom|Explode%20and%20Destory
  (bind _returnvalue (Transformation|GetActorTransform))
  (bind (_location _rotation) (Math|Transform|BreakTransform _returnvalue))
  ;[1 1 1] explode and destroy
  (Effects|SpawnEmitteratLocation "/Game/Particles/Emitters/P_Explosion_A.P_Explosion_A" _location _rotation)
  (Utilities|FlowControl|Delay 0.2)
  (Default|CallHasBeenKilled)
  (Variables|Default|SetbAutoDestroyWhenFinished true))

(event Custom|Initialize
  ;[1 1 1] This must be called if begin play is overriden
  (Variables|Default|SetForward%20Vector%20at%20Start (Transformation|GetActorForwardVector))
  (Utilities|IsValid (Pawn|GetController)
    (:Is%20Not%20Valid
      (Pawn|SpawnDefaultController))))

(event EventBeginPlay
  (Variables|Default|SetForward%20Vector%20at%20Start (Transformation|GetActorForwardVector))
  (Utilities|IsValid (Pawn|GetController)
    (:Is%20Not%20Valid
      (Pawn|SpawnDefaultController))))

(event EventPlayerDetatched
  (params (Player :type Character%20Object%20Reference))
  ;[1 1 1] some grapple functions that may not actually be used, i'm not really sure.
  (Variables|Default|SetMob%20State "NewEnumerator0"))

(event Game|Damage|EventAnyDamage
  (params (Damage :type Float%20%28single-precision%29) (DamageType :type Damage%20Type%20Object%20Reference) (InstigatedBy :type Controller%20Object%20Reference) (DamageCauser :type Actor%20Object%20Reference))
  (bind _mesh (Variables|Character|GetMesh))
  (bind _returnvalue (Rendering|Material|GetMaterials _mesh))
  ;[1 1 1] flash white when damaged
  (Variables|Default|SetHealth (Math|Float|SelectFloat 0.0 (|(hlth-dmg) (Variables|Default|GetHealth) Damage) (<= (|(hlth-dmg) (Variables|Default|GetHealth) Damage) 0.0)))
  (if (<= (|(hlth-dmg) (Variables|Default|GetHealth) Damage) 0.0)
    (Utilities|FlowControl|DoOnce false
      (:Completed
        (CallFunction|ExplodeandDestory)))
    (else
      (for (_ _array_index) _returnvalue
        (Rendering|Material|SetMaterial _mesh _array_index "/Game/Materials/M_HitEffect.M_HitEffect"))
      (Utilities|FlowControl|Delay 0.05)
      (for (_ _array_index_2) _returnvalue
        (Rendering|Material|SetMaterial _mesh _array_index_2 (Utilities|Array|Get(acopy) (Variables|Default|GetDefault%20Materials) _array_index_2))))))

(event EventGetGrappled
  (params (Grabber :type Character%20Object%20Reference))
  ;[1 1 1] some grapple functions that may not actually be used, i'm not really sure.
  (Variables|Default|SetMob%20State "NewEnumerator3")
  (CallFunction|BasicGetGrappled Grabber self))

(event EventGetStunned
  (params (Stunner :type Actor%20Object%20Reference))
  (CallFunction|BasicGetStunned self))

(fn ConstructionScript
  (Variables|Default|SetDefault%20Materials (Rendering|Material|GetMaterials (Variables|Character|GetMesh))))

(fn CanbeGrappled
  (return true))

(fn CanbeStunned
  (return true))

(fn GrappleBoost
  (return "0, 0, 0" false))