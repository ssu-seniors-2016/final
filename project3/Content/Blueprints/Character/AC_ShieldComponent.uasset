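; Character component giving BP_MainCharacter a shield whose timer serves as both duration and health.
; Spawns and attaches a shield actor, toggling visibility and collision on activation and deactivation.
; Tick drains or recharges the timer, breaking the shield into cooldown when empty; damage drains it too, with PassDamageToShield returning overflow.
; A dynamic material recreated each tick shows charge through green, and opacity marks the upgrade's brief post-activation reflect window.
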(event Custom|Damage%20Received_Event_0
  (params (Health%20Percent :type Float%20%28single-precision%29))
  (Variables|Default|SetShield%20Timer (- (Variables|Default|GetShield%20Timer) (* (Variables|Default|GetmaxShieldTime) Health%20Percent)))
  (Development|PrintString (Utilities|String|Append "blocked damage for " (Utilities|String|ToString(Float) Health%20Percent) "% of shield's timer")))

(event EventBeginPlay
  (CallFunction|CreateShield)
  (EventDispatchers|AssignDamageReceived (Variables|Default|GetmShield) (delegate Custom|Damage%20Received_Event_0)))

(event EventTick
  (params (DeltaSeconds :type Float%20%28single-precision%29))
  (bind _maxshieldtime (Variables|Default|GetmaxShieldTime))
  (CallFunction|UpdateShieldColor)
  (if (Variables|Default|GetisDestroyed) ; checks if sheild was destroyed
    ;[0.02671 0.9235 1] Shield was destroyed, cooldown timer
    (Variables|Default|SetdestroyTimer (- (Variables|Default|GetdestroyTimer) DeltaSeconds))
    (if (<= (Variables|Default|GetdestroyTimer) 0.0)
      (Variables|Default|SetisDestroyed false)
      (Variables|Default|SetdestroyTimer 5.0)
      (Variables|Default|SetShield%20Timer (Variables|Default|GetmaxShieldTime)))
    (elif (Variables|Default|GetisShieldActive) ; check if shield is on
      ;[0 1 0.07377] Subtracting from shield timer, shield is active
      (Variables|Default|SetShield%20Timer (- (Variables|Default|GetShield%20Timer) DeltaSeconds))
      (if (<= (Variables|Default|GetShield%20Timer) 0.0)
        (Variables|Default|SetisDestroyed true)
        (CallFunction|DeactivateShield)
        (CallFunction|BreakShield)
        (Variables|Default|SetShield%20Timer 0.0))
      (else
        ;[1 0 0.01801] adding to shield timer, shield if not active
        (Variables|Default|SetShield%20Timer (+ (Variables|Default|GetShield%20Timer) (* DeltaSeconds 5.0)))
        (if (> (Variables|Default|GetShield%20Timer) _maxshieldtime)
          (Variables|Default|SetShield%20Timer _maxshieldtime))))))

(fn ActivateShield
  (bind _mshield (Variables|Default|GetmShield))
  (Variables|Default|SetisShieldActive true)
  (if (Variables|Default|GetisDestroyed)
    (CallFunction|Fizzle)
    (else
      (Rendering|SetVisibility (Variables|/Game/Blueprints/Shield.Shield_C|GetDefaultSceneRoot _mshield) true true)
      (Collision|SetCollisionEnabled (Variables|/Game/Blueprints/Shield.Shield_C|GetSphere _mshield) "QueryAndPhysics")
      (Variables|Default|SetShield%20Start%20Time (Variables|Default|GetShield%20Timer)))))

(fn CreateShield
  (bind _asbp_main_character (Utilities|Casting|CastToBP_MainCharacter (Components|GetOwner)))
  (Variables|Default|Setowner _asbp_main_character)
  (if (Variables|Default|GetHas%20Shield)
    (bind _returnvalue (Game|SpawnActorfromClass "/Game/Blueprints/Shield.Shield_C" (Math|Conversions|ToTransform(Vector) (Transformation|GetActorLocation (Variables|Default|Getowner))) "AlwaysSpawn" 0 (Variables|Default|Getowner)))
    (Variables|Default|SetmShield _returnvalue)
    (Collision|IgnoreActorwhenMoving (Variables|/Script/Engine.Character|GetCapsuleComponent (Variables|Default|Getowner)) _returnvalue true)
    (Class|SceneComponent|Attachto (Variables|/Game/Blueprints/Shield.Shield_C|GetDefaultSceneRoot _returnvalue) (Variables|/Script/Engine.Character|GetCapsuleComponent (Variables|Default|Getowner)) "None" "KeepWorldPosition" false)
    (CallFunction|DeactivateShield)))

(fn DeactivateShield
  (bind _mshield (Variables|Default|GetmShield))
  (if (Variables|Default|GetisShieldActive)
    (Variables|Default|SetisShieldActive false)
    (Rendering|SetVisibility (Variables|/Game/Blueprints/Shield.Shield_C|GetDefaultSceneRoot _mshield) false true)
    (Collision|SetCollisionEnabled (Variables|/Game/Blueprints/Shield.Shield_C|GetSphere _mshield) "NoCollision")
    (elif (Variables|Default|GetisDestroyed)
      _)))

(fn UpdateShieldColor
  (bind _returnvalue (Rendering|Material|CreateDynamicMaterialInstance "/Game/Particles/Materials/M_Shield.M_Shield" :!class /Script/Engine.KismetMaterialLibrary))
  (Variables|Default|SetShield%20Color (Math|Color|MakeColor (.R (Math|Color|BreakColor (Variables|Default|GetShield%20Color))) (* (Variables|Default|GetMax%20Green) (/ (Variables|Default|GetShield%20Timer) (Variables|Default|GetmaxShieldTime))) (.B (Math|Color|BreakColor (Variables|Default|GetShield%20Color))) (.A (Math|Color|BreakColor (Variables|Default|GetShield%20Color)))))
  (Rendering|Material|SetVectorParameterValue _returnvalue "Base_Color" (Variables|Default|GetShield%20Color) :!class /Script/Engine.MaterialInstanceDynamic)
  (if (Variables|/Game/Blueprints/Character/BP_MainCharacter.BP_MainCharacter_C|GetHas%20Shield%20Upgrade (Variables|Default|Getowner))
    (bind _output_get (Variables|Default|SetIs%20Not%20Reflecting (< (Variables|Default|GetShield%20Timer) (- (Variables|Default|GetShield%20Start%20Time) 0.2))))
    (if _output_get
      (Rendering|Material|SetScalarParameterValue _returnvalue "Opacity" (Variables|Default|GetRegular%20Opacity) :!class /Script/Engine.MaterialInstanceDynamic :!label _label)
      (else
        (Rendering|Material|SetScalarParameterValue _returnvalue "Opacity" (Variables|Default|GetUpgrade%20Opacity) :!class /Script/Engine.MaterialInstanceDynamic)))
    (else
      (goto _label)))
  (Default|SetMaterial (Variables|Default|GetmShield) _returnvalue))

(fn BreakShield
  (bind _returnvalue (Game|SpawnActorfromClass "/Game/Blueprints/BP_ShieldBreak.BP_ShieldBreak_C" (Math|Conversions|ToTransform(Vector) (Transformation|GetWorldLocation (Variables|/Script/Engine.Character|GetMesh (Variables|Default|Getowner)))) "AlwaysSpawn" 0 0))
  (Default|Break _returnvalue)
  (return))

(fn Fizzle
  (Audio|PlaySoundatLocation "/Game/Audio/SC_Fizzle.SC_Fizzle" (Transformation|GetActorLocation (Variables|Default|Getowner))))

(fn PassDamagetoShield
  (params (Damage :type Float%20%28single-precision%29))
  (bind _mshield (Variables|Default|GetmShield))
  (bind _maxshieldtime (Variables|Default|GetmaxShieldTime))
  (bind _shield_health (Variables|/Game/Blueprints/Shield.Shield_C|GetShield%20Health _mshield))
  (if (and (Variables|Default|GetisShieldActive) (> (Variables|Default|GetShield%20Timer) 0.0))
    (bind _output_get (LocalVariables|SetLeftover%20Damage (Math|Float|Absolute(Float) (* (/ (- (Variables|Default|GetShield%20Timer) (* (/ Damage _shield_health) _maxshieldtime)) _maxshieldtime) _shield_health))))
    (bind _output_get_2 (Variables|Default|SetShield%20Timer (- (Variables|Default|GetShield%20Timer) (* (/ Damage _shield_health) _maxshieldtime))))
    (return (Math|Float|SelectFloat _output_get 0.0 (< _output_get_2 0.0)))
    (else
      (return Damage))))