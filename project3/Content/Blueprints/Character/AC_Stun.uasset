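; AC_Stun is a component on BP_MainCharacter that fires a stun ability.
; ActivateStun calls FireStun when Ready, then clears Ready and sets a cooldown, otherwise FizzleStun plays a failure sound.
; FireStun plays a sound, spawns BP_StunField at the owner's StunField, attaches it to the owner and disables its collision.
; The cooldown countdown that restores Ready is disconnected from Tick, so it never runs.
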(event `self.ReceiveBeginPlay`
  (bind _asbp_main_character (cast `/Game/Blueprints/Character/BP_MainCharacter` (`self.GetOwner`))
    (:`then`
      (set `self.Owner` _asbp_main_character))
    (:`CastFailed`
      (`KismetSystemLibrary.PrintString` "ERROR CASTING AC_STUN'S OWNER" true true (struct :`R` 1.0 :`A` 1.0)))))

(event `self.ReceiveTick`
  (params (DeltaSeconds :type "Float (single-precision)")))

(event `Activate Stun`
  (if (`self.Ready`)
    (`self.Fire Stun`)
    (set `self.Cooldown` 5.0)
    (set `self.Ready` false)
    (else
      (`self.Fizzle Stun`))))

(fn `Fire Stun`
  (bind _owner (`self.Owner`))
  (bind _returnvalue (`SceneComponent.GetSocketLocation` (`/Game/Blueprints/Character/BP_MainCharacter.Stun_field` _owner) "None"))
  (`GameplayStatics.PlaySoundAtLocation` "/Game/Audio/SC_Stun.SC_Stun" _returnvalue)
  (bind _returnvalue_2 (`|SpawnActorFromClass` "/Game/Blueprints/Character/BP_StunField.BP_StunField_C" (`KismetMathLibrary.Conv_VectorToTransform` _returnvalue) "AlwaysSpawn" "OverrideRootScale" null _owner))
  (`Actor.K2_AttachRootComponentToActor` _returnvalue_2 _owner "None" "SnapToTargetIncludingScale" true)
  (`Actor.SetActorEnableCollision` _returnvalue_2 false))

(fn `Fizzle Stun`
  (`GameplayStatics.PlaySoundAtLocation` "/Game/Audio/SC_Fizzle.SC_Fizzle" (`Actor.K2_GetActorLocation` (`self.Owner`))))