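; BP_HoTPowerup is a heal-over-time powerup actor that follows its Target and restores that target's health.
; Each Tick, it interpolates its location toward the Target and adds a small fraction of the Target's MaxHealth.
; Both steps use a hardcoded time step of about 1/120 second instead of DeltaSeconds, so follow speed and heal rate depend on frame rate.
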(event `self.ReceiveTick`
  (params (DeltaSeconds :type "Float (single-precision)"))
  (bind _target (`self.Target`))
  (`self.K2_SetActorLocation` (`KismetMathLibrary.VInterpTo` (`self.K2_GetActorLocation`) (`self.K2_GetActorLocation` (`self.Target`)) 0.0083 80.0))
  (`/Game/Blueprints/Character/BP_MainCharacter.Add Health` _target (* (`/Game/Blueprints/Character/BP_MainCharacter.Max Health` _target) 0.1 0.0083)))

(fn `UserConstructionScript`
  (`parent.UserConstructionScript`))