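; Shared versus-mode camera that becomes player 0's view target and frames all pawns registered through VersusGameMode.
; FindFurthestPlayers finds the farthest-apart pair, returning their midpoint and separation as arm length.
; For three or more players it calls FindTriangleMidPoint with a third player, but that function's centroid formula is unconnected.
; Tick interpolates position and spring arm length, capped at MaxDistance, which keys 8 and 9 adjust.
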(event Custom|Player%20Loop)

(event Custom|New%20Pawn_Event_0
  (params (New%20Pawn :type BP%20Main%20Character%20Object%20Reference))
  (Utilities|Array|Add (Variables|Default|GetPlayers) New%20Pawn))

(event EventBeginPlay
  (bind _asversus_game_mode (Utilities|Casting|CastToVersusGameMode (Game|GetGameMode)))
  (EventDispatchers|AssignNewPawn _asversus_game_mode (delegate Custom|New%20Pawn_Event_0))
  (Game|Player|SetViewTargetwithBlend (Game|GetPlayerController 0) self 0.0 "VTBlend_Linear" 0.0 false)
  (bind (_1 _2 _spring_arm_position _arm_length) (CallFunction|FindFurthestPlayers))
  (Transformation|SetActorLocation _spring_arm_position false true)
  (Variables|/Script/Engine.SpringArmComponent|SetTargetArmLength (Variables|Default|GetSpringArm) _arm_length))

(event EventTick
  (params (DeltaSeconds :type Float%20%28single-precision%29))
  (bind _springarm (Variables|Default|GetSpringArm))
  (bind _max_distance (Variables|Default|GetMax%20Distance))
  (if (> (Utilities|Array|Length (Variables|Default|GetPlayers)) 0)
    (bind (_1 _2 _spring_arm_position _arm_length) (CallFunction|FindFurthestPlayers))
    (Transformation|SetActorLocation (Math|Interpolation|VInterpTo (Transformation|GetActorLocation) _spring_arm_position DeltaSeconds 2.0) false false)
    (Variables|/Script/Engine.SpringArmComponent|SetTargetArmLength _springarm (Math|Interpolation|FInterpTo (Variables|/Script/Engine.SpringArmComponent|GetTargetArmLength _springarm) (Math|Float|SelectFloat _max_distance (+ _arm_length (Variables|Default|GetBase%20Offset)) (> (+ _arm_length (Variables|Default|GetBase%20Offset)) _max_distance)) DeltaSeconds 2.0))
    (goto _label Reset)
    (else
      (Utilities|FlowControl|DoOnce false :!label _label))))

(event Input|KeyboardEvents|9
  (params (Key :type Key%20Structure :default "AnyKey"))
  (:Pressed
    (Variables|Default|SetMax%20Distance (- (Variables|Default|GetMax%20Distance) 1e+02))))

(event Input|KeyboardEvents|8
  (params (Key :type Key%20Structure :default "AnyKey"))
  (:Pressed
    (Variables|Default|SetMax%20Distance (+ (Variables|Default|GetMax%20Distance) 1e+02))))

(fn ConstructionScript)

(fn FindFurthestPlayers
  (bind _players (Variables|Default|GetPlayers))
  (bind _returnvalue (Utilities|Array|Length _players))
  (bind _item (Utilities|Array|Get(acopy) _players))
  (if (> _returnvalue 1)
    (for _array_element _players
      (Utilities|IsValid (Variables|/Script/Engine.Character|GetCapsuleComponent _array_element)
        (:Is%20Valid
          (for _array_element_2 _players
            (Utilities|IsValid _array_element_2
              (:Is%20Valid
                (if (> (Math|Vector|VectorLength (- (Transformation|GetWorldLocation (Variables|/Script/Engine.Character|GetMesh _array_element)) (Transformation|GetWorldLocation (Variables|/Script/Engine.Character|GetMesh _array_element_2)))) (LocalVariables|GetLongest%20Distance))
                  (LocalVariables|SetLongest%20Distance (Math|Vector|VectorLength (- (Transformation|GetWorldLocation (Variables|/Script/Engine.Character|GetMesh _array_element)) (Transformation|GetWorldLocation (Variables|/Script/Engine.Character|GetMesh _array_element_2)))))
                  (LocalVariables|SetP1 _array_element)
                  (LocalVariables|SetP2 _array_element_2)
                  (LocalVariables|SetMidpoint (/ (+ (Transformation|GetWorldLocation (Variables|/Script/Engine.Character|GetMesh _array_element)) (Transformation|GetWorldLocation (Variables|/Script/Engine.Character|GetMesh _array_element_2))) 2.0)))))))
        (:Is%20Not%20Valid
          (Utilities|Array|RemoveItem _players _array_element))))
    (if (> _returnvalue 2)
      (bind _array_element_3 (Utilities|Array|ForEachLoopwithBreak (Variables|Default|GetPlayers) :!label _label)
        (:LoopBody
          (if (and (!= (LocalVariables|GetP1) _array_element_3) (!= (LocalVariables|GetP2) _array_element_3))
            (LocalVariables|SetP3 (Transformation|GetActorLocation _array_element_3))
            (goto _label Break)))
        (:Completed
          (Utilities|FlowControl|Sequence
            (:then_1
              (return (LocalVariables|GetP1) (LocalVariables|GetP2) (Math|Vector|MakeVector (Utilities|FindTriangleMidPoint (.X (Math|Vector|BreakVector (LocalVariables|GetMidpoint))) (.X (Math|Vector|BreakVector (LocalVariables|GetP3)))) (Utilities|FindTriangleMidPoint (.Y (Math|Vector|BreakVector (LocalVariables|GetMidpoint))) (.Y (Math|Vector|BreakVector (LocalVariables|GetP3)))) (Utilities|FindTriangleMidPoint (.Z (Math|Vector|BreakVector (LocalVariables|GetMidpoint))) (.Z (Math|Vector|BreakVector (LocalVariables|GetP3))))) (LocalVariables|GetLongest%20Distance))))))
      (else
        (return (LocalVariables|GetP1) (LocalVariables|GetP2) (LocalVariables|GetMidpoint) (LocalVariables|GetLongest%20Distance))))
    (else
      (Utilities|IsValid _item
        (:Is%20Valid
          (return _item 0 (Transformation|GetActorLocation _item) 1.1e+03))
        (:Is%20Not%20Valid
          (return 0 0 (Variables|Default|GetDesired%20Position) (Variables|Default|GetCurrent%20Length)))))))

(fn Initialize
  (bind _players (Variables|Default|GetPlayers))
  (bind _outactors (Actor|GetAllActorsOfClass "/Game/Blueprints/Character/BP_MainCharacter.BP_MainCharacter_C"))
  (Utilities|Array|Clear _players)
  (for _array_element _outactors
    (bind _asbp_main_character (Utilities|Casting|CastToBP_MainCharacter _array_element))
    (Utilities|Array|AddUnique _players _asbp_main_character))
  (bind (_1 _2 _spring_arm_position _arm_length) (CallFunction|FindFurthestPlayers))
  (Transformation|SetActorLocation _spring_arm_position false true)
  (Variables|/Script/Engine.SpringArmComponent|SetTargetArmLength (Variables|Default|GetSpringArm) (+ _arm_length (Variables|Default|GetBase%20Offset))))