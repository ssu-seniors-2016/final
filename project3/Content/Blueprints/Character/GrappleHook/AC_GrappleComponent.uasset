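; AC_GrappleComponent is an actor component that gives BP_MainCharacter a grappling hook it can fire.
; BeginPlay caches the owning character and prints a warning if the cast fails.
; Fire spawns a BP_Hook at the mesh's BulletSocket with a normalized direction, only when the hook is neither firing nor attached.
; Tick branches on the firing, attached and pulling states, but its pull logic is still empty.
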(event `self.ReceiveBeginPlay`
  (bind _asbp_main_character (cast `/Game/Blueprints/Character/BP_MainCharacter` (`self.GetOwner`))
    (:`then`
      (set `self.Owner` _asbp_main_character))
    (:`CastFailed`
      (`KismetSystemLibrary.PrintString` "AC_HookComponent: Owned by a non-player?"))))

(event `self.ReceiveTick`
  (params (DeltaSeconds :type "Float (single-precision)"))
  (if (`self.IsFiring`)
    _
    (elif (`self.IsAttached`)
      (if (`self.IsPulling`)
        _))))

(fn `Fire`
  (params (Dir :type "Vector Structure"))
  (bind _owner (`self.Owner`))
  (if (`KismetMathLibrary.BooleanNOR` (`self.IsFiring`) (`self.IsAttached`))
    (set `self.IsFiring` true)
    (bind _returnvalue (`|SpawnActorFromClass` "/Game/Blueprints/Character/GrappleHook/BP_Hook.BP_Hook_C" (`SceneComponent.GetSocketTransform` (`Character.Mesh` _owner) "BulletSocket" "RTS_World") "AlwaysSpawn" "OverrideRootScale" _owner (`KismetMathLibrary.Normal` Dir) _owner))
    (set `self.Hook` _returnvalue)))