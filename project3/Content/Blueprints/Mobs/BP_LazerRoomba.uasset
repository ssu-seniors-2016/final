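; Roomba mob that patrols between its spawn point and a PatrolLocation offset while pulsing a laser on and off.
; Tick runs the state machine: Waiting traces along its local down and eases onto the surface, restoring gravity only if IsOnGround; Roaming moves and reverses at endpoints.
; Attacking just returns to Roaming.
; The laser is a child BP_WallLaser, reconfigured as movable with its node hidden and toggled by a timer.
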(event `self.ReceiveTick`
  (params (DeltaSeconds :type "Float (single-precision)"))
  (bind _charactermovement (`self.CharacterMovement`))
  (bind _returnvalue (`KismetMathLibrary.SelectVector` (`self.End Location`) (`self.Start Location`) (> (`self.Movement Direction`) 0.0)))
  (switch `/Game/Blueprints/Mobs/E_MobState` (`self.Mob State`)
    (:`NewEnumerator0`
      ;[0.001401 0.4552 1] this makes the roomba fall it's "down" till it finds the floor then starts its wandering.
      (set `CharacterMovementComponent.GravityScale` 0.0 _charactermovement)
      (set `MovementComponent.Velocity` (0.0 0.0 0.0) _charactermovement)
      (bind (_out_length _outhit _returnvalue_2) (`/Game/Blueprints/FunctionLibraries/BPL_LineTraceFunctions.Channel Trace Actor Vector` self -300.0 "TraceTypeQuery1" (`|MakeArray` null :!type "Actor Object Reference") "ForDuration" true false (`self.GetActorUpVector`)))
      (if _returnvalue_2
        (`self.K2_SetActorLocation` (`KismetMathLibrary.VInterpTo` (`self.K2_GetActorLocation`) (`.Location` (`GameplayStatics.BreakHitResult` _outhit)) DeltaSeconds 30.0) true)
        (if (< _out_length 50.0)
          (set `self.Mob State` "NewEnumerator1")
          (if (`self.Is On Ground`)
            (set `CharacterMovementComponent.GravityScale` 1.0 (`self.CharacterMovement`))))))
    (:`NewEnumerator1`
      (`self.Toggle lasers` DeltaSeconds)
      ;[1 0.02056 0.9663] roams back and forth between its stat and end location
      (if (== (`self.K2_GetActorLocation`) _returnvalue :`ErrorTolerance` 10.0)
        (`/Game/Blueprints/Mobs/BML_EnemyMacros.Reverse Direction`)
        (else
          (`/Game/Blueprints/Mobs/BML_EnemyMacros.Move Toward` _returnvalue (`self.Movement Speed`)))))
    (:`NewEnumerator2`
      (set `self.Mob State` "NewEnumerator1"))))

(event `self.ReceiveBeginPlay`
  (`parent.ReceiveBeginPlay`)
  (`KismetSystemLibrary.Delay` 0.2)
  (`/Game/Blueprints/Environment/Hazards/Lazer/BP_WallLaser.ToggleLasers` (`self.Actual laser`))
  (set `self.Start Location` (`self.K2_GetActorLocation`))
  (set `self.End Location` (`KismetMathLibrary.TransformLocation` (`self.GetTransform`) (`self.Patrol Location`))))

(event `self.ReceiveAnyDamage`
  (params (Damage :type "Float (single-precision)") (DamageType :type "DamageType Object Reference") (InstigatedBy :type "Controller Object Reference") (DamageCauser :type "Actor Object Reference"))
  (`parent.ReceiveAnyDamage` Damage null null null))

(fn `Toggle lasers`
  (params (`Delta time` :type "Float (double-precision)"))
  (set `self.Timer` (+ `Delta time` (`self.Timer`)))
  (if (`self.LaserOn`)
    (if (<= (`self.LaserTimeOn`) (`self.Timer`))
      (`/Game/Blueprints/Environment/Hazards/Lazer/BP_WallLaser.ToggleLasers` (`self.Actual laser`))
      (set `self.LaserOn` false)
      (set `self.Timer` 0.0))
    (elif (<= (`self.LaserTimeOff`) (`self.Timer`))
      (`/Game/Blueprints/Environment/Hazards/Lazer/BP_WallLaser.ToggleLasers` (`self.Actual laser`))
      (set `self.LaserOn` true)
      (set `self.Timer` 0.0))))

(fn `UserConstructionScript`
  (bind _actual_laser (`self.Actual laser`))
  (`parent.UserConstructionScript`)
  (bind _asbp_wall_laser (cast `/Game/Blueprints/Environment/Hazards/Lazer/BP_WallLaser` (`ChildActorComponent.ChildActor` (`self.laser`))))
  (bind _output_get (set `self.Actual laser` _asbp_wall_laser))
  (`self.SetOwner` _output_get self)
  (bind _node (`/Game/Blueprints/Environment/Hazards/Lazer/BP_WallLaser.Node` _output_get))
  (`SceneComponent.SetVisibility` _node false false)
  (`PrimitiveComponent.SetCollisionEnabled` _node "NoCollision")
  (set `/Game/Blueprints/Environment/Hazards/Lazer/BP_WallLaser.Emitter Template` "/Game/Blueprints/Environment/Hazards/Lazer/Laser_ParticleSystem2.Laser_ParticleSystem2" _actual_laser)
  (set `/Game/Blueprints/Environment/Hazards/Lazer/BP_WallLaser.isMovable?` true _actual_laser))