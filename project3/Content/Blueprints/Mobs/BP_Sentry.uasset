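; BP_Sentry is an enemy mob that roams and wanders, cannot be grappled, and runs a timed attack on the player.
; Tick switches on MobState; Attacking fires once, checking SightSphere for BP_MainCharacter, then reversing direction, crouching and easing through a 90-degree timeline turn.
; A looping timer then deals damage through three fanned sphere traces until AttackTimeLength expires, when EndAttack restores roaming and resets the DoOnce.
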(event `self.ReceiveTick`
  (params (DeltaSeconds :type "Float (single-precision)"))
  (switch `/Game/Blueprints/Mobs/E_MobState` (`self.Mob State`)
    (:`NewEnumerator0`
      (set `self.Mob State` "NewEnumerator1"))
    (:`NewEnumerator1`
      (`/Game/Blueprints/Mobs/BML_EnemyMacros.Move Forward` (`self.Movement Speed`))
      (`/Game/Blueprints/Mobs/BML_EnemyMacros.Wander`))
    (:`NewEnumerator2`
      (`/Engine/EditorBlueprintResources/StandardMacros.DoOnce` false :!label _label
        (:`Completed`
          (`/Engine/EditorBlueprintResources/StandardMacros.IsValid` (`KismetArrayLibrary.Array_Get` (`PrimitiveComponent.GetOverlappingActors` (`self.Sight Sphere`) "/Game/Blueprints/Character/BP_MainCharacter.BP_MainCharacter_C"))
            (:`Is Valid`
              (`/Game/Blueprints/Mobs/BML_EnemyMacros.Reverse Direction`)
              (`self.Crouch`)
              (`Timeline|90 Degree Turn` :!via `PlayFromStart`
                (:`Update`
                  (`self.SetActorRotation` (`KismetMathLibrary.RInterpTo` (`self.K2_GetActorRotation`) (`KismetMathLibrary.SelectRotator` (struct :`Yaw` -90.0) (struct :`Yaw` 90.0) (> (`self.Movement Direction`) 0.0)) (`GameplayStatics.GetWorldDeltaSeconds`) 5.0)))
                (:`Finished`
                  (`KismetSystemLibrary.K2_SetTimerDelegate` (delegate `Execute Attack`) 0.1 true))))
            (:`Is Not Valid`
              (`self.EndAttack`))))))))

(event `EndAttack`
  (`|ExecutionSequence`
    (:`then_0`
      (`self.UnCrouch`)
      (`/Game/Blueprints/Mobs/BML_EnemyMacros.Reverse Direction`)
      (set `self.Mob State` "NewEnumerator1"))
    (:`then_1`
      (goto _label :!via `Reset`))))

(event `Execute Attack`
  (bind _returnvalue (`self.GetActorForwardVector`))
  (bind _returnvalue_2 (`self.GetActorUpVector`))
  (bind _output_get (set `self.Attack Timer` (+ 0.1 (`self.Attack Timer`))))
  (if (<= _output_get (`self.Attack Time Length`))
    (for _index (range 3)
      (bind (_return_value _outhit) (`/Game/Blueprints/FunctionLibraries/BPL_LineTraceFunctions.Object Sphere Trace Vector` self (select `int` _index :`0` _returnvalue :`1` (- _returnvalue _returnvalue_2) :`2` (* _returnvalue_2 -1.0)) -280.0 (`|MakeArray` "ObjectTypeQuery3" :!type "EObjectTypeQuery Enum") false (`|MakeArray` null :!type "Actor Object Reference") "ForDuration" true 45.0))
      (bind _asbp_main_character (cast `/Game/Blueprints/Character/BP_MainCharacter` (`.HitActor` (`GameplayStatics.BreakHitResult` _outhit))))
      (`GameplayStatics.ApplyDamage` _asbp_main_character 2.0 null self "/Game/Blueprints/Character/BP_DamageTypeBasic.BP_DamageTypeBasic_C"))
    (else
      (`KismetSystemLibrary.K2_SetTimerDelegate` (delegate `Execute Attack`))
      (set `self.Attack Timer` 0.0)
      (`self.EndAttack`))))

(fn `CanBeGrappled`
  (returns (`Yes?` :type Boolean))
  (return false))

(fn `UserConstructionScript`
  (`parent.UserConstructionScript`))