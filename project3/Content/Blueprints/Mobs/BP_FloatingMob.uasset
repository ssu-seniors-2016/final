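; BP_FloatingMob is a flying enemy that patrols between two points and shoots at the player.
; A Tick state machine switches between roaming and attacking using sight-sphere overlaps and line-of-sight checks.
; While attacking, it turns toward the target and fires lime bullets with randomized aim, continuing its patrol unless StopToAttack is set.
; Being grappled disables flight before the delayed grapple, and player detachment makes it explode.
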(event `self.ReceiveBeginPlay`
  (`parent.ReceiveBeginPlay`)
  (set `self.Start Location` (`self.K2_GetActorLocation`))
  (if (not (`self.Spawned`))
    (set `self.End Location` (`KismetMathLibrary.TransformLocation` (`self.GetTransform`) (`self.Patrol Location`))))
  (`/Game/Blueprints/Character/AC_GunComponent.Change Bullet Type` (`self.AC_GunComponent`) "/Game/Blueprints/Weapons/BP_LimeBullet.BP_LimeBullet_C")
  (`self.SetActorTickEnabled` true))

(event `self.ReceiveTick`
  (params (DeltaSeconds :type "Float (single-precision)"))
  (bind _returnvalue (`self.K2_GetActorLocation`))
  (bind _overlappingactors (`PrimitiveComponent.GetOverlappingActors` (`self.Sight Sphere`) "/Game/Blueprints/Character/BP_MainCharacter.BP_MainCharacter_C"))
  (bind _returnvalue_2 (`self.K2_GetActorLocation` (`self.Attack Target`)))
  (bind _item (`KismetArrayLibrary.Array_Get` _overlappingactors))
  (bind _returnvalue_3 (`KismetMathLibrary.SelectVector` (`self.End Location`) (`self.Start Location`) (> (`self.Movement Direction`) 0.0)))
  (switch `/Game/Blueprints/Mobs/E_MobState` (`self.Mob State`)
    (:`NewEnumerator0`
      (set `self.Mob State` "NewEnumerator1" :!label _label))
    (:`NewEnumerator1`
      (if (== (`KismetArrayLibrary.Array_Length` _overlappingactors) 0)
        (if (== (`self.K2_GetActorLocation`) _returnvalue_3 :`ErrorTolerance` 10.0) :!label _label_2
          (`/Game/Blueprints/Mobs/BML_EnemyMacros.Reverse Direction`)
          (else
            (`/Game/Blueprints/Mobs/BML_EnemyMacros.Move Toward` _returnvalue_3)))
        (else
          (`/Game/Blueprints/Mobs/BML_EnemyMacros.Is Player in Sight?` _item
            (:`true`
              (set `self.Mob State` "NewEnumerator2"))
            (:`false`
              (set `self.Attack Target` null)
              (goto _label_2))))))
    (:`NewEnumerator2`
      (`/Engine/EditorBlueprintResources/StandardMacros.IsValid` (`self.Attack Target`)
        (:`Is Valid`
          _)
        (:`Is Not Valid`
          (`/Engine/EditorBlueprintResources/StandardMacros.IsValid` _item
            (:`Is Valid`
              (bind _output_get (set `self.Attack Target` _item)))
            (:`Is Not Valid`
              (goto _label)))))
      (`/Game/Blueprints/Mobs/BML_EnemyMacros.Is Player in Sight?` _output_get
        (:`true`
          (`|ExecutionSequence`
            (:`then_0`
              (`self.SetActorRotation` (`KismetMathLibrary.MakeRotator` 0.0 0.0 (.yaw (`KismetMathLibrary.RInterpTo_Constant` (`self.K2_GetActorRotation`) (`KismetMathLibrary.FindLookAtRotation` _returnvalue _returnvalue_2) (`GameplayStatics.GetWorldDeltaSeconds`) 500.0)))))
            (:`then_1`
              (`/Game/Blueprints/Character/AC_GunComponent.Fire Bullet` (`self.AC_GunComponent`) (`KismetMathLibrary.Normal` (- (`KismetMathLibrary.RandomPointInBoundingBox` _returnvalue_2 (`KismetMathLibrary.MakeVector` 40.0 40.0 100.0)) _returnvalue)))
              (if (not (`self.Stop to Attack?`))
                (goto _label_2)))))
        (:`false`
          (set `self.Attack Target` null)
          (goto _label))))))

(event `/Game/Blueprints/Character/GrappleHook/BPI_Grapple_Interface.GetGrappled`
  (params (Grabber :type "Character Object Reference"))
  (if (`|EnumInequality` (`self.Mob State`) "NewEnumerator3")
    (`|ExecutionSequence`
      (:`then_0`
        (`self.Disable Flight and Fall`)
        (set `self.Mob State` "NewEnumerator3"))
      (:`then_1`
        (`KismetSystemLibrary.Delay` (* (`GameplayStatics.GetWorldDeltaSeconds`) 5.0))
        (`/Game/Blueprints/Character/GrappleHook/BPL_GrappleFunctions.BasicGetGrappled` Grabber self)))))

(event `/Game/Blueprints/Character/GrappleHook/BPI_Grapple_Interface.PlayerDetatched`
  (params (Player :type "Character Object Reference"))
  (`self.Explode and Destory`))

(fn `CanBeGrappled`
  (returns (`Yes?` :type Boolean))
  (bind _yes_ (`parent.CanBeGrappled`))
  (return _yes_))

(fn `ChangePatrolLocation`
  (params (`New Patrol` :type "Vector Structure"))
  (bind _output_get (set `self.Patrol Location` `New Patrol`))
  (set `self.Start Location` (`self.K2_GetActorLocation`))
  (set `self.End Location` (`KismetMathLibrary.TransformLocation` (`self.GetTransform`) _output_get)))

(fn `Disable Flight and Fall`
  (bind _charactermovement (`self.CharacterMovement`))
  (set `CharacterMovementComponent.GravityScale` 1.0 _charactermovement)
  (set `CharacterMovementComponent.FallingLateralFriction` 0.0 _charactermovement)
  (set `CharacterMovementComponent.AirControl` 0.0 _charactermovement)
  (`CharacterMovementComponent.SetMovementMode` _charactermovement "MOVE_Walking" 0))

(fn `UserConstructionScript`
  (`parent.UserConstructionScript`))