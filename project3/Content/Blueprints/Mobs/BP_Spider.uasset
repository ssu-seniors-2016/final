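; Spider mob with two behaviors, aggressive leaper or passive crawler, driven on Tick by a Waiting, Roaming and Attacking state switch.
; Passive crawlers disable sight and gravity, then trace along their negative up vector to settle on a surface before roaming.
; Roaming calls MoveForward and Wander through a Gate that a looping timer randomly closes for short pauses.
; Attacking repeats velocity-driven leaps toward the player while visible, otherwise returning to Roaming.
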(event `self.ReceiveTick`
  (params (DeltaSeconds :type "Float (single-precision)"))
  (bind _charactermovement (`self.CharacterMovement`))
  (bind _item (`KismetArrayLibrary.Array_Get` (`PrimitiveComponent.GetOverlappingActors` (`self.Sight Sphere`) "/Game/Blueprints/Character/BP_MainCharacter.BP_MainCharacter_C")))
  (switch `/Game/Blueprints/Mobs/E_MobState` (`self.Mob State`)
    (:`NewEnumerator0`
      ;[1 1 1] Initialize passive spider by tracing to a walkable surface
      (switch `/Game/Blueprints/Mobs/E_SpiderBehavior` (`self.Behavior`)
        (:`NewEnumerator0`
          (set `self.Mob State` "NewEnumerator1"))
        (:`NewEnumerator1`
          (set `CharacterMovementComponent.GravityScale` 0.0 _charactermovement)
          (set `MovementComponent.Velocity` (0.0 0.0 0.0) _charactermovement)
          (bind (_out_length _outhit _returnvalue) (`/Game/Blueprints/FunctionLibraries/BPL_LineTraceFunctions.Channel Trace Actor Vector` self -300.0 "TraceTypeQuery1" (`|MakeArray` null :!type "Actor Object Reference") "ForDuration" true false (`self.GetActorUpVector`)))
          (if _returnvalue
            (`self.K2_SetActorLocation` (`KismetMathLibrary.VInterpTo` (`self.K2_GetActorLocation`) (`.Location` (`GameplayStatics.BreakHitResult` _outhit)) DeltaSeconds 30.0) true)
            (if (< _out_length 50.0)
              (set `self.Mob State` "NewEnumerator1"))))))
    (:`NewEnumerator1`
      (`/Engine/EditorBlueprintResources/StandardMacros.Gate` false :!label _label
        (:`Exit`
          (`/Game/Blueprints/Mobs/BML_EnemyMacros.Move Forward` 8.0)
          (`/Game/Blueprints/Mobs/BML_EnemyMacros.Wander`))))
    (:`NewEnumerator2`
      ;[1 1 1] Attack the player as long as he's within sight
      (`/Engine/EditorBlueprintResources/StandardMacros.DoOnce` false :!label _label_2
        (:`Completed`
          (`self.Jump`)
          (set `MovementComponent.Velocity` (* (`self.Attack Direction`) (`self.Jump Speed`)) (`self.CharacterMovement`))
          (`KismetSystemLibrary.Delay` 2.0)
          (`/Engine/EditorBlueprintResources/StandardMacros.IsValid` _item
            (:`Is Valid`
              (`/Game/Blueprints/Mobs/BML_EnemyMacros.Is Player in Sight?` _item ; if player is in sight, reset do once node to allow another attack
                (:`true`
                  (set `self.Attack Direction` (`KismetMathLibrary.Normal` (- (`self.K2_GetActorLocation` _item) (`self.K2_GetActorLocation`))))
                  (goto _label_2 :!via `Reset`))
                (:`false`
                  _)))
            (:`Is Not Valid`
              _))
          (set `self.Mob State` "NewEnumerator1")
          (goto _label_2 :!via `Reset`))))))

(event `Skitter Delay`
  ;[1 1 1] Sit around and do nothing for a random amount of time
  (`|ExecutionSequence`
    (:`then_0`
      (set `MovementComponent.Velocity` (0.0 0.0 0.0) (`self.CharacterMovement`)) ; zero out velocity and close movement gate
      (goto _label :!via `Close`))
    (:`then_1`
      (`KismetSystemLibrary.Delay` (`KismetMathLibrary.RandomFloatInRange` 0.5 4.5))
      (set `self.Movement Direction` (`KismetMathLibrary.SignOfFloat` (`KismetMathLibrary.RandomFloatInRange` -1.0 1.0)))
      (goto _label :!via `Open`))))

(event `self.ReceiveBeginPlay`
  ;[1 1 1] 1/20 chance to sit around and do nothing.  Checked every 1 second.
  (`self.Initialize`)
  (`KismetSystemLibrary.K2_SetTimerDelegate` (delegate `SkitterTrigger`) 1.0 true)
  (switch `/Game/Blueprints/Mobs/E_SpiderBehavior` (`self.Behavior`)
    (:`NewEnumerator1`
      (`PrimitiveComponent.SetCollisionResponseToAllChannels` (`self.Sight Sphere`) "ECR_Ignore") ; turn off sight on the wandering spider
    )))

(event `SkitterTrigger`
  ;[1 1 1] 1/20 chance to sit around and do nothing.  Checked every 1 second.
  (if (and (== (`KismetMathLibrary.RandomIntegerInRange` 1 20) 13) (`|EnumInequality` (`self.Mob State`) "NewEnumerator2"))
    (`self.Skitter Delay`)))

(fn `UserConstructionScript`
  (`parent.UserConstructionScript`))