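; A Versus-mode wrap-around volume that teleports characters and bullets entering its box to the capsule of its linked MirrorEnd.
; Characters move by actor location, or by mesh location when their hips are simulating physics, so ragdolls wrap too.
; Bullets have their particle system deactivated before the teleport and reactivated after a zero-length delay if still valid.
; Enemy teleporting is present but unwired, and other skeletal mesh overlaps only print a debug string.
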(event `self.ReceiveBeginPlay`)

(event `self.ReceiveActorBeginOverlap`
  (params (OtherActor :type "Actor Object Reference")))

(event `self.ReceiveTick`
  (params (DeltaSeconds :type "Float (single-precision)")))

(event `self.Box.OnComponentBeginOverlap`
  (params (OtherActor :type "Actor Object Reference") (OtherComp :type "PrimitiveComponent Object Reference") (OtherBodyIndex :type Integer) (bFromSweep :type Boolean) (SweepResult :type "HitResult Structure (by ref)"))
  (bind _returnvalue (`SceneComponent.K2_GetComponentLocation` (`/Game/Blueprints/Versus/BP_WrapAroundVolume.Capsule` (`self.Mirror End`))))
  (bind _asbp_main_character (cast `/Game/Blueprints/Character/BP_MainCharacter` OtherActor)
    (:`then`
      (bind _mesh (`Character.Mesh` _asbp_main_character))
      (if (`SceneComponent.IsSimulatingPhysics` _mesh "Hips")
        (`SceneComponent.K2_SetWorldLocation` _mesh (`SceneComponent.K2_GetComponentLocation` (`/Game/Blueprints/Versus/BP_WrapAroundVolume.Capsule` (`self.Mirror End`))) false true)
        (else
          (`self.K2_SetActorLocation` _asbp_main_character _returnvalue false true))))
    (:`CastFailed`
      (bind _asbp_projectile_bullet_parent (cast `/Game/Blueprints/Weapons/BP_ProjectileBulletParent` OtherActor)
        (:`then`
          (bind _particlesystem (`/Game/Blueprints/Weapons/BP_ProjectileBulletParent.ParticleSystem` _asbp_projectile_bullet_parent))
          (`ActorComponent.Deactivate` _particlesystem)
          (`self.K2_SetActorLocation` _asbp_projectile_bullet_parent _returnvalue false true)
          (`KismetSystemLibrary.Delay` 0.0)
          (`/Engine/EditorBlueprintResources/StandardMacros.IsValid` _asbp_projectile_bullet_parent
            (:`Is Valid`
              (`ActorComponent.Activate` _particlesystem false))))
        (:`CastFailed`
          (cast `SkeletalMeshComponent` OtherComp)
          (`KismetSystemLibrary.PrintString` "Hello"))))))

(fn `UserConstructionScript`)