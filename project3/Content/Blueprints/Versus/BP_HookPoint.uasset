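; BP_HookPoint is a Versus-mode spawn point that places weapon or health pickups at its transform.
; It raises FreedUp when the spawned pickup is picked up or destroyed, or when spawning fails, so the point can be reused.
; The construction script shows a preview mesh for the point's type: a capsule for pickup types, or the configured drone, Roomba or spider model for enemies.
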(event `Picked Up_Event_0`
  (params (Player :type "/Game/Blueprints/Character/BP_MainCharacter Object Reference"))
  (`self.Freed Up` self :!label _label))

(event `OnDestroyed_Event_1`
  (goto _label))

(event `Spawn Weapon Pickup`
  (params (Class :type "/Game/Blueprints/Environment/BP_Weapon_Pickup Class Reference"))
  (bind _returnvalue (`|SpawnActorFromClass` Class (`self.GetTransform`) "AlwaysSpawn" "OverrideRootScale"))
  (`/Engine/EditorBlueprintResources/StandardMacros.IsValid` _returnvalue
    (:`Is Valid`
      (add `/Game/Blueprints/Environment/BP_Pickup.Picked Up` _returnvalue (delegate `Picked Up_Event_0`))
      (add `self.OnDestroyed` _returnvalue (delegate `OnDestroyed_Event_1`)))
    (:`Is Not Valid`
      (`self.Freed Up` self))))

(event `Spawn Health Pickup`
  (bind _returnvalue (`|SpawnActorFromClass` "/Game/Blueprints/Environment/BP_Pickup_Health.BP_Pickup_Health_C" (`self.GetTransform`) "AlwaysSpawn" "OverrideRootScale"))
  (`/Engine/EditorBlueprintResources/StandardMacros.IsValid` _returnvalue
    (:`Is Valid`
      (add `/Game/Blueprints/Environment/BP_Pickup.Picked Up` _returnvalue (delegate `CustomEvent_0`))
      (add `self.OnDestroyed` _returnvalue (delegate `OnDestroyed_Event_0`)))
    (:`Is Not Valid`
      (`self.Freed Up` self))))

(event `CustomEvent_0`
  (params (Player :type "/Game/Blueprints/Character/BP_MainCharacter Object Reference"))
  (`self.Freed Up` self :!label _label_2))

(event `OnDestroyed_Event_0`
  (goto _label_2))

(fn `UserConstructionScript`
  (bind _preview_skeletal (`self.Preview Skeletal`))
  (bind _preview_static (`self.Preview Static`))
  (switch `/Game/Blueprints/Versus/E_HookPointType` (`self.Hook Point Type`)
    (:`NewEnumerator0`
      (`StaticMeshComponent.SetStaticMesh` _preview_static "/Game/3D_Assets/Weapons/ItemCapsule/SM_Item_Capsule.SM_Item_Capsule" :!label _label))
    (:`NewEnumerator1`
      (goto _label))
    (:`NewEnumerator2`
      (goto _label))
    (:`NewEnumerator3`
      (goto _label))
    (:`NewEnumerator4`
      (switch `/Game/Blueprints/Versus/E_HookEnemySetting` (`self.Enemy Settings`)
        (:`NewEnumerator0`
          (`SkinnedMeshComponent.SetSkinnedAssetAndUpdate` _preview_skeletal "/Game/3D_Assets/Enemies/JellyFishDrone/SK_JellyfishDrone.SK_JellyfishDrone"))
        (:`NewEnumerator1`
          (`StaticMeshComponent.SetStaticMesh` _preview_static "/Game/3D_Assets/Enemies/SatelliteDishDrone/SM_SatelliteDishDrone.SM_SatelliteDishDrone"))
        (:`NewEnumerator2`
          (`SkinnedMeshComponent.SetSkinnedAssetAndUpdate` _preview_skeletal "/Game/3D_Assets/Enemies/SpiderBot/SK_Prison_SpiderBot.SK_Prison_SpiderBot" :!label _label_2))
        (:`NewEnumerator3`
          (goto _label_2))))))