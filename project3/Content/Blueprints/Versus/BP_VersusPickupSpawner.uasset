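; Versus-mode pickup spawner that periodically places health and weapon pickups at BP_HookPoint actors, as the deathmatch rules allow.
; At BeginPlay it sorts hook points into health and weapon pools by type, prunes locked weapons and starts looping timers.
; Each spawn takes a random point out of the pools, with weapon picks checked against the last one to avoid repeats.
; Points rejoin their pools through each hook point's FreedUp event.
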(event Custom|Freed%20Up_Event_1
  (params (Hook%20Point :type BP%20Hook%20Point%20Object%20Reference))
  (Utilities|Array|AddUnique (Variables|Default|GetHealth%20Only%20Hook%20Points) Hook%20Point)
  (if (Utilities|Enum|Equal(Enum) (Variables|/Game/Blueprints/Versus/BP_HookPoint.BP_HookPoint_C|GetHook%20Point%20Type Hook%20Point) "NewEnumerator0")
    (Utilities|Array|AddUnique (Variables|Default|GetWeapon%20Only%20Hook%20Points) Hook%20Point)))

(event Custom|Freed%20Up_Event_2
  (params (Hook%20Point :type BP%20Hook%20Point%20Object%20Reference))
  (Utilities|Array|AddUnique (Variables|Default|GetWeapon%20Only%20Hook%20Points) Hook%20Point)
  (if (Utilities|Enum|Equal(Enum) (Variables|/Game/Blueprints/Versus/BP_HookPoint.BP_HookPoint_C|GetHook%20Point%20Type Hook%20Point) "NewEnumerator0")
    (Utilities|Array|AddUnique (Variables|Default|GetHealth%20Only%20Hook%20Points) Hook%20Point)))

(event EventBeginPlay
  (bind _health_only_hook_points (Variables|Default|GetHealth%20Only%20Hook%20Points))
  (bind _weapon_only_hook_points (Variables|Default|GetWeapon%20Only%20Hook%20Points))
  (bind _asbp_instance_main (Utilities|Casting|CastToBP_Instance_Main (Game|GetGameInstance)))
  (bind _outactors (Actor|GetAllActorsOfClass "/Game/Blueprints/Versus/BP_HookPoint.BP_HookPoint_C"))
  (for _array_element _outactors
    (switch Utilities|FlowControl|Switch|SwitchonE_HookPointType (Variables|/Game/Blueprints/Versus/BP_HookPoint.BP_HookPoint_C|GetHook%20Point%20Type _array_element)
      (:NewEnumerator0
        (Utilities|Array|AddUnique _health_only_hook_points _array_element)
        (Utilities|Array|AddUnique _weapon_only_hook_points _array_element))
      (:NewEnumerator1
        (Utilities|Array|AddUnique _health_only_hook_points _array_element))
      (:NewEnumerator2
        (Utilities|Array|AddUnique _weapon_only_hook_points _array_element))))
  (Utilities|FlowControl|Sequence
    (:then_0
      (if (.HealthPickups (Utilities|Struct|BreakDeathMatchRules (Variables|/Game/Blueprints/BP_Instance_Main.BP_Instance_Main_C|GetDeathmatch%20Rules _asbp_instance_main)))
        (if (> (Utilities|Array|Length (Variables|Default|GetHealth%20Only%20Hook%20Points)) 0)
          (Utilities|Time|SetTimerbyFunctionName 0 "Spawn Health Pickups" 3e+01 true))))
    (:then_1
      (if (.WeaponPickups (Utilities|Struct|BreakDeathMatchRules (Variables|/Game/Blueprints/BP_Instance_Main.BP_Instance_Main_C|GetDeathmatch%20Rules _asbp_instance_main)))
        (if (> (Utilities|Array|Length (Variables|Default|GetWeapon%20Only%20Hook%20Points)) 0)
          (CallFunction|InitBulletArray (.UnlockedBullets (Utilities|Struct|BreakDeathMatchRules (Variables|/Game/Blueprints/BP_Instance_Main.BP_Instance_Main_C|GetDeathmatch%20Rules _asbp_instance_main))))
          (CallFunction|SpawnWeaponPickups)
          (Utilities|Time|SetTimerbyFunctionName 0 "Spawn Weapon Pickups" 5.0 true))))
    (:then_2
      (for _array_element_2 (Variables|Default|GetHealth%20Only%20Hook%20Points)
        (EventDispatchers|AssignFreedUp _array_element_2 (delegate Custom|Freed%20Up_Event_1)))
      (for _array_element_3 (Variables|Default|GetWeapon%20Only%20Hook%20Points)
        (EventDispatchers|AssignFreedUp _array_element_3 (delegate Custom|Freed%20Up_Event_2))))))

(fn ConstructionScript)

(fn SpawnHealthPickups
  (bind _health_only_hook_points (Variables|Default|GetHealth%20Only%20Hook%20Points))
  (bind _item (Utilities|Array|Get(acopy) _health_only_hook_points))
  (Utilities|Array|Shuffle _health_only_hook_points)
  (Utilities|IsValid _item
    (:Is%20Valid
      (Default|SpawnHealthPickup _item)
      (Utilities|Array|RemoveItem (Variables|Default|GetWeapon%20Only%20Hook%20Points) _item)
      (Utilities|Array|RemoveIndex _health_only_hook_points))))

(fn SpawnWeaponPickups
  (bind _returnvalue (Math|Random|RandomInteger 7200))
  (bind _spawnable_weapons (Variables|Default|GetSpawnable%20Weapons))
  (bind _weapon_only_hook_points (Variables|Default|GetWeapon%20Only%20Hook%20Points))
  (bind _item (Utilities|Array|Get(acopy) _weapon_only_hook_points))
  (bind _returnvalue_2 (Utilities|Array|Length _spawnable_weapons))
  (bind _returnvalue_3 (Math|Random|MakeRandomStream _returnvalue))
  (bind _returnvalue_4 (Class|KismetMathLibrary|RandomIntegerfromStream _returnvalue_2 _returnvalue_3))
  (bind _item_2 (Utilities|Array|Get(acopy) _spawnable_weapons _returnvalue_4))
  (Utilities|Array|Shuffle _weapon_only_hook_points)
  (Utilities|IsValid _item
    (:Is%20Valid
      (if (== _item_2 (Variables|Default|GetLast%20Spawn))
        (bind _array_element (Utilities|Array|ForEachLoopwithBreak _spawnable_weapons :!label _label)
          (:LoopBody
            (if (!= _array_element (Variables|Default|GetLast%20Spawn))
              (LocalVariables|SetLoopResult _array_element)
              (goto _label Break))))
        (else
          (Default|SpawnWeaponPickup _item _item_2)
          (Variables|Default|SetLast%20Spawn (select (!= (LocalVariables|GetLoopResult) 0) (LocalVariables|GetLoopResult) _item_2))
          (Utilities|Array|RemoveItem (Variables|Default|GetHealth%20Only%20Hook%20Points) _item)
          (Utilities|Array|RemoveIndex _weapon_only_hook_points))))))

(fn InitBulletArray
  (params (Array :type Array%20of%20Booleans))
  (bind _spawnable_weapons (Variables|Default|GetSpawnable%20Weapons))
  (bind _guns_removed (LocalVariables|GetGuns%20Removed))
  (for (_array_element _array_index) Array
    (if (not _array_element)
      (Utilities|Array|RemoveIndex _spawnable_weapons (- _array_index _guns_removed))
      (Math|Integer|IncrementInt _guns_removed)))
  (for _array_element_2 _spawnable_weapons
    _)
  (return))