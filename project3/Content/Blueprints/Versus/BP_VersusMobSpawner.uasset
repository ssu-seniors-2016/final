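; Versus-mode spawner that places jellyfish drones, roombas and spiders at enemy BP_HookPoints, removing itself when disabled or without points.
; EnemySwitch picks easy or hard caps, start delay and wave interval.
; Recursive Spawn fills shuffled, pawn-free points, tracking live enemies via death delegates; at cap, waves add to a queue serviced by a pausable timer.
; Optional health-orb odds rise with SpawnsSinceLastOrb, whose reset branch is hard-wired off.
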(event Custom|BindEnemyDelegates
  (params (New%20Enemy :type BP%20Enemy%20Object%20Reference))
  (EventDispatchers|AssignHasBeenKilled New%20Enemy (delegate Custom|Has%20Been%20Killed_Event_0)))

(event Custom|Has%20Been%20Killed_Event_0
  (Math|Integer|DecrementInt (Variables|Default|GetCurrent%20Enemies%20Active)))

(event EventBeginPlay
  (bind _enemy_switch (Variables|Default|GetEnemy%20Switch))
  (switch int _enemy_switch
    (:0
      (Actor|DestroyActor))
    (:1
      (Variables|Default|SetTime%20Limit (- (Variables|Default|GetTime%20Limit) 20))
      (Utilities|SetupActorArray
        (:Completed
          (Utilities|FlowControl|Delay 2e+01)
          (CallFunction|Spawn :!label _label)
          (Utilities|Time|SetTimerbyFunctionName 0 "Spawn" (Utilities|Select :Index _enemy_switch :Option%200 0.0 :Option%201 3e+01 :Option%202 15.0) true)
          (bind _returnvalue (Utilities|Time|SetTimerbyFunctionName 0 "Spawn Queued Enemies" 1.0 true))
          (Variables|Default|SetSpawn%20Queue%20Timer _returnvalue))))
    (:2
      (Variables|Default|SetTime%20Limit (- (Variables|Default|GetTime%20Limit) 10))
      (Utilities|SetupActorArray
        (:Completed
          (Utilities|FlowControl|Delay 1e+01)
          (goto _label))))))

(fn ConstructionScript)

(fn Spawn
  (bind _enemy_switch (Variables|Default|GetEnemy%20Switch))
  (bind _easy_enemy_count (Variables|Default|GetEasy%20Enemy%20Count))
  (bind _hard_enemy_count (Variables|Default|GetHard%20Enemy%20Count))
  (bind _spawn_queue_timer (Variables|Default|GetSpawn%20Queue%20Timer))
  (bind _returnvalue (Utilities|Select :Index _enemy_switch :Option%200 0 :Option%201 _easy_enemy_count :Option%202 _hard_enemy_count))
  (bind _output_get (LocalVariables|SetSuccesful%20Spawns (Variables|Default|GetCurrent%20Enemies%20Active)))
  (if (>= _output_get _returnvalue)
    (Variables|Default|SetQueued%20Enemies (+ (Variables|Default|GetQueued%20Enemies) _returnvalue))
    (if (Class|KismetSystemLibrary|IsTimerPausedHandle _spawn_queue_timer)
      (Utilities|Time|UnpauseTimerbyHandle _spawn_queue_timer))
    (else
      (bind _bool2 (Utilities|TrytoSpawnAnEnemy (LocalVariables|GetSpawning)))
      (if _bool2
        (if (not (>= (Variables|Default|GetCurrent%20Enemies%20Active) (Utilities|SelectHardorEasyLimit)))
          (CallFunction|Spawn))))))

(fn SpawnQueuedEnemies
  (if (and (> (Variables|Default|GetCurrent%20Enemies%20Active) (Utilities|SelectHardorEasyLimit)) (> (Variables|Default|GetQueued%20Enemies) 0))
    (bind _bool2 (Utilities|TrytoSpawnAnEnemy (LocalVariables|GetFailed%20Spawn)))
    (if _bool2
      (Math|Integer|DecrementInt (Variables|Default|GetQueued%20Enemies)
        (:%20%20
          _)))
    (else
      (Utilities|Time|PauseTimerbyHandle (Variables|Default|GetSpawn%20Queue%20Timer))))
  (return))