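; BP_CarryObjective is an oddball-style Versus pickup that scores for whichever character carries it.
; Overlapping an eligible character makes it the holder, which the objective follows overhead each Tick until a drop callback clears it.
; A looping timer, scaled from the game mode's time limit and paused on drop, raises per-player scores shown on a countdown widget.
; Reaching ten points declares the winner; the bob animation never runs.
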(event `self.ReceiveTick`
  (params (DeltaSeconds :type "Float (single-precision)"))
  (bind _current_holder (`self.Current Holder`)
    (:`then`
      (`self.K2_SetActorLocation` (+ (`self.K2_GetActorLocation` _current_holder) (0.0 0.0 260.0))))
    (:`else`)))

(event `self.ReceiveBeginPlay`
  (bind _asversus_game_mode (cast `/Game/Blueprints/GameModes/Versus/VersusGameMode` (`GameplayStatics.GetGameMode`)))
  (set `self.Time to Score` (/ (/ (`KismetMathLibrary.Conv_IntToDouble` (`/Game/Blueprints/GameModes/Versus/VersusGameMode.Time Limit` _asversus_game_mode)) 4.0) 10.0))
  (`SceneComponent.SetVisibility` (`self.Widget`) false false))

(event `self.Box.OnComponentBeginOverlap`
  (params (OtherActor :type "Actor Object Reference") (OtherComp :type "PrimitiveComponent Object Reference") (OtherBodyIndex :type Integer) (bFromSweep :type Boolean) (SweepResult :type "HitResult Structure (by ref)"))
  (bind _score_timer_handle (`self.Score Timer Handle`))
  (`self.Current Holder`
    (:`then`)
    (:`else`
      (bind _asbp_main_character (cast `/Game/Blueprints/Character/BP_MainCharacter` OtherActor))
      (bind _state (`/Game/Blueprints/Character/BP_MainCharacter.Get Current State` _asbp_main_character))
      (if (`|EnumInequality` _state "NewEnumerator10")
        (`/Engine/EditorBlueprintResources/StandardMacros.IsValid` (`Pawn.GetController` _asbp_main_character)
          (:`Is Valid`
            (bind _output_get (set `self.Current Holder` _asbp_main_character))
            (add `/Game/Blueprints/Character/BP_MainCharacter.Drop Objective` _output_get (delegate `Drop Objective_Event_0`))
            (if (`KismetSystemLibrary.K2_TimerExistsHandle` _score_timer_handle)
              (`KismetSystemLibrary.K2_UnPauseTimerHandle` _score_timer_handle)
              (else
                (bind _returnvalue (`KismetSystemLibrary.K2_SetTimer` null "ScoreTimer" (`self.Time to Score`) true))
                (set `self.Score Timer Handle` _returnvalue)))
            (bind _asbpw_oddball_count_down (cast `/Game/Blueprints/GUI/Widgets/VersusInGame/BPW_OddballCountDown` (`WidgetComponent.GetUserWidgetObject` (`self.Widget`))))
            (`/Game/Blueprints/GUI/Widgets/VersusInGame/BPW_OddballCountDown.Set Count` _asbpw_oddball_count_down (`KismetArrayLibrary.Array_Get` (`self.Carry Scores`) (`/Game/Blueprints/Character/BP_MainCharacter.Player Index` _output_get)))
            (`SceneComponent.SetVisibility` (`self.Widget`) true false)))))))

(event `Drop Objective_Event_0`
  (`SceneComponent.SetVisibility` (`self.Widget`) false false)
  (set `self.Current Holder` null)
  (`KismetSystemLibrary.K2_PauseTimerHandle` (`self.Score Timer Handle`)))

(fn `ScoreTimer`
  (bind _carry_scores (`self.Carry Scores`))
  (bind _current_holder (`self.Current Holder`)
    (:`then`
      (bind _player_index (`/Game/Blueprints/Character/BP_MainCharacter.Player Index` _current_holder))
      (bind _item (`KismetArrayLibrary.Array_Get` _carry_scores _player_index))
      (`KismetArrayLibrary.Array_Set` _carry_scores _player_index (+ _item 1))
      (if (>= _item 10)
        (bind _asmain_player_controller (cast `/Game/Blueprints/GameModes/MainPlayerController` (`Pawn.GetController` _current_holder)))
        (`self.Winner Determined` _asmain_player_controller)
        (`KismetSystemLibrary.K2_PauseTimerHandle` (`self.Score Timer Handle`))
        (else
          (bind _asbpw_oddball_count_down (cast `/Game/Blueprints/GUI/Widgets/VersusInGame/BPW_OddballCountDown` (`WidgetComponent.GetUserWidgetObject` (`self.Widget`))))
          (`/Game/Blueprints/GUI/Widgets/VersusInGame/BPW_OddballCountDown.Set Count` _asbpw_oddball_count_down _item)
          (`KismetSystemLibrary.PrintString` (`KismetStringLibrary.Concat_StrStr` "Adding to a player " (`KismetStringLibrary.Conv_IntToString` _player_index) "'s score. Current Score: " (`KismetStringLibrary.Conv_IntToString` _item)) true true (struct :`R` 1.0 :`G` 0.788235 :`A` 1.0) 6.0))))
    (:`else`)))

(fn `UserConstructionScript`)