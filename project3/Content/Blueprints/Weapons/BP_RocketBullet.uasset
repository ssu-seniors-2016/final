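; Rocket projectile that homes in on the first non-instigator main character entering its Box1 trigger, targeting their GrappleOrigin.
; It explodes once on hit, confirmed hit or destruction, using a Gate and DoOnce to prevent repeats.
; The explosion hides the rocket, spawns an emitter, applies radial falloff damage and launches nearby characters away, also pushing the hips of ragdolled meshes.
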(event `OnDestroyed_Event_0`
  (bind _returnvalue (`self.K2_GetActorLocation`))
  (bind _box (`self.Box`))
  (`/Engine/EditorBlueprintResources/StandardMacros.Gate` false :!label _label
    (:`Exit`
      (`/Engine/EditorBlueprintResources/StandardMacros.DoOnce` false :!label _label_2
        (:`Completed`
          (`SceneComponent.SetVisibility` _box false true)
          (`PrimitiveComponent.SetCollisionEnabled` _box "NoCollision")
          (`PrimitiveComponent.SetCollisionEnabled` (`self.Box1`) "NoCollision")
          (`GameplayStatics.SpawnEmitterAtLocation` "/Game/Particles/Emitters/P_Explosion_A.P_Explosion_A" _returnvalue)
          (`GameplayStatics.ApplyRadialDamageWithFalloff` :`BaseDamage` (`self.Splash Damage`) :`MinimumDamage` 60.0 :`Origin` _returnvalue :`DamageInnerRadius` 90.0 :`DamageOuterRadius` 160.0 :`DamageFalloff` 2.0 :`DamageTypeClass` "/Game/Blueprints/Character/BP_DamageTypeBasic.BP_DamageTypeBasic_C" :`DamageCauser` self :`InstigatedByController` (`self.GetInstigatorController`))
          (bind _outactors (`KismetSystemLibrary.SphereOverlapActors_NEW` _returnvalue 300.0 (`|MakeArray` "ObjectTypeQuery3" "ObjectTypeQuery4" :!type "EObjectTypeQuery Enum") "/Script/Engine.Character"))
          (for _array_element _outactors
            (bind _ascharacter (cast `Character` _array_element))
            (bind _mesh (`Character.Mesh` _ascharacter))
            (bind _returnvalue_2 (`KismetMathLibrary.GetDirectionVector` (`self.K2_GetActorLocation`) (`SceneComponent.K2_GetComponentLocation` _mesh)))
            (`CharacterMovementComponent.AddImpulse` (`Character.CharacterMovement` _ascharacter) (* _returnvalue_2 6600.0) true)
            (if (`SceneComponent.IsSimulatingPhysics` _mesh "Hips")
              (`PrimitiveComponent.AddImpulse` _mesh (* _returnvalue_2 15000.0) "Hips" true))))))))

(event `self.ReceiveBeginPlay`
  (`parent.ReceiveBeginPlay`)
  (add `self.OnDestroyed` (delegate `OnDestroyed_Event_0`))
  (add `self.Confirm Hit` (delegate `Confirm Hit_Event_0`)))

(event `Confirm Hit_Event_0`
  (`|ExecutionSequence`
    (:`then_0`
      (goto _label :!via `Close`))
    (:`then_1`
      (goto _label_2))
    (:`then_2`
      (`KismetSystemLibrary.Delay` 1.0)
      (`self.K2_DestroyActor`))))

(event `self.ReceiveHit`
  (params (MyComp :type "PrimitiveComponent Object Reference") (Other :type "Actor Object Reference") (OtherComp :type "PrimitiveComponent Object Reference") (bSelfMoved :type Boolean) (HitLocation :type "Vector Structure") (HitNormal :type "Vector Structure") (NormalImpulse :type "Vector Structure") (Hit :type "HitResult Structure (by ref)"))
  (`|ExecutionSequence`
    (:`then_0`
      (goto _label :!via `Close`))
    (:`then_1`
      (goto _label_2))
    (:`then_2`
      (`AudioComponent.Stop` (`self.ExhaustNoise`))
      (`parent.ReceiveHit` MyComp Other OtherComp bSelfMoved HitLocation HitNormal NormalImpulse Hit))))

(event `self.Box1.OnComponentBeginOverlap`
  (params (OtherActor :type "Actor Object Reference") (OtherComp :type "PrimitiveComponent Object Reference") (OtherBodyIndex :type Integer) (bFromSweep :type Boolean) (SweepResult :type "HitResult Structure (by ref)"))
  (`/Engine/EditorBlueprintResources/StandardMacros.DoOnce` false :!label _label_3
    (:`Completed`
      (bind _asbp_main_character (cast `/Game/Blueprints/Character/BP_MainCharacter` OtherActor)
        (:`then`
          (if (!= _asbp_main_character (`self.GetInstigator`))
            (set `ProjectileMovementComponent.HomingTargetComponent` (`/Game/Blueprints/Character/BP_MainCharacter.GrappleOrigin` _asbp_main_character) (`self.ProjectileMovement`))))
        (:`CastFailed`
          (goto _label_3 :!via `Reset`))))))

(fn `UserConstructionScript`
  (`parent.UserConstructionScript`))