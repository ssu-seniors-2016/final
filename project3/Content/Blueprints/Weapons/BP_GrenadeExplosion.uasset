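; BP_GrenadeExplosion is a grenade blast actor that plays its explosion sound and deals radial shock damage as soon as it begins play.
; Both damage and radius are multiplied by the actor's relative X scale, so scaling the actor scales the blast.
; Damage is applied at full strength across the radius, with no falloff, and is credited to the Instigator's controller.
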(event `self.ReceiveBeginPlay`
  (bind _x (.x (`self.GetActorRelativeScale3D`)))
  (`AudioComponent.Play` (`self.Explosion_Audio`) 0.0)
  (`GameplayStatics.ApplyRadialDamage` :`BaseDamage` (* _x (`self.Blast Damage`)) :`Origin` (`self.K2_GetActorLocation`) :`DamageRadius` (* (`self.Blast Radius`) _x) :`DamageTypeClass` "/Game/Blueprints/Character/BP_ShockDamage.BP_ShockDamage_C" :`DamageCauser` self :`InstigatedByController` (`Pawn.GetController` (`self.Instigator`)) :`bDoFullDamage` true))

(fn `UserConstructionScript`)