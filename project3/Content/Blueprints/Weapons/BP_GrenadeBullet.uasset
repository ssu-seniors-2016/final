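; Grenade projectile that bounces, sticks to characters and spawns BP_GrenadeExplosion when destroyed, launched faster with higher ChargePercent.
; Its second bounce removes movement and starts a fuse, while hitting a character attaches it to the mesh on a shorter fuse, ignoring the instigator while still moving.
; A gate cancels the bounce fuse once stuck.
; An unused Detonate event splits it into four smaller grenades, gating off its own explosion.
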(event `self.ReceiveHit`
  (params (MyComp :type "PrimitiveComponent Object Reference") (Other :type "Actor Object Reference") (OtherComp :type "PrimitiveComponent Object Reference") (bSelfMoved :type Boolean) (HitLocation :type "Vector Structure") (HitNormal :type "Vector Structure") (NormalImpulse :type "Vector Structure") (Hit :type "HitResult Structure (by ref)"))
  (bind _projectilemovement (`self.ProjectileMovement`))
  (bind _asbp_main_character (cast `/Game/Blueprints/Character/BP_MainCharacter` Other))
  (`/Engine/EditorBlueprintResources/StandardMacros.IsValid` (`self.ProjectileMovement`)
    (:`Is Valid`
      (if (not (== _asbp_main_character (`self.GetInstigator`)))
        (`self.K2_AttachRootComponentTo` (`Character.Mesh` _asbp_main_character) "None" "KeepWorldPosition" :!label _label)
        (`|ExecutionSequence` :!label _label_2
          (:`then_0`
            (goto _label_4 :!via `Close`))
          (:`then_1`
            (`PrimitiveComponent.SetCollisionEnabled` (`self.Box`) "NoCollision")
            (`self.K2_SetActorRelativeLocation` (`KismetMathLibrary.MakeVector` 0.0 0.0 (.z (.location (`SceneComponent.GetRelativeTransform` (`self.Box`))))))
            (`/Engine/EditorBlueprintResources/StandardMacros.IsValid` _projectilemovement
              (:`Is Valid`
                (`ActorComponent.K2_DestroyComponent` _projectilemovement))
              (:`Is Not Valid`
                _))
            (`KismetSystemLibrary.Delay` 1.4)
            (`self.K2_DestroyActor`)))))
    (:`Is Not Valid`
      (goto _label))))

(event `self.ReceiveBeginPlay`
  (`parent.ReceiveBeginPlay`)
  (add `self.OnDestroyed` (delegate `OnDestroyed_Event_0`))
  (add `self.Confirm Hit` (delegate `Confirm Hit_Event_0`))
  (add `ProjectileMovementComponent.OnProjectileBounce` (`self.ProjectileMovement`) (delegate `OnProjectileBounce_Event_0`)))

(event `OnProjectileBounce_Event_0`
  (params (ImpactResult :type "HitResult Structure (by ref)") (ImpactVelocity :type "Vector Structure (by ref)"))
  (bind _projectilemovement (`self.ProjectileMovement`))
  (bind _asbp_main_character (cast `/Game/Blueprints/Character/BP_MainCharacter` (`.HitActor` (`GameplayStatics.BreakHitResult` ImpactResult)))
    (:`then`
      (`/Engine/EditorBlueprintResources/StandardMacros.IsValid` (`self.ProjectileMovement`)
        (:`Is Valid`
          (if (== _asbp_main_character (`self.GetInstigator`))
            _
            (else
              (`self.K2_AttachRootComponentTo` (`Character.Mesh` _asbp_main_character) "None" "KeepWorldPosition" :!label _label_3)
              (goto _label_2))))
        (:`Is Not Valid`
          (goto _label_3))))
    (:`CastFailed`
      _))
  (bind _result (`/Engine/EditorBlueprintResources/StandardMacros.IncrementInt` (`self.Bounces`))
    (:`  `
      (if (>= _result 2)
        (`/Engine/EditorBlueprintResources/StandardMacros.IsValid` _projectilemovement
          (:`Is Valid`
            (`ActorComponent.K2_DestroyComponent` _projectilemovement)
            (`KismetSystemLibrary.Delay` 3.0)
            (`/Engine/EditorBlueprintResources/StandardMacros.Gate` false :!label _label_4
              (:`Exit`
                (`self.K2_DestroyActor`)))))))))

(event `Confirm Hit_Event_0`)

(event `OnDestroyed_Event_0`
  (`/Engine/EditorBlueprintResources/StandardMacros.Gate` false :!label _label_5
    (:`Exit`
      (`PrimitiveComponent.SetCollisionEnabled` (`self.Box`) "NoCollision")
      (`ActorComponent.K2_DestroyComponent` (`self.ParticleSystem`))
      (`|SpawnActorFromClass` "/Game/Blueprints/Weapons/BP_GrenadeExplosion.BP_GrenadeExplosion_C" (`KismetMathLibrary.MakeTransform` (`self.K2_GetActorLocation`) (struct) (* (`self.GetActorRelativeScale3D`) 2.0)) "Undefined" "OverrideRootScale" (`self.GetInstigatorController`) (`self.GetInstigator`)))))

(event `Detonate`
  (bind _returnvalue (`self.K2_GetActorLocation`))
  (bind _returnvalue_2 (* (0.0 1.0 0.0) -10.0))
  (bind _returnvalue_3 (* (0.0 1.0 0.0) 10.0))
  (bind _returnvalue_4 (* (0.0 0.0 1.0) 10.0))
  (bind _returnvalue_5 (* (0.0 0.0 1.0) -10.0))
  ;[1 1 1] detonate (unused)
  (`/Engine/EditorBlueprintResources/StandardMacros.DoOnce` false
    (:`Completed`
      (`|ExecutionSequence`
        (:`then_0`
          (goto _label_5 :!via `Close`))
        (:`then_1`
          (for _index (range 4)
            (`|SpawnActorFromClass` "BP_GrenadeBullet_C" (`KismetMathLibrary.MakeTransform` _returnvalue (select `int` _index :`0` (`KismetMathLibrary.FindLookAtRotation` _returnvalue (+ _returnvalue_4 _returnvalue)) :`1` (`KismetMathLibrary.FindLookAtRotation` _returnvalue (+ _returnvalue_5 _returnvalue)) :`2` (`KismetMathLibrary.FindLookAtRotation` _returnvalue (+ _returnvalue_3 _returnvalue)) :`3` (`KismetMathLibrary.FindLookAtRotation` _returnvalue (+ _returnvalue_2 _returnvalue)) :`4` (`KismetMathLibrary.FindLookAtRotation` _returnvalue (+ _returnvalue_4 _returnvalue_3 _returnvalue)) :`5` (`KismetMathLibrary.FindLookAtRotation` _returnvalue (+ _returnvalue_5 _returnvalue_3 _returnvalue)) :`6` (`KismetMathLibrary.FindLookAtRotation` _returnvalue (+ _returnvalue_4 _returnvalue_2 _returnvalue)) :`7` (`KismetMathLibrary.FindLookAtRotation` _returnvalue (+ _returnvalue_5 _returnvalue_2 _returnvalue))) (0.5 0.5 0.5)) "Undefined" "OverrideRootScale" (`self.GetInstigatorController`) 1 0.0 (`self.GetInstigator`)))
          (`self.K2_DestroyActor`))))))

(fn `UserConstructionScript`
  (bind _projectilemovement (`self.ProjectileMovement`))
  (`parent.UserConstructionScript`)
  (set `ProjectileMovementComponent.InitialSpeed` (+ (`ProjectileMovementComponent.InitialSpeed` _projectilemovement) (* (`self.Charge Percent`) 1400.0)) _projectilemovement))