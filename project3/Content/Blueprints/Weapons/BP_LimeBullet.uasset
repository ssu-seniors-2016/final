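; Charged lime projectile that scales its look, size and damage with ChargePercent, built on a parent bullet class.
; On BeginPlay, InitCharge swaps the trail particle by charge tier, grows the actor and sets damage as a fraction of MaxDamage.
; Hit and the bound ConfirmHit event share one path that spawns a damage-tiered impact effect, with an upward variant for strong floor or ceiling hits, then calls the parent Hit.
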(event `self.ReceiveBeginPlay`
  (`self.InitCharge` (`self.Charge Percent`))
  (`parent.ReceiveBeginPlay`)
  (add `self.Confirm Hit` (delegate `Confirm Hit_Event_0`)))

(event `Confirm Hit_Event_0`
  (bind _returnvalue (/ (`self.Damage Value`) (`self.Max Damage`)))
  (`GameplayStatics.SpawnEmitterAtLocation` (select `bool` (>= _returnvalue 0.9) :`false` (select `bool` (< _returnvalue 0.3) :`false` "/Game/Particles/Emitters/P_Lime_Hit_2.P_Lime_Hit_2" :`true` "/Game/Particles/Emitters/P_Lime_Hit.P_Lime_Hit" :!type "ParticleSystem Object Reference") :`true` (select `bool` (>= (`KismetMathLibrary.Abs` (.z (stale `self.ReceiveHit` HitNormal))) 0.9) :`false` "/Game/Particles/Emitters/P_Lime_Hit_3.P_Lime_Hit_3" :`true` "/Game/Particles/Emitters/P_Lime_Hit_3_Up.P_Lime_Hit_3_Up" :!type "ParticleSystem Object Reference")) (`self.K2_GetActorLocation`) (struct) :!label _label)
  (`parent.ReceiveHit` (stale `self.ReceiveHit` MyComp) (stale `self.ReceiveHit` Other) (stale `self.ReceiveHit` OtherComp) (stale `self.ReceiveHit` bSelfMoved) (stale `self.ReceiveHit` HitLocation) (stale `self.ReceiveHit` HitNormal) (stale `self.ReceiveHit` NormalImpulse) (stale `self.ReceiveHit` Hit)))

(event `self.ReceiveHit`
  (params (MyComp :type "PrimitiveComponent Object Reference") (Other :type "Actor Object Reference") (OtherComp :type "PrimitiveComponent Object Reference") (bSelfMoved :type Boolean) (HitLocation :type "Vector Structure") (HitNormal :type "Vector Structure") (NormalImpulse :type "Vector Structure") (Hit :type "HitResult Structure (by ref)"))
  (goto _label))

(fn `InitCharge`
  (params (`Charge Value` :type "Float (double-precision)"))
  (bind _particlesystem (`self.ParticleSystem`))
  (bind _returnvalue (+ (* `Charge Value` 2.0) 1.0))
  (`|ExecutionSequence`
    (:`then_0`
      (if (and (> `Charge Value` 0.29) (< `Charge Value` 1.0))
        (`ParticleSystemComponent.SetTemplate` _particlesystem "/Game/Particles/Emitters/P_Lime_2.P_Lime_2")
        (elif (>= `Charge Value` 1.0)
          (`ParticleSystemComponent.SetTemplate` _particlesystem "/Game/Particles/Emitters/P_Lime_3.P_Lime_3"))))
    (:`then_1`
      (`self.SetActorScale3D` (`KismetMathLibrary.MakeVector` _returnvalue _returnvalue _returnvalue))
      (set `self.Damage Value` (* (`self.Max Damage`) `Charge Value`)))))

(fn `Reflectable`
  (returns (canBe :type Boolean))
  (bind _canbe (`parent.Reflectable`))
  (return _canbe))

(fn `UserConstructionScript`
  (`parent.UserConstructionScript`))