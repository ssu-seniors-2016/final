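; Sonic blaster weapon effect that pushes back and damages characters caught inside an expanding cone.
; A looping timer grows the cone mesh from zero while easing its position and audio volume, stopping at full size.
; Cone overlaps maintain a target list, excluding the instigator.
; Each tick damages targets and applies outward impulses that weaken with distance, with a stronger hips impulse for ragdolled meshes.
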(event OnComponentBeginOverlap(SM_LightCone)
  (params (OtherActor :type Actor%20Object%20Reference) (OtherComp :type Primitive%20Component%20Object%20Reference) (OtherBodyIndex :type Integer) (bFromSweep :type Boolean) (SweepResult :type Hit%20Result%20Structure%20%28by%20ref%29))
  (if (!= OtherActor (Game|GetInstigator))
    (bind _ascharacter (Utilities|Casting|CastToCharacter OtherActor))
    (Utilities|Array|AddUnique (Variables|Default|GetPushback%20Targets) _ascharacter)))

(event OnComponentEndOverlap(SM_LightCone)
  (params (OtherActor :type Actor%20Object%20Reference) (OtherComp :type Primitive%20Component%20Object%20Reference) (OtherBodyIndex :type Integer))
  (bind _ascharacter (Utilities|Casting|CastToCharacter OtherActor))
  (Utilities|Array|RemoveItem (Variables|Default|GetPushback%20Targets) _ascharacter))

(event EventTick
  (params (DeltaSeconds :type Float%20%28single-precision%29))
  (bind _box (Variables|Default|GetBox))
  (bind _returnvalue (Transformation|GetWorldLocation _box))
  (for _array_element (Variables|Default|GetPushback%20Targets)
    (Physics|AddImpulse (Variables|/Script/Engine.Character|GetCharacterMovement _array_element) (* (Class|KismetMathLibrary|GetDirectionVector _returnvalue (Transformation|GetWorldLocation (Variables|/Script/Engine.Character|GetMesh _array_element))) (- (Variables|Default|GetPush%20Power) (Math|Vector|VectorLength (- _returnvalue (Transformation|GetWorldLocation (Variables|/Script/Engine.Character|GetMesh _array_element)))))) true)
    (Game|Damage|ApplyDamage _array_element (Variables|Default|GetDamage%20Value) (Game|GetInstigatorController) self "/Game/Blueprints/Character/BP_DamageTypeBasic.BP_DamageTypeBasic_C")
    (if (Physics|IsSimulatingPhysics (Variables|/Script/Engine.Character|GetMesh _array_element) "None")
      (Physics|AddImpulse (Variables|/Script/Engine.Character|GetMesh _array_element) (* (* (Class|KismetMathLibrary|GetDirectionVector _returnvalue (Transformation|GetWorldLocation (Variables|/Script/Engine.Character|GetMesh _array_element))) (- (Variables|Default|GetPush%20Power) (Math|Vector|VectorLength (- _returnvalue (Transformation|GetWorldLocation (Variables|/Script/Engine.Character|GetMesh _array_element)))))) 5.0) "Hips" true))))

(event EventBeginPlay
  (Utilities|Time|SetTimerbyFunctionName 0 "Scale Cone" 0.1 true)
  (Transformation|SetRelativeScale3D (Variables|Default|GetSM_LightCone) "0, 0, 0"))

(fn ConstructionScript
  (|CallParentFunction))

(fn ScaleCone
  (bind _audio (Variables|Default|GetAudio))
  (bind _sm_lightcone (Variables|Default|GetSM_LightCone))
  (bind _relativescale3d (Variables|/Script/Engine.SceneComponent|GetRelativeScale3D _sm_lightcone))
  (Transformation|SetRelativeScale3D _sm_lightcone (Math|Interpolation|VInterptoConstant _relativescale3d "1.430000,1.000000,0.460000" 0.1 3.0))
  (Transformation|SetRelativeLocation _sm_lightcone (Math|Interpolation|VInterptoConstant (Variables|/Script/Engine.SceneComponent|GetRelativeLocation _sm_lightcone) "0.000000,0.000000,0.000000" 0.1 8e+01) false false)
  (Audio|Components|Audio|SetVolumeMultiplier _audio (Math|Interpolation|FInterptoConstant (Variables|/Script/Engine.AudioComponent|GetVolumeMultiplier _audio) 0.05 0.1 0.05) :!class /Script/Engine.AudioComponent)
  (if (Math|Vector|Equal(Vector) _relativescale3d (LocalVariables|GetMax%20Size) 0.005)
    (Utilities|Time|SetTimerbyFunctionName 0 "Scale Cone" 0.0)))