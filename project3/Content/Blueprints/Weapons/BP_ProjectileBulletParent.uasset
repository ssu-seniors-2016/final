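; Base bullet projectile Blueprint, named as the parent for bullet variants, that can be reflected back by other actors.
; On hit it plays an impact sound; non-bouncing bullets then destroy themselves, applying damage here only to Shield actors.
; It reports itself as reflectable, and reflection reassigns Instigator to the new owning Pawn, so later damage is credited to the reflector.
; The ConfirmHit binding is empty and the shoot sound is unwired.
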(event `self.ReceiveBeginPlay`
  (add `self.Confirm Hit` (delegate `Confirm Hit_Event_0`)))

(event `Confirm Hit_Event_0`)

(event `self.ReceiveHit`
  (params (MyComp :type "PrimitiveComponent Object Reference") (Other :type "Actor Object Reference") (OtherComp :type "PrimitiveComponent Object Reference") (bSelfMoved :type Boolean) (HitLocation :type "Vector Structure") (HitNormal :type "Vector Structure") (NormalImpulse :type "Vector Structure") (Hit :type "HitResult Structure (by ref)"))
  (bind _instigator (`self.Instigator`))
  (`GameplayStatics.PlaySoundAtLocation` (`AudioComponent.Sound` (`self.HitNoise`)) HitLocation)
  (if (not (`ProjectileMovementComponent.bShouldBounce` (`self.ProjectileMovement`)))
    (bind _asshield (cast `/Game/Blueprints/Shield` (`.HitActor` (`GameplayStatics.BreakHitResult` Hit)))
      (:`then`
        (`GameplayStatics.ApplyDamage` _asshield (`self.Damage Value`) (`Pawn.GetController` _instigator) _instigator (`self.Damage Type`)))
      (:`CastFailed`
        _))
    (`self.K2_DestroyActor`)))

(fn `Reflectable`
  (returns (canBe :type Boolean))
  (return true))

(fn `reflected`
  (params (`New Owner` :type "Actor Object Reference"))
  (bind _aspawn (cast `Pawn` `New Owner`))
  (set `self.Instigator` _aspawn))

(fn `UserConstructionScript`)