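; Player-fired area bullet that damages every enemy along a forward trace, plus other players with FriendlyFire enabled.
; DoRayCast and DoSphereCast run multi-object line or sphere traces over RayCastLength, store impact points and apply damage credited to the instigator's controller.
; Both only print a warning for non-player instigators, and DoSphereColliderCheck is an unimplemented stub.
; The event graph is empty, so nothing here calls these functions.
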(event `self.ReceiveBeginPlay`)

(event `self.ReceiveActorBeginOverlap`
  (params (OtherActor :type "Actor Object Reference")))

(event `self.ReceiveTick`
  (params (DeltaSeconds :type "Float (single-precision)")))

(fn `DoRayCast`
  (bind _returnvalue (`self.GetInstigator`))
  (bind _returnvalue_2 (`self.GetInstigator`))
  (bind _returnvalue_3 (`self.K2_GetActorLocation`))
  (bind _returnvalue_4 (`self.GetInstigatorController` _returnvalue_2))
  (bind _output_get (set `self.RayCastEndVector` (+ _returnvalue_3 (* (`self.GetActorForwardVector`) (`self.RayCastLength`)))))
  (bind _asbp_main_character (cast `/Game/Blueprints/Character/BP_MainCharacter` _returnvalue)
    (:`then`
      (`KismetSystemLibrary.LineTraceMultiForObjects` _returnvalue_3 _output_get (`|MakeArray` "ObjectTypeQuery1" "ObjectTypeQuery2" "ObjectTypeQuery3" "ObjectTypeQuery4" "ObjectTypeQuery5" :!type "EObjectTypeQuery Enum") true (`|MakeArray` (`self.Instigator`) :!type "Actor Object Reference") "Persistent")
      (for _array_element _
        (bind (_bblockinghit _binitialoverlap _time _location _impactpoint _normal _impactnormal _physmat _hitactor) (`GameplayStatics.BreakHitResult` _array_element))
        (`KismetArrayLibrary.Array_Add` (`self.ImpactPoints`) _impactpoint)
        (bind _asbp_enemy (cast `/Game/Blueprints/Character/BP_Enemy` _hitactor)
          (:`then`
            (`GameplayStatics.ApplyDamage` _asbp_enemy (`self.Damage Value`) (`self.GetInstigatorController` _returnvalue) self "/Game/Blueprints/Character/BP_ContactDamage.BP_ContactDamage_C"))
          (:`CastFailed`
            (bind _asbp_main_character_2 (cast `/Game/Blueprints/Character/BP_MainCharacter` _hitactor))
            (if (and (`/Game/Blueprints/Character/BP_MainCharacter.Friendly Fire` _asbp_main_character_2) (not (== _asbp_main_character_2 _returnvalue_2)))
              (`/Engine/EditorBlueprintResources/StandardMacros.IsValid` _returnvalue_4
                (:`Is Valid`
                  (`GameplayStatics.ApplyDamage` _asbp_main_character_2 (`self.Damage Value`) _returnvalue_4 self (`self.Damage Type`)))
                (:`Is Not Valid`
                  (`KismetSystemLibrary.PrintString` "Instigator controller not valid." false false)))))))
      (return))
    (:`CastFailed`
      (`KismetSystemLibrary.PrintString` "Owner of this bullet was NOT the player... if needed for enemies, logic needs to change in BP_AOEBullet.")
      (return))))

(fn `DoSphereCast`
  (bind _returnvalue (`self.GetInstigator`))
  (bind _returnvalue_2 (`self.GetInstigator`))
  (bind _returnvalue_3 (`self.K2_GetActorLocation`))
  (bind _returnvalue_4 (`self.GetInstigatorController` _returnvalue_2))
  (bind _output_get (set `self.RayCastEndVector` (+ _returnvalue_3 (* (`self.GetActorForwardVector`) (`self.RayCastLength`)))))
  (bind _asbp_main_character (cast `/Game/Blueprints/Character/BP_MainCharacter` _returnvalue)
    (:`then`
      (bind _outhits (`KismetSystemLibrary.SphereTraceMultiForObjects` _returnvalue_3 _output_get 30.0 (`|MakeArray` "ObjectTypeQuery1" "ObjectTypeQuery3" "ObjectTypeQuery4" :!type "EObjectTypeQuery Enum") false (`|MakeArray` (`self.Instigator`) :!type "Actor Object Reference")))
      (for _array_element _outhits
        (bind (_bblockinghit _binitialoverlap _time _location _impactpoint _normal _impactnormal _physmat _hitactor) (`GameplayStatics.BreakHitResult` _array_element))
        (`KismetArrayLibrary.Array_Add` (`self.ImpactPoints`) _impactpoint)
        (bind _asbp_enemy (cast `/Game/Blueprints/Character/BP_Enemy` _hitactor)
          (:`then`
            (`GameplayStatics.ApplyDamage` _asbp_enemy (`self.Damage Value`) (`self.GetInstigatorController` _returnvalue) self "/Game/Blueprints/Character/BP_ContactDamage.BP_ContactDamage_C"))
          (:`CastFailed`
            (bind _asbp_main_character_2 (cast `/Game/Blueprints/Character/BP_MainCharacter` _hitactor))
            (if (and (`/Game/Blueprints/Character/BP_MainCharacter.Friendly Fire` _asbp_main_character_2) (not (== _asbp_main_character_2 _returnvalue_2)))
              (`/Engine/EditorBlueprintResources/StandardMacros.IsValid` _returnvalue_4
                (:`Is Valid`
                  (`GameplayStatics.ApplyDamage` _asbp_main_character_2 (`self.Damage Value`) _returnvalue_4 self (`self.Damage Type`)))
                (:`Is Not Valid`
                  (`KismetSystemLibrary.PrintString` "Instigator controller not valid." false false)))))))
      (return))
    (:`CastFailed`
      (`KismetSystemLibrary.PrintString` "Owner of this bullet was NOT the player... if needed for enemies, logic needs to change in BP_AOEBullet.")
      (return))))

(fn `DoSphereColliderCheck`
  (`KismetSystemLibrary.PrintString` "Sphere collider check not yet implemented.")
  (return))

(fn `UserConstructionScript`
  (`parent.UserConstructionScript`))