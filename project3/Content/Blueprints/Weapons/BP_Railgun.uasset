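; BP_Railgun is a railgun shot actor that fires a beam when almost fully charged on spawn, and otherwise only spawns a small hit effect just ahead of itself.
; A charged shot runs a sphere cast, draws the beam to the cast's end and spawns hit effects at each impact point.
; Tick slides the actor toward that end at constant speed, with the actor set as the beam's source parameter.
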(event `self.ReceiveTick`
  (params (DeltaSeconds :type "Float (single-precision)"))
  (`self.K2_SetActorLocation` (`KismetMathLibrary.VInterpTo_Constant` (`self.K2_GetActorLocation`) (`self.RayCastEndVector`) DeltaSeconds 2000.0)))

(event `self.ReceiveBeginPlay`
  (bind _impactpoints (`self.ImpactPoints`))
  (`parent.ReceiveBeginPlay`)
  (`ParticleSystemComponent.SetActorParameter` (`self.BeamParticle`) "Source" self)
  (if (>= (`self.Charge Percent`) 0.98)
    (`self.DoSphereCast`)
    (`ActorComponent.Activate` (`self.BeamParticle`) false)
    (`ParticleSystemComponent.SetBeamEndPoint` (`self.BeamParticle`) 0 (`self.RayCastEndVector`))
    (`self.SetActorTickEnabled` true)
    (for _array_element _impactpoints
      (`GameplayStatics.SpawnEmitterAtLocation` "/Game/Particles/Emitters/P_Laser_Rifle_Hit.P_Laser_Rifle_Hit" _array_element))
    (`KismetArrayLibrary.Array_Clear` _impactpoints)
    (else
      (`GameplayStatics.SpawnEmitterAtLocation` "/Game/Particles/Emitters/P_Laser_Rifle_Hit.P_Laser_Rifle_Hit" (+ (`self.K2_GetActorLocation`) (* (`self.GetActorForwardVector`) 30.0))))))

(fn `UserConstructionScript`
  (`parent.UserConstructionScript`))