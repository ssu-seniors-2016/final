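; BP_MagmaBullet is a chargeable magma projectile that leaves a half-scale BP_MagmaRemnant on hit or confirmed hit, then runs parent hit logic.
; A looping timer grows it toward a size, and sets damage, that both rise as ChargePercent falls.
; At near-maximum ChargePercent, most bullets destroy themselves on BeginPlay through a random roll.
; A capped self-respawn chain is present but unconnected.
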(event `self.ReceiveBeginPlay`
  (`parent.ReceiveBeginPlay`)
  (if (>= (`self.Charge Percent`) 0.98)
    (if (== (`KismetMathLibrary.RandomInteger` 4) 1)
      (`KismetSystemLibrary.K2_SetTimer` null "Scale Up" 0.1 true :!label _label)
      (add `self.Confirm Hit` (delegate `Confirm Hit_Event_0`))
      (else
        (`self.K2_DestroyActor`)))
    (else
      (goto _label))))

(event `Confirm Hit_Event_0`
  (`|SpawnActorFromClass` "/Game/Blueprints/Weapons/BP_MagmaRemnant.BP_MagmaRemnant_C" (`KismetMathLibrary.MakeTransform` (.location (`self.GetTransform`)) (struct) (/ (.scale (`self.GetTransform`)) 2.0)) "Undefined" "OverrideRootScale" (`self.GetOwner`) (`self.GetInstigator`) :!label _label_2)
  (`parent.ReceiveHit` (stale `self.ReceiveHit` MyComp) (stale `self.ReceiveHit` Other) (stale `self.ReceiveHit` OtherComp) (stale `self.ReceiveHit` bSelfMoved) (stale `self.ReceiveHit` HitLocation) (stale `self.ReceiveHit` HitNormal) (stale `self.ReceiveHit` NormalImpulse) (stale `self.ReceiveHit` Hit)))

(event `self.ReceiveHit`
  (params (MyComp :type "PrimitiveComponent Object Reference") (Other :type "Actor Object Reference") (OtherComp :type "PrimitiveComponent Object Reference") (bSelfMoved :type Boolean) (HitLocation :type "Vector Structure") (HitNormal :type "Vector Structure") (NormalImpulse :type "Vector Structure") (Hit :type "HitResult Structure (by ref)"))
  (goto _label_2))

(fn `Scale Up`
  (bind _returnvalue (- 1.0 (`self.Charge Percent`)))
  (bind _returnvalue_2 (+ (* _returnvalue 4.0) 1.0))
  (`self.SetActorRelativeScale3D` (`KismetMathLibrary.VInterpTo_Constant` (`self.GetActorRelativeScale3D`) (`KismetMathLibrary.MakeVector` _returnvalue_2 _returnvalue_2 _returnvalue_2) 0.1 15.0))
  (set `self.Damage Value` (* (`self.Max Damage`) _returnvalue)))

(fn `UserConstructionScript`
  (`parent.UserConstructionScript`))