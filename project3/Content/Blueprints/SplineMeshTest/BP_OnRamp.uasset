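; Spline-driven on-ramp, in a spline mesh test folder, that builds its geometry in the construction script.
; It divides RampSpline by MeshLength and adds two overlapping spline meshes per segment, enabling collision on the second.
; Segments use world-space positions and normalized tangents with manual attachment.
; An empty every-tenth-segment branch and unconnected static mesh placement and debug print nodes remain, and the event graph is unused.
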(event `self.ReceiveBeginPlay`)

(event `self.ReceiveActorBeginOverlap`
  (params (OtherActor :type "Actor Object Reference")))

(event `self.ReceiveTick`
  (params (DeltaSeconds :type "Float (single-precision)")))

(fn `UserConstructionScript`
  (bind _rampspline (`self.RampSpline`))
  (bind _rampspline_2 (`self.RampSpline`))
  (bind _meshlength (`self.MeshLength`))
  (for _index (range (+ (`KismetMathLibrary.FTrunc` (/ (`SplineComponent.GetDistanceAlongSplineAtSplinePoint` _rampspline (- (`SplineComponent.GetNumberOfSplinePoints` _rampspline) 1)) (`self.MeshLength`))) 1))
    (bind _returnvalue (`AddComponent|Spline Mesh Component_168` :`bManualAttachment` true))
    (bind _returnvalue_2 (`AddComponent|Spline Mesh Component_7709` :`bManualAttachment` true))
    (`PrimitiveComponent.SetCollisionEnabled` _returnvalue_2 "QueryAndPhysics")
    (bind _returnvalue_3 (* _index _meshlength))
    (bind _returnvalue_4 (`SplineComponent.GetLocationAtDistanceAlongSpline` _rampspline_2 _returnvalue_3 "World"))
    (bind _returnvalue_5 (`KismetMathLibrary.Normal` (`SplineComponent.GetTangentAtDistanceAlongSpline` _rampspline_2 _returnvalue_3 "World")))
    (bind _returnvalue_6 (+ _returnvalue_3 _meshlength))
    (bind _returnvalue_7 (`SplineComponent.GetLocationAtDistanceAlongSpline` _rampspline_2 _returnvalue_6 "World"))
    (bind _returnvalue_8 (`KismetMathLibrary.Normal` (`SplineComponent.GetTangentAtDistanceAlongSpline` _rampspline_2 _returnvalue_6 "World")))
    (`SplineMeshComponent.SetStartAndEnd` _returnvalue _returnvalue_4 _returnvalue_5 _returnvalue_7 _returnvalue_8)
    (`SplineMeshComponent.SetStartAndEnd` _returnvalue_2 _returnvalue_4 _returnvalue_5 _returnvalue_7 _returnvalue_8)
    (if (== (mod _index 10) 5)
      _)))