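; Spline-based vine actor that builds its mesh in the construction script along an editable spline component.
; It divides the spline length by Spacing and adds a vine segment spline mesh per interval, with material M_Vine.
; Segment endpoints use world-space spline positions, with tangents from spline direction multiplied by Tangentscale.
; After the loop, a scaled end-cap mesh is placed at the last index's distance, oriented along the spline.
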(event `self.ReceiveBeginPlay`)

(event `self.ReceiveActorBeginOverlap`
  (params (OtherActor :type "Actor Object Reference")))

(event `self.ReceiveTick`
  (params (DeltaSeconds :type "Float (single-precision)")))

(fn `UserConstructionScript`
  (bind _tangentscale (`self.tangentscale`))
  (bind _splinecomonentexample (`self.Splinecomonentexample`))
  (bind _spacing (`self.Spacing`))
  (for _index (range (+ (`.ReturnValue` (`KismetMathLibrary.FMod` (`SplineComponent.GetSplineLength` _splinecomonentexample) _spacing)) 1))
    (bind _returnvalue (`AddComponent|Spline Mesh Component_0` :`bManualAttachment` true :`RelativeTransform` (`self.Vinesize`)))
    (`StaticMeshComponent.SetStaticMesh` _returnvalue "/Game/3D_Assets/Forest/Vine/SM_VineSegment.SM_VineSegment")
    (`PrimitiveComponent.SetMaterial` _returnvalue 0 "/Game/3D_Assets/Forest/Vine/M_Vine.M_Vine")
    (bind _returnvalue_2 (* _index _spacing))
    (bind _returnvalue_3 (`SplineComponent.GetLocationAtDistanceAlongSpline` _splinecomonentexample _returnvalue_2 "World"))
    (bind _returnvalue_4 (* (`SplineComponent.GetDirectionAtDistanceAlongSpline` _splinecomonentexample _returnvalue_2 "World") _tangentscale))
    (bind _returnvalue_5 (+ _returnvalue_2 _spacing))
    (`SplineMeshComponent.SetStartAndEnd` _returnvalue _returnvalue_3 _returnvalue_4 (`SplineComponent.GetLocationAtDistanceAlongSpline` _splinecomonentexample _returnvalue_5 "World") (* (`SplineComponent.GetDirectionAtDistanceAlongSpline` _splinecomonentexample _returnvalue_5 "World") _tangentscale)))
  (bind _returnvalue_6 (`AddComponent|SplineMeshComponent_24764` :`bManualAttachment` true :`RelativeTransform` (`KismetMathLibrary.MakeTransform` _returnvalue_3 (`KismetMathLibrary.Conv_VectorToRotator` _returnvalue_4) (0.25 1.0 1.0))))
  (`StaticMeshComponent.SetStaticMesh` _returnvalue_6 "/Game/3D_Assets/Forest/Vine/SM_VineSegment_End.SM_VineSegment_End"))