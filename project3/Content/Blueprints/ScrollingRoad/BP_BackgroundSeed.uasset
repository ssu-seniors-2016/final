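; BP_BackgroundSeed scatters seeded background instances, named as trees, for the scrolling road.
; The construction script fills two instanced static mesh components with jittered grids, stepping random distances along X and Y and randomizing yaw, roll and scale.
; One random stream is reseeded from Seed and then Seed2, so each layer's layout is repeatable; the event graph has no active logic.
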(event EventBeginPlay)

(event EventActorBeginOverlap
  (params (OtherActor :type Actor%20Object%20Reference)))

(event EventTick
  (params (DeltaSeconds :type Float%20%28single-precision%29)))

(fn ConstructionScript
  (bind _random_stream (Variables|Default|GetRandom%20Stream))
  (bind _random_stream_2 (Variables|Default|GetRandom%20Stream))
  (|CallParentFunction)
  (Math|Random|SetRandomStreamSeed _random_stream_2 (Variables|Default|GetSeed))
  (for _index (range 0 4)
    (bind _output_get (LocalVariables|SetTree%20Instance%20Location (Math|Vector|MakeVector (+ (.X (Math|Vector|BreakVector (LocalVariables|GetTree%20Instance%20Location))) (Math|Random|RandomFloatinRangefromStream 3e+03 5e+03 _random_stream_2)) 0.0 0.0)))
    (for _index_2 (range 0 4)
      (Components|InstancedStaticMesh|AddInstance (Variables|Default|GetInstancedStaticMesh) (Math|Transform|MakeTransform _output_get (Math|Rotator|MakeRotator (Math|Random|RandomFloatinRangefromStream -15.0 15.0 _random_stream_2) 0.0 (Math|Random|RandomFloatinRangefromStream 0.0 3.6e+02 _random_stream_2)) (Math|Vector|MakeVector (Math|Random|RandomFloatinRangefromStream 1.0 2.0 _random_stream_2) (Math|Random|RandomFloatinRangefromStream 1.0 2.0 _random_stream_2) (Math|Random|RandomFloatinRangefromStream 1.0 4.0 _random_stream_2))))
      (LocalVariables|SetTree%20Instance%20Location (+ (LocalVariables|GetTree%20Instance%20Location) (Math|Vector|MakeVector 0.0 (Math|Random|RandomFloatinRangefromStream 3e+03 4e+03 _random_stream_2) 0.0))))
    (LocalVariables|SetTree%20Instance%20Location (Math|Vector|MakeVector (.X (Math|Vector|BreakVector (LocalVariables|GetTree%20Instance%20Location))) 0.0 0.0)))
  (LocalVariables|SetTree%20Instance%20Location "0, 0, 0")
  (Math|Random|SetRandomStreamSeed _random_stream (Variables|Default|GetSeed2))
  (for _index_3 (range 0 4)
    (bind _output_get_2 (LocalVariables|SetTree%20Instance%20Location (Math|Vector|MakeVector (+ (.X (Math|Vector|BreakVector (LocalVariables|GetTree%20Instance%20Location))) (Math|Random|RandomFloatinRangefromStream 2e+03 3e+03 _random_stream)) 0.0 0.0)))
    (for _index_4 (range 0 4)
      (Components|InstancedStaticMesh|AddInstance (Variables|Default|GetInstancedStaticMesh1) (Math|Transform|MakeTransform _output_get_2 (Math|Rotator|MakeRotator (Math|Random|RandomFloatinRangefromStream -15.0 15.0 _random_stream) 0.0 (Math|Random|RandomFloatinRangefromStream 0.0 3.6e+02 _random_stream)) (Math|Vector|MakeVector (Math|Random|RandomFloatinRangefromStream 1.0 2.0 _random_stream) (Math|Random|RandomFloatinRangefromStream 1.0 2.0 _random_stream) (Math|Random|RandomFloatinRangefromStream 1.0 4.0 _random_stream))))
      (LocalVariables|SetTree%20Instance%20Location (Math|Vector|MakeVector (.X (Math|Vector|BreakVector (+ (LocalVariables|GetTree%20Instance%20Location) (Math|Vector|MakeVector 0.0 (Math|Random|RandomFloatinRangefromStream 3e+03 6e+03 _random_stream) 0.0)))) (.Y (Math|Vector|BreakVector (+ (LocalVariables|GetTree%20Instance%20Location) (Math|Vector|MakeVector 0.0 (Math|Random|RandomFloatinRangefromStream 3e+03 6e+03 _random_stream) 0.0)))) 0.0)))
    (LocalVariables|SetTree%20Instance%20Location (Math|Vector|MakeVector (.X (Math|Vector|BreakVector (LocalVariables|GetTree%20Instance%20Location))) 0.0 0.0))))