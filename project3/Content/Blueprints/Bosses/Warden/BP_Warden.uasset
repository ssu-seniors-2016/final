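; Warden boss that fights with a grappling hook in two phases, switched on Tick by Phase, and cannot itself be grappled.
; Phase 0 fires the hook along a sequence of swing nodes, throwing a bomb toward a random player between swings.
; Phase 1 chases a random player, grapples them at mid range after a line-of-sight trace, and damages and knocks them back through PunchBox up close.
; DoOnce nodes pace each action.
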(event `Jump to Center`
  (bind _grapple_positions (`self.Grapple Positions`))
  (`|ExecutionSequence`
    (:`then_0`
      (`/Engine/EditorBlueprintResources/StandardMacros.DoOnce` false
        (:`Completed`
          (`self.Jump`)
          (goto _label :!via `Open`))))
    (:`then_1`
      (`/Engine/EditorBlueprintResources/StandardMacros.Gate` true :!label _label
        (:`Exit`
          (`self.AddMovementInput` (`KismetMathLibrary.Normal` (- (`KismetArrayLibrary.Array_Get` _grapple_positions (- (`KismetArrayLibrary.Array_Length` _grapple_positions) 1)) (`self.K2_GetActorLocation`)))))))))

(event `self.ReceiveBeginPlay`
  (bind _grapplinghook (`self.GrapplingHook`))
  (bind _returnvalue (== (`self.Phase`) 0))
  (`parent.ReceiveBeginPlay`)
  (set `/Game/Blueprints/Character/GrappleHook/GrapplingHook.Tether Length` (`KismetMathLibrary.SelectFloat` 9999.0 650.0 _returnvalue) _grapplinghook)
  (set `/Game/Blueprints/Character/GrappleHook/GrapplingHook.Acceptance Range` (`KismetMathLibrary.SelectFloat` 650.0 100.0 _returnvalue) _grapplinghook)
  (set `/Game/Blueprints/Character/GrappleHook/GrapplingHook.Pull Strength` 600.0 _grapplinghook)
  (bind _outactors (`GameplayStatics.GetAllActorsOfClass` "/Game/Blueprints/Character/BP_MainCharacter.BP_MainCharacter_C"))
  (set `self.Players` _outactors))

(event `Fall and then Swing`
  (bind _current_phase_iterations (`self.Current Phase Iterations`))
  (bind _item (`KismetArrayLibrary.Array_Get` (`self.Grapple Positions`) (`KismetArrayLibrary.Array_Get` (`self.Swing Node Indices`) _current_phase_iterations)))
  ;[1 1 1] Swing phase
  (`KismetSystemLibrary.Delay` 0.25)
  (goto _label_2 :!via `Reset`))

(event `Allow Stop Grapple`
  (bind _returnvalue (`self.K2_GetActorLocation`))
  (bind _players (`self.Players`))
  (bind _returnvalue_2 (`KismetMathLibrary.Normal` (- (`self.K2_GetActorLocation` (`KismetArrayLibrary.Array_Get` _players (`KismetMathLibrary.RandomInteger` (`KismetArrayLibrary.Array_Length` _players)))) _returnvalue)))
  ;[1 1 1] Swing phase
  (goto _label_3 :!via `Reset`))

(event `self.ReceiveTick`
  (params (DeltaSeconds :type "Float (single-precision)"))
  (bind _returnvalue (`self.K2_GetActorLocation`))
  (bind _returnvalue_2 (`self.K2_GetActorLocation`))
  (bind _grapplinghook (`self.GrapplingHook`))
  (bind _players (`self.Players`))
  (bind _attack_target_0 (`self.Attack Target_0`))
  (bind _current_phase_iterations (`self.Current Phase Iterations`))
  (bind _players_2 (`self.Players`))
  (bind _returnvalue_3 (`self.GetDistanceTo` _attack_target_0))
  (bind _returnvalue_4 (`self.K2_GetActorLocation` _attack_target_0))
  (bind _item (`KismetArrayLibrary.Array_Get` (`self.Grapple Positions`) (`KismetArrayLibrary.Array_Get` (`self.Swing Node Indices`) _current_phase_iterations)))
  (bind _returnvalue_5 (`KismetMathLibrary.Normal` (- (`self.K2_GetActorLocation` (`KismetArrayLibrary.Array_Get` _players (`KismetMathLibrary.RandomInteger` (`KismetArrayLibrary.Array_Length` _players)))) _returnvalue)))
  (switch `int` (`self.Phase`)
    (:`0`
      ;[1 1 1] Swing phase
      (`|ExecutionSequence`
        (:`then_0`
          (`/Engine/EditorBlueprintResources/StandardMacros.DoOnce` false :!label _label_2
            (:`Completed`
              (`/Game/Blueprints/Character/GrappleHook/GrapplingHook.Fire` _grapplinghook _item true false)
              (`self.SetActorRotation` (`KismetMathLibrary.MakeRotator` (.roll (`KismetMathLibrary.FindLookAtRotation` (`self.K2_GetActorLocation`) _item)) 0.0 (.yaw (`KismetMathLibrary.FindLookAtRotation` (`self.K2_GetActorLocation`) _item))))
              (set `self.Current Phase Iterations` (`KismetMathLibrary.SelectInt` 0 (+ _current_phase_iterations 1) (> _current_phase_iterations 4))))))
        (:`then_1`
          (if (`/Game/Blueprints/Character/GrappleHook/GrapplingHook.Grapple Attached` _grapplinghook)
            (`/Game/Blueprints/Character/GrappleHook/GrapplingHook.PullTo` _grapplinghook)
            (else
              (`/Engine/EditorBlueprintResources/StandardMacros.DoOnce` true :!label _label_3
                (:`Completed`
                  (`self.Stop Grapple`)
                  (`self.Fall and then Swing`)
                  ;[1 1 1] throw bombs
                  (bind _returnvalue_6 (`|SpawnActorFromClass` "/Game/Blueprints/Bosses/Warden/BP_WardenBomb.BP_WardenBomb_C" (`KismetMathLibrary.MakeTransform` (+ _returnvalue (* _returnvalue_5 300.0)) (struct) (0.25 0.25 0.25)) "Undefined" "OverrideRootScale" null (* _returnvalue_5 1000.0) self))
                  (`PrimitiveComponent.IgnoreActorWhenMoving` (`self.CapsuleComponent`) _returnvalue_6 true))))))
        (:`then_2`
          (goto _label_4 :!via `Reset`))))
    (:`1`
      (`|ExecutionSequence`
        (:`then_0`
          ;[1 1 1] select a player. really kind of useless for single player.
          (`/Engine/EditorBlueprintResources/StandardMacros.DoOnce` false :!label _label_4
            (:`Completed`
              (set `self.Attack Target_0` (`KismetArrayLibrary.Array_Get` _players_2 (`KismetMathLibrary.RandomInteger` (`KismetArrayLibrary.Array_Length` _players_2)))))))
        (:`then_1`
          (`self.SetActorRotation` (`KismetMathLibrary.RInterpTo_Constant` (`self.K2_GetActorRotation`) (`KismetMathLibrary.MakeRotator` 0.0 0.0 (.yaw (`KismetMathLibrary.FindLookAtRotation` _returnvalue_2 _returnvalue_4))) (`GameplayStatics.GetWorldDeltaSeconds`) 800.0)))
        (:`then_2`
          ;[1 1 1] eithrer move toward player, or fire grappling hook at him
          (if (< _returnvalue_3 300.0)
            (set `self.Mob State` "NewEnumerator2")
            (else
              (set `self.Mob State` "NewEnumerator0")
              (if (< _returnvalue_3 600.0)
                (`/Engine/EditorBlueprintResources/StandardMacros.DoOnce` false :!label _label_5
                  (:`Completed`
                    (bind _outhit (`KismetSystemLibrary.LineTraceSingle` :`Start` _returnvalue_2 :`End` _returnvalue_4 :`TraceChannel` "TraceTypeQuery1" :`DrawDebugType` "ForDuration"))
                    (cast `/Game/Blueprints/Character/BP_MainCharacter` (`.HitActor` (`GameplayStatics.BreakHitResult` _outhit))
                      (:`then`
                        (`/Game/Blueprints/Character/GrappleHook/GrapplingHook.Fire` (`self.GrapplingHook`) (`KismetMathLibrary.Normal` (- (`self.K2_GetActorLocation` (`self.Attack Target_0`)) (`self.K2_GetActorLocation`))) false true)
                        (`KismetSystemLibrary.Delay` 1.8)
                        (goto _label_5 :!via `Reset`))
                      (:`CastFailed`
                        _)))))
              (`self.AddMovementInput` (`KismetMathLibrary.Normal` (`KismetMathLibrary.GetDirectionVector` _returnvalue_2 _returnvalue_4)))
              (goto _label_5 :!via `Reset`))))))))

(event `BombHit`
  (`self.Stop Grapple`))

(event `self.PunchBox.OnComponentBeginOverlap`
  (params (OtherActor :type "Actor Object Reference") (OtherComp :type "PrimitiveComponent Object Reference") (OtherBodyIndex :type Integer) (bFromSweep :type Boolean) (SweepResult :type "HitResult Structure (by ref)"))
  ;[1 1 1] deal damage when player is touched by punchbox
  (bind _asbp_main_character (cast `/Game/Blueprints/Character/BP_MainCharacter` OtherActor))
  (if (`|EnumEquality` (`self.Mob State`) "NewEnumerator2")
    (`GameplayStatics.ApplyDamage` _asbp_main_character 100.0 (`self.GetController`) self "/Game/Blueprints/Character/BP_ContactDamage.BP_ContactDamage_C")
    (`CharacterMovementComponent.AddImpulse` (`Character.CharacterMovement` _asbp_main_character) (* (`KismetMathLibrary.Normal` (`KismetMathLibrary.GetDirectionVector` (`self.K2_GetActorLocation`) (`self.K2_GetActorLocation` _asbp_main_character))) 600.0) true)))

(fn `CanBeGrappled`
  (returns (`Yes?` :type Boolean))
  (return false))

(fn `Change Phase`
  (params (`New Phase` :type Integer))
  (switch `int` `New Phase`
    (:`0`
      (set `/Game/Blueprints/Character/GrappleHook/GrapplingHook.Tether Length` 99999.0 (`self.GrapplingHook`)))
    (:`1`
      (set `/Game/Blueprints/Character/GrappleHook/GrapplingHook.Tether Length` 650.0 (`self.GrapplingHook`))
      (set `CharacterMovementComponent.GravityScale` 1.0 (`self.CharacterMovement`)))))

(fn `Stop Grapple`
  (bind _charactermovement (`self.CharacterMovement`))
  (set `CharacterMovementComponent.GravityScale` 1.0 _charactermovement)
  (set `MovementComponent.Velocity` (0.0 0.0 0.0) _charactermovement)
  (return))

(fn `UserConstructionScript`
  (set `self.Health` 1000.0))