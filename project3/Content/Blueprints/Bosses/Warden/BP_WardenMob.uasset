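; Flying mob for the Warden boss that travels to an assigned Destination before the parent class's Tick behavior takes over.
; While traveling, a visibility trace toward the Destination flattens movement to horizontal when blocked and allows direct 3D movement when clear.
; On arrival it sets EndLocation above itself and flags AtLocation.
; When killed, it fires FlyerDestroyed with its MobIndex.
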(event `self.ReceiveBeginPlay`
  (set `self.Patrol Location` (0.0 0.0 280.0))
  (`parent.ReceiveBeginPlay`)
  (set `self.Stop to Attack?` false)
  (add `self.Has Been Killed` (delegate `Has Been Killed_Event_0`))
  (set `self.Start Location` (`self.Destination`)))

(event `Has Been Killed_Event_0`
  (`self.Flyer Destroyed` (`self.Mob Index`)))

(event `self.ReceiveTick`
  (params (DeltaSeconds :type "Float (single-precision)"))
  (bind _returnvalue (`self.K2_GetActorLocation`))
  (bind _destination (`self.Destination`))
  (bind _returnvalue_2 (`KismetMathLibrary.Normal` (- _destination _returnvalue)))
  (if (`self.At Location`)
    (`parent.ReceiveTick` DeltaSeconds)
    (else
      (`|ExecutionSequence`
        (:`then_0`
          (if (== _returnvalue _destination :`ErrorTolerance` 5.0)
            (set `self.End Location` (+ (`self.K2_GetActorLocation`) (0.0 0.0 300.0)))
            (set `self.At Location` true)
            (else
              (bind (_outhit _returnvalue_3) (`KismetSystemLibrary.LineTraceSingle` :`Start` _returnvalue :`End` _destination :`TraceChannel` "TraceTypeQuery1" :`DrawDebugType` "ForOneFrame"))
              (`self.AddMovementInput` (`KismetMathLibrary.SelectVector` (`KismetMathLibrary.MakeVector` (.x _returnvalue_2) (.y _returnvalue_2)) _returnvalue_2 _returnvalue_3)))))))))

(fn `UserConstructionScript`
  (`parent.UserConstructionScript`))