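; BP_Squadron is a versus-map actor that flies three jets in patterns between nine placed points.
; On a timer it randomly picks the Risers, Burner or Sliders pattern, giving each jet two endpoints and a random speed.
; Tick moves jets at constant speed, swapping endpoints on arrival.
; Occasionally speed flips negative as a flag to spin the jet for one leg, with absolute value driving movement.
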(event EventBeginPlay)

(event EventActorBeginOverlap
  (params (OtherActor :type Actor%20Object%20Reference)))

(event EventTick
  (params (DeltaSeconds :type Float%20%28single-precision%29))
  (if (Variables|Default|GetNew_State)
    (CallFunction|GetNewState))
  (CallFunction|Update DeltaSeconds)
  (bind _output_get (Variables|Default|SetState_Timer (- (Variables|Default|GetState_Timer) DeltaSeconds)))
  (if (< _output_get 0.0)
    (Variables|Default|SetNew_State true)))

(fn ConstructionScript
  (Variables|Default|SetJet%20Array (Utilities|Array|MakeArray (Variables|Default|GetJet1) (Variables|Default|GetJet2) (Variables|Default|GetJet3)))
  (Variables|Default|SetPoint%20Array (Utilities|Array|MakeArray (Transformation|GetWorldLocation (Variables|Default|GetPoint1)) (Transformation|GetWorldLocation (Variables|Default|GetPoint2)) (Transformation|GetWorldLocation (Variables|Default|GetPoint3)) (Transformation|GetWorldLocation (Variables|Default|GetPoint4)) (Transformation|GetWorldLocation (Variables|Default|GetPoint5)) (Transformation|GetWorldLocation (Variables|Default|GetPoint6)) (Transformation|GetWorldLocation (Variables|Default|GetPoint7)) (Transformation|GetWorldLocation (Variables|Default|GetPoint8)) (Transformation|GetWorldLocation (Variables|Default|GetPoint9)))))

(fn GetNewState
  (bind _returnvalue (Math|Random|RandomIntegerinRange 0 2))
  (Variables|Default|SetState_Num (Math|Integer|%(Integer) (+ _returnvalue (Math|Conversions|ToInteger(Boolean) (== (Variables|Default|GetState_Num) _returnvalue))) 3))
  (bind _output_get (LocalVariables|SetState (Utilities|Select :Index (Variables|Default|GetState_Num) :Option%200 (Variables|States|GetState_Risers) :Option%201 (Variables|States|GetState_Burner) :Option%202 (Variables|States|GetState_Sliders))))
  (if (!= (Utilities|Array|Length _output_get) 3)
    (Development|PrintString "BP_SQUADRON: Bad State")
    (else
      (for (_array_element _array_index) _output_get
        (Utilities|Array|SetArrayElem (Variables|Default|GetState%20Array) _array_index _array_element)
        (Utilities|Array|SetArrayElem (Variables|Default|GetSpeed%20Array) _array_index (Math|Random|RandomFloatinRange 4e+02 1e+03))
        (Transformation|SetRelativeRotation (Utilities|Array|Get(acopy) (Variables|Default|GetJet%20Array) _array_index) (Math|Vector|RotatorfromAxisandAngle "1.000000,0.000000,0.000000" 9e+01) false false))
      (Variables|Default|SetNew_State false)
      (Variables|Default|SetState_Timer (Variables|Default|GetState_Time)))))

(fn Update
  (params (dT :type Float%20%28single-precision%29))
  (for (_array_element _array_index) (Variables|Default|GetJet%20Array)
    (bind _target (CallFunction|GetJetTarget _array_index))
    (if (< (Math|Vector|VectorLength (- (Transformation|GetWorldLocation _array_element) _target)) (Variables|Default|GetTolerance))
      (CallFunction|SwitchJetTarget _array_index)
      (Transformation|SetRelativeRotation _array_element (Math|Vector|RotatorfromAxisandAngle "1.000000,0.000000,0.000000" 9e+01) false false)
      (else
        (Transformation|SetWorldLocation _array_element (Math|Interpolation|VInterptoConstant (Transformation|GetWorldLocation _array_element) _target dT (Math|Float|Absolute(Float) (Utilities|Array|Get(acopy) (Variables|Default|GetSpeed%20Array) _array_index))) false false)
        (if (< (Utilities|Array|Get(acopy) (Variables|Default|GetSpeed%20Array) _array_index) 0.0)
          (Transformation|AddLocalRotation _array_element (Math|Vector|RotatorfromAxisandAngle "0,0.000000,1.000000" 3.0) false false))))))

(fn GetJetTarget
  (params (Index :type Integer))
  (bind _state_array (Variables|Default|GetState%20Array))
  (bind _point_array (Variables|Default|GetPoint%20Array))
  (bind _item (Utilities|Array|Get(acopy) _state_array Index))
  (bind (_state0 _state1 _state) (Utilities|Struct|BreakJet_State _item))
  (bind _returnvalue (Math|Integer|SelectInt _state1 _state0 _state))
  (if (== _returnvalue 0)
    (LocalVariables|SetTemp_Dest (Utilities|Array|Get(acopy) _point_array (- _state0 1)))
    (else
      (LocalVariables|SetTemp_Dest (Utilities|Array|Get(acopy) _point_array (- _returnvalue 1)))))
  (return (LocalVariables|GetTemp_Dest)))

(fn SwitchJetTarget
  (params (Index :type Integer))
  (bind _speed_array (Variables|Default|GetSpeed%20Array))
  (bind _state_array (Variables|Default|GetState%20Array))
  (bind _item (Utilities|Array|Get(acopy) _state_array Index))
  (bind _item_2 (Utilities|Array|Get(acopy) _speed_array Index))
  (bind (_state0 _state1 _state) (Utilities|Struct|BreakJet_State _item))
  (Utilities|Array|SetArrayElem _state_array Index (Utilities|Struct|MakeJet_State _state0 _state1 (not _state)))
  (if (or (> (Math|Random|RandomFloat) 0.94) (< _item_2 0.0))
    (Utilities|Array|SetArrayElem _speed_array Index (* _item_2 -1.0))))