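; Builder actor that gathers the level's StaticMeshActors and recreates them as instanced static meshes in its Construction Script.
; It collects the unique meshes, adds one InstancedStaticMeshComponent per mesh, then adds a world-space instance at each matching actor's transform, printing instance counts.
; Only the mesh and transform are copied, and the source actors remain because the DestroyActor loops are disconnected.
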(event `self.ReceiveBeginPlay`)

(event `self.ReceiveActorBeginOverlap`
  (params (OtherActor :type "Actor Object Reference")))

(event `self.ReceiveTick`
  (params (DeltaSeconds :type "Float (single-precision)")))

(fn `UserConstructionScript`
  (bind _isms (`self.ISMs`))
  (bind _outactors (`GameplayStatics.GetAllActorsOfClass` "/Script/Engine.StaticMeshActor"))
  (`|ExecutionSequence`
    (:`then_0`
      (bind _output_get (set `self.Meshes` _outactors))
      (for _array_element _output_get
        (`KismetArrayLibrary.Array_AddUnique` (`self.Meshes In Scene`) (`StaticMeshComponent.StaticMesh` (`StaticMeshActor.StaticMeshComponent` _array_element))))
      (for _array_element_2 (`self.Meshes In Scene`)
        (bind _returnvalue (`AddComponent|Instanced Static Mesh Component_0` :`bManualAttachment` true :`RelativeTransform` (`KismetMathLibrary.MakeTransform` (0.0 0.0 0.0))))
        (`KismetArrayLibrary.Array_Add` _isms _returnvalue)
        (`StaticMeshComponent.SetStaticMesh` _returnvalue _array_element_2))
      (for _array_element_3 _output_get
        (for _array_element_4 _isms
          (bind _staticmeshcomponent (`StaticMeshActor.StaticMeshComponent` _array_element_3))
          (if (== (`StaticMeshComponent.StaticMesh` _staticmeshcomponent) (`StaticMeshComponent.StaticMesh` _array_element_4))
            (`KismetSystemLibrary.PrintString` (`KismetStringLibrary.Conv_IntToString` (`InstancedStaticMeshComponent.GetInstanceCount` _array_element_4)))
            (`InstancedStaticMeshComponent.AddInstanceWorldSpace` _array_element_4 (`SceneComponent.K2_GetComponentToWorld` _staticmeshcomponent))))))))