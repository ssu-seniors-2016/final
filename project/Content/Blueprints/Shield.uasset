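; Shield actor for the main character that intercepts overlapping bullets fired by other instigators.
; With the shield upgrade, while the owner's ACShieldComponent is reflecting, reflectable bullets have their velocity reversed and receive the owner as instigator through Reflected.
; Otherwise the bullet is destroyed and drains the component's ShieldTimer, which flags destruction and deactivates the shield at zero.
; Helper functions set the sphere's material or replace it with a destructible component.
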(event `self.ReceiveActorBeginOverlap`
  (params (OtherActor :type "Actor Object Reference"))
  (bind _other_actor (`self.Other Actor`))
  (bind _output_get (set `self.Other Actor` OtherActor))
  (if (== (`GameplayStatics.GetObjectClass` _output_get) "/Game/Blueprints/Bullet.Bullet_C")
    (if (not (== (`self.GetInstigator`) (`self.GetInstigator` (`self.Other Actor`))))
      (bind _asbp_main_character (cast `/Game/Blueprints/Character/BP_MainCharacter` (`self.GetInstigator`)))
      (if (`/Game/Blueprints/Character/BP_MainCharacter.Has Shield Upgrade` _asbp_main_character)
        (bind _ac_shieldcomponent (`/Game/Blueprints/Character/BP_MainCharacter.AC_ShieldComponent` _asbp_main_character))
        (if (`/Game/Blueprints/Character/AC_ShieldComponent.Is Not Reflecting` _ac_shieldcomponent)
          ;[0 1 0.01606] Not Reflecting Branch
          (set `/Game/Blueprints/Character/AC_ShieldComponent.Shield Timer` (- (`/Game/Blueprints/Character/AC_ShieldComponent.Shield Timer` _ac_shieldcomponent) 1.0) _ac_shieldcomponent :!label _label)
          (if (<= (`/Game/Blueprints/Character/AC_ShieldComponent.Shield Timer` _ac_shieldcomponent) 0.0)
            (set `/Game/Blueprints/Character/AC_ShieldComponent.isDestroyed` true _ac_shieldcomponent)
            (`/Game/Blueprints/Character/AC_ShieldComponent.Deactivate_Shield` _ac_shieldcomponent))
          (`self.K2_DestroyActor` (`self.Other Actor`))
          (else
            (bind _canbe (message `/Game/Blueprints/BPI_Bullet_Interface.Reflectable` _other_actor))
            (if _canbe
              ;[1 0 0.7378] Reflecting Branch
              (bind _asbullet (cast `/Game/Blueprints/Bullet` _other_actor))
              (bind _projectilemovement (`/Game/Blueprints/Bullet.ProjectileMovement` _asbullet))
              (set `MovementComponent.Velocity` (`KismetMathLibrary.NegateVector` (`MovementComponent.Velocity` _projectilemovement)) _projectilemovement)
              (`/Game/Blueprints/Bullet.reflected` _asbullet (`self.GetInstigator`))
              (else
                (goto _label)))))
        (else
          (goto _label))))))

(event `self.ReceiveTick`
  (params (DeltaSeconds :type "Float (single-precision)")))

(event `self.ReceiveBeginPlay`)

(fn `Break`
  (`ActorComponent.K2_DestroyComponent` (`self.Sphere`))
  (bind _returnvalue (`AddComponent|Destructible Component_4`))
  (`PrimitiveComponent.SetMaterial` _returnvalue 0 "/Game/Blueprints/ProgrammerArt/Shield_Material.Shield_Material"))

(fn `Set Material`
  (params (Material :type "MaterialInstanceDynamic Object Reference"))
  (`PrimitiveComponent.SetMaterial` (`self.Sphere`) 0 Material))

(fn `UserConstructionScript`)