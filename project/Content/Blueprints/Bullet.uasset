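; Bullet projectile that launches along an initial velocity and destroys itself after three seconds.
; On hit it is destroyed unless its projectile movement allows bouncing.
; It reports itself as reflectable, and reflection makes the new owner the ignored actor in place of the instigator.
; The line trace that reads that ignore list and damages enemies or the player is disconnected, so the bullet applies no damage here.
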(event `self.ReceiveBeginPlay`
  (bind _projectilemovement (`self.ProjectileMovement`))
  ;[0.02878 1 0.01511] Startup code
  (set `MovementComponent.Velocity` (* (`self.Initial Velocity`) (`ProjectileMovementComponent.InitialSpeed` _projectilemovement)) _projectilemovement)
  (set `self.Actors to ignore` (`|MakeArray` (`self.GetInstigator`) :!type "Actor Object Reference"))
  (`KismetSystemLibrary.Delay` 3.0)
  (`self.K2_DestroyActor`))

(event `self.ReceiveTick`
  (params (DeltaSeconds :type "Float (single-precision)")))

(event `self.Box.OnComponentBeginOverlap`
  (params (OtherActor :type "Actor Object Reference") (OtherComp :type "PrimitiveComponent Object Reference") (OtherBodyIndex :type Integer) (bFromSweep :type Boolean) (SweepResult :type "HitResult Structure (by ref)")))

(event `self.ReceiveHit`
  (params (MyComp :type "PrimitiveComponent Object Reference") (Other :type "Actor Object Reference") (OtherComp :type "PrimitiveComponent Object Reference") (bSelfMoved :type Boolean) (HitLocation :type "Vector Structure") (HitNormal :type "Vector Structure") (NormalImpulse :type "Vector Structure") (Hit :type "HitResult Structure (by ref)"))
  (if (not (`ProjectileMovementComponent.bShouldBounce` (`self.ProjectileMovement`)))
    (`self.K2_DestroyActor`)))

(fn `Reflectable`
  (returns (canBe :type Boolean))
  (return true))

(fn `reflected`
  (params (`New Owner` :type "Actor Object Reference"))
  (set `self.Actors to ignore` (`|MakeArray` `New Owner`)))

(fn `UserConstructionScript`)