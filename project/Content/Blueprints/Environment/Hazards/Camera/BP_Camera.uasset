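; Security camera hazard with a spotlight and feed render target that detects and tracks the player, configured in the construction script.
; Each tick, DoMath checks distance and a dot-product view cone, stepping pitch and yaw toward a detected player.
; After losing the player, it seeks random angles with decaying Determination, then settles to a rest pose.
; Interpolated rotations smooth hinge and camera motion, while timelines blend light and beam between search, detected and "sad" colors.
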(event `self.ReceiveTick`
  (params (DeltaSeconds :type "Float (single-precision)"))
  (bind _light_mesh_material (`self.Light Mesh Material`))
  (bind _pitch (`self.Pitch`))
  (bind _yaw (`self.Yaw`))
  (bind _pitch_2 (`self.Pitch`))
  (bind _yaw_2 (`self.Yaw`))
  (bind _spotlight (`self.SpotLight`))
  (`|ExecutionSequence`
    (:`then_0`
      (set `self.Delta Seconds` DeltaSeconds)
      (bind (_pawn _inrange) (`self.Do Math`))
      (`/Engine/EditorBlueprintResources/StandardMacros.IsValid` _pawn
        (:`Is Valid`
          (set `self.Player In Range` _inrange)
          (`SceneComponent.K2_SetWorldRotation` (`self.Camera Mesh`) (`KismetMathLibrary.RInterpTo` (`SceneComponent.K2_GetComponentRotation` (`self.Camera Mesh`)) (`KismetMathLibrary.MakeRotator` (.roll (`SceneComponent.K2_GetComponentRotation` (`self.Camera Mesh`))) _pitch_2 (.yaw (`SceneComponent.K2_GetComponentRotation` (`self.Camera Mesh`)))) (`self.Delta Seconds`) 6.0) false false)
          (`SceneComponent.K2_SetWorldRotation` (`self.Hinge Mesh`) (`KismetMathLibrary.RInterpTo` (`SceneComponent.K2_GetComponentRotation` (`self.Hinge Mesh`)) (`KismetMathLibrary.MakeRotator` (.roll (`SceneComponent.K2_GetComponentRotation` (`self.Hinge Mesh`))) (.pitch (`SceneComponent.K2_GetComponentRotation` (`self.Hinge Mesh`))) _yaw_2) (`self.Delta Seconds`) 4.125) false false)
          (if (`self.Player In Range`)
            (bind (_direction _newtrack_0) (`Timeline|Fade To Detection Color` :!label _label)
              (:`Update`
                (if (`self.decreasing`)
                  (bind (_direction_2 _newtrack_0_2) (`Timeline|Fade To Sad Color` :!via `Reverse` :!label _label_2)
                    (:`Update`
                      (bind _returnvalue (`KismetMathLibrary.LinearColorLerp` (`KismetMathLibrary.LinearColorLerp` (`self.Search Color`) (`self.Detected Color`) _newtrack_0) (`self.Sad Color`) _newtrack_0_2))
                      (`LightComponent.SetLightColor` _spotlight _returnvalue true)
                      (`LightComponent.SetIntensity` _spotlight (`.A` (`KismetMathLibrary.BreakColor` _returnvalue)))
                      (`|ExecutionSequence`
                        (:`then_0`
                          (`/Engine/EditorBlueprintResources/StandardMacros.IsValid` _light_mesh_material
                            (:`Is Valid`
                              (`MaterialInstanceDynamic.SetVectorParameterValue` _light_mesh_material "Color" _returnvalue))))
                        (:`then_1`
                          (`/Engine/EditorBlueprintResources/StandardMacros.IsValid` _light_mesh_material)))))
                  (else
                    (goto _label_2)))))
            (else
              (goto _label :!via `Reverse`))))))
    (:`then_1`
      ;[1 1 1] player is in range
      (if (`self.Player In Range`)
        (set `self.Pitch` (`KismetMathLibrary.SelectFloat` (- _pitch_2 0.5) (+ _pitch_2 0.5) (> _pitch_2 (.pitch (`KismetMathLibrary.FindLookAtRotation` (`SceneComponent.K2_GetComponentLocation` (`self.Camera Mesh`)) (`self.K2_GetActorLocation` (`GameplayStatics.GetPlayerPawn` 0)))))))
        (set `self.Yaw` (`KismetMathLibrary.SelectFloat` (- _yaw_2 0.5) (+ _yaw_2 0.5) (> _yaw_2 (.yaw (`KismetMathLibrary.FindLookAtRotation` (`SceneComponent.K2_GetComponentLocation` (`self.Camera Mesh`)) (`self.K2_GetActorLocation` (`GameplayStatics.GetPlayerPawn` 0)))))))
        (set `self.decreasing` true)
        (set `self.determination` 0.5)
        (else
          (`|ExecutionSequence`
            (:`then_0`
              (if (`self.decreasing`)
                (bind _output_get (set `self.determination` (`KismetMathLibrary.FClamp` (- (`self.determination`) 0.002) 0.001 0.5)))
                (if (<= _output_get 0.001)
                  (set `self.decreasing` false))
                (else
                  (set `self.pitchDest` -35.0)
                  (set `self.yawDest` 0.0)
                  (set `self.determination` 0.05))))
            (:`then_1`
              (if (not (`self.approachingDest`))
                (set `self.pitchDest` (`KismetMathLibrary.RandomFloatInRange` -45.0 45.0))
                (set `self.yawDest` (`KismetMathLibrary.RandomFloatInRange` -45.0 45.0))
                (set `self.approachingDest` true))
              (set `self.Pitch` (+ (* (- (`self.pitchDest`) _pitch) (`self.determination`)) _pitch))
              (set `self.Yaw` (+ (* (- (`self.yawDest`) _yaw) (`self.determination`)) _yaw)))
            (:`then_2`
              (if (and (`self.decreasing`) (and (< (`KismetMathLibrary.Abs` (- (`self.pitchDest`) (`self.Pitch`))) 0.001) (< (`KismetMathLibrary.Abs` (- (`self.yawDest`) (`self.Yaw`))) 0.001)))
                (set `self.approachingDest` false)))))))))

(fn `Do Math`
  (returns (Pawn :type "Pawn Object Reference") (inRange :type Boolean))
  (bind _returnvalue (`GameplayStatics.GetPlayerPawn` 0))
  (return _returnvalue (and (>= (`KismetMathLibrary.Dot_VectorVector` (`KismetMathLibrary.Normal` (- (`self.K2_GetActorLocation` _returnvalue) (`self.K2_GetActorLocation`))) (`SceneComponent.GetForwardVector` (`self.SpotLight`))) 0.8) (<= (`KismetMathLibrary.VSize` (- (`self.K2_GetActorLocation`) (`self.K2_GetActorLocation` _returnvalue))) (`self.Detection Range`)))))

(fn `UserConstructionScript`
  (bind _spotlight (`self.SpotLight`))
  (bind _search_color (`self.Search Color`))
  (`PointLightComponent.SetAttenuationRadius` (`self.SpotLight`) (`self.Detection Range`))
  (set `SceneCaptureComponent2D.TextureTarget` (`self.Feed Texture Target`) (`self.Feed`))
  (bind _output_get (set `self.Pitch` (`KismetMathLibrary.FClamp` (`self.Pitch`) -222.0 42.0)))
  (`SceneComponent.K2_SetRelativeRotation` (`self.Camera Mesh`) (`KismetMathLibrary.MakeRotator` 0.0 _output_get) false false)
  (`SceneComponent.K2_SetWorldRotation` (`self.Hinge Mesh`) (`KismetMathLibrary.MakeRotator` 0.0 0.0 (`self.Yaw`)) false false)
  (if (`self.Turned Off`)
    (`SceneComponent.SetVisibility` (`self.SpotLight`) false false)
    (`SceneComponent.SetVisibility` (`self.Light Beam Mesh`) false false)
    (else
      ;[1 1 1] this empty source is what's causing the errors accessing the parameter
      (bind _returnvalue (`PrimitiveComponent.CreateDynamicMaterialInstance` (`self.Camera Mesh`) 1 null))
      (set `self.Spotlight Lens Material` _returnvalue)
      (`MaterialInstanceDynamic.SetVectorParameterValue` _returnvalue "Color" (`self.Search Color`))
      (`LightComponent.SetLightColor` _spotlight _search_color true)
      (`LightComponent.SetIntensity` _spotlight (`.A` (`KismetMathLibrary.BreakColor` _search_color)))
      (`PointLightComponent.SetAttenuationRadius` _spotlight (`self.Light Radius`))
      (bind _returnvalue_2 (`PrimitiveComponent.CreateDynamicMaterialInstance` (`self.Light Beam Mesh`) 0 null))
      (set `self.Light Mesh Material` _returnvalue_2)
      (`MaterialInstanceDynamic.SetVectorParameterValue` _returnvalue_2 "Color" (`self.Search Color`))
      (`SceneComponent.SetRelativeScale3D` (`self.Light Beam Mesh`) (`KismetMathLibrary.ClampVectorSize` (* (`KismetMathLibrary.MakeVector` 0.005 0.005 0.007) (`self.Light Radius`)) 0.0 20.0)))))