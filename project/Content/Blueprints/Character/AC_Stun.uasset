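; Character component that gives BP_MainCharacter a stun ability on a cooldown.
; ActivateStun enters a DoOnce that calls FireStun and starts the cooldown; Tick counts it down and resets the gate once it expires.
; FireStun spawns a BP_StunField at the owner's StunField component, attaches it to the owner and disables its collision.
; FizzleStun is an empty, unreached stub.
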(event `self.ReceiveBeginPlay`
  (bind _asbp_main_character (cast `/Game/Blueprints/Character/BP_MainCharacter` (`self.GetOwner`))
    (:`then`
      (set `self.Owner` _asbp_main_character))
    (:`CastFailed`
      (`KismetSystemLibrary.PrintString` "ERROR CASTING AC_STUN'S OWNER" true true (struct :`R` 1.0 :`A` 1.0)))))

(event `self.ReceiveTick`
  (params (DeltaSeconds :type "Float (single-precision)"))
  (bind _cooldown (`self.Cooldown`))
  (if (> _cooldown 0.0)
    (set `self.Cooldown` (- _cooldown DeltaSeconds))
    (else
      (goto _label :!via `Reset`))))

(event `Activate Stun`
  (`/Engine/EditorBlueprintResources/StandardMacros.DoOnce` false :!label _label
    (:`Completed`
      (`self.Fire Stun`)
      (set `self.Cooldown` 5.0))))

(fn `Fire Stun`
  (bind _owner (`self.Owner`))
  (bind _returnvalue (`|SpawnActorFromClass` "/Game/Blueprints/Character/BP_StunField.BP_StunField_C" (`KismetMathLibrary.Conv_VectorToTransform` (`SceneComponent.GetSocketLocation` (`/Game/Blueprints/Character/BP_MainCharacter.Stun_field` _owner) "None")) "AlwaysSpawn" "OverrideRootScale" null _owner))
  (`Actor.K2_AttachRootComponentToActor` _returnvalue _owner "None" "SnapToTargetIncludingScale" true)
  (`Actor.SetActorEnableCollision` _returnvalue false))

(fn `Fizzle Stun`)