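; AI guard character, derived from BP_Enemy, that shoots at the enemy actor stored in its Blackboard.
; BeginPlay writes its two target objects to the Blackboard.
; Tick polls EnemyActor, using a DoOnce to start a looping FireRate timer that fires ACGunComponent toward it, and clears the timer when none is set.
; Damage handling defers to the parent, and Shoot only prints a debug string.
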(event `Attack Player`
  (`/Game/Blueprints/Character/AC_GunComponent.Fire Bullet` (`self.AC_GunComponent`) (`KismetMathLibrary.Normal` (- (`self.K2_GetActorLocation` (stale `self.ReceiveTick` _asactor)) (`self.K2_GetActorLocation`)))))

(event `self.ReceiveTick`
  (params (DeltaSeconds :type "Float (single-precision)"))
  ;[1 0.3071 0.2689] Bullets
  (bind _asactor (cast `Actor` (`BlackboardComponent.GetValueAsObject` (`AIBlueprintHelperLibrary.GetBlackboard` self) "EnemyActor")) ; If guard sees player, fire at it
    (:`then`
      (`/Engine/EditorBlueprintResources/StandardMacros.DoOnce` false :!label _label
        (:`Completed`
          (`KismetSystemLibrary.K2_SetTimerDelegate` (delegate `Attack Player`) (`self.Fire Rate`) true))))
    (:`CastFailed`
      (`|ExecutionSequence`
        (:`then_0`
          (goto _label :!via `Reset`))
        (:`then_1`
          (`KismetSystemLibrary.K2_SetTimerDelegate` (delegate `Attack Player`)))))))

(event `self.ReceiveBeginPlay`
  ;[0.6036 1 0.5841] Initialize
  (`BlackboardComponent.SetValueAsObject` (`AIBlueprintHelperLibrary.GetBlackboard` self) "Guard1Target1Key" (`self.Target1`))
  (`BlackboardComponent.SetValueAsObject` (`AIBlueprintHelperLibrary.GetBlackboard` self) "Guard1Target2Key" (`self.Target2`)))

(event `self.ReceiveAnyDamage`
  (params (Damage :type "Float (single-precision)") (DamageType :type "DamageType Object Reference") (InstigatedBy :type "Controller Object Reference") (DamageCauser :type "Actor Object Reference"))
  ;[1 0.009546 0.0382] See AnyDamage event in BP_Enemy parent class
  (`parent.ReceiveAnyDamage` Damage null null null))

(fn `Shoot`
  (`KismetSystemLibrary.PrintString` "Bang! Bang!"))

(fn `UserConstructionScript`)