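; AC_WallJumpVolume is an actor component that turns its owning StaticMeshActor into a wall-jump surface.
; On BeginPlay it casts the owner, binds to its OnActorHit event and sets the owner's tags to just WallJump.
; Each hit sends a StartWallJump message to the other actor with the sign of the hit normal's Y as an integer, giving a left or right direction.
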(event `self.ReceiveTick`
  (params (DeltaSeconds :type "Float (single-precision)")))

(event `self.ReceiveBeginPlay`
  (bind _asstatic_mesh_actor (cast `StaticMeshActor` (`self.GetOwner`)))
  (add `Actor.OnActorHit` _asstatic_mesh_actor (delegate `JumpWallHit`))
  (set `Actor.Tags` (`|MakeArray` "WallJump" :!type "Name") (`self.GetOwner`)))

(event `JumpWallHit`
  (params (SelfActor :type "Actor Object Reference") (OtherActor :type "Actor Object Reference") (NormalImpulse :type "Vector Structure") (Hit :type "HitResult Structure (by ref)"))
  (message `/Game/Blueprints/Character/BPI_WallJump.StartWallJump` OtherActor (`KismetMathLibrary.FTrunc` (`KismetMathLibrary.SignOfFloat` (.y (`.Normal` (`GameplayStatics.BreakHitResult` Hit)))))))